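; End-of-level pickup that, when collected with EndsLevel set, finishes the play phase for the player's kaiju.
; It locks the walk cycle, converts remaining countdown time times TimeBonusScale into bonus PropertyDamageDealt score, and shows that bonus in a popup widget.
; It then starts the game mode's post-play phase as Success if at least three baby kaijus were saved, otherwise as EarlyExit.
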(event EventBeginPlay
  (|CallParentFunction) ; This node is disabled and will not be called.\nDrag off pins to build functionality.
)

(event Collision|EventActorBeginOverlap
  (params (OtherActor :type Actor%20Object%20Reference))
  (|CallParentFunction OtherActor) ; This node is disabled and will not be called.\nDrag off pins to build functionality.
)

(event EventTick
  (params (DeltaSeconds :type Float%20%28single-precision%29)))

(event EventOnPickedUp
  (params (Character :type Kaiju%20Character%20Object%20Reference))
  (bind _returnvalue (Game|GetPlayerCharacter 0))
  (if (Variables|Default|GetEndsLevel)
    (bind _asplay_level_game_mode (Utilities|Casting|CastToPlayLevelGameMode (Game|GetGameMode)))
    (bind _askaiju_score_state (Utilities|Casting|CastToKaijuScoreState (Variables|/Script/Engine.Pawn|GetPlayerState _returnvalue)))
    (bind _askaiju_character (Utilities|Casting|CastToKaijuCharacter _returnvalue))
    (Variables|/Script/Neokaiju.KaijuMovementComponent|SetbLockWalkCycle (Variables|/Script/Neokaiju.KaijuCharacter|GetKaijuMovement _askaiju_character) true)
    (Variables|/Script/Neokaiju.KaijuScoreState|SetPropertyDamageDealt _askaiju_score_state (+ (Variables|/Script/Neokaiju.KaijuScoreState|GetPropertyDamageDealt _askaiju_score_state) (* (Class|BaseCountdownTimer|GetTimeRemaining (Variables|/Script/Neokaiju.PlayLevelGameMode|GetCountdownTimer _asplay_level_game_mode)) (Variables|Default|GetTimeBonusScale))))
    (bind _returnvalue_2 (UserInterface|CreateWidget "/Game/NeoKaiju/UI/StaticViewport/BP_TimeBonusPopup.BP_TimeBonusPopup_C" 0 (* (Class|BaseCountdownTimer|GetTimeRemaining (Variables|/Script/Neokaiju.PlayLevelGameMode|GetCountdownTimer _asplay_level_game_mode)) (Variables|Default|GetTimeBonusScale))))
    (UserInterface|Viewport|AddtoViewport _returnvalue_2 0)
    (bind _asphased_game_mode (Utilities|Casting|CastToPhasedGameMode (Game|GetGameMode)))
    (Class|PhasedGameMode|BeginPostPlayPhase _asphased_game_mode (select (>= (Variables|/Script/Neokaiju.KaijuScoreState|GetBabyKaijusSaved _askaiju_score_state) 3.0) "Success" "EarlyExit"))))

(fn ConstructionScript
  (|CallParentFunction))