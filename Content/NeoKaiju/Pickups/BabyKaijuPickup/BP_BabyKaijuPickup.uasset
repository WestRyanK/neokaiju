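; Baby kaiju pickup that the player's kaiju rescues by overlapping it, and that reacts when it comes on screen.
; A looping timer projects its location to the viewport until it is visible, then clears itself and plays a one-shot excited animation.
; Overlap with a KaijuCharacter's root component calls PickUp, while OnPickedUp plays the rescue event and spawns an impact emitter.
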(event OnComponentBeginOverlap(PickupCollision)
  (params (OverlappedComponent :type Primitive%20Component%20Object%20Reference) (OtherActor :type Actor%20Object%20Reference) (OtherComp :type Primitive%20Component%20Object%20Reference) (OtherBodyIndex :type Integer) (bFromSweep :type Boolean) (SweepResult :type Hit%20Result%20Structure%20%28by%20ref%29))
  (if (CallFunction|IsRootComponent OtherActor OtherComp)
    (bind _askaiju_character (Utilities|Casting|CastToKaijuCharacter OtherActor))
    (Class|PickupBase|PickUp _askaiju_character)))

(event Custom|Check%20if%20on%20Camera
  (bind _returnvalue (Transformation|GetActorLocation))
  (bind _returnvalue_2 (Viewport|GetViewportSize))
  (bind _returnvalue_3 (Game|GetPlayerController 0))
  (bind _screenposition (Class|GameplayStatics|ProjectWorldtoScreen _returnvalue_3 _returnvalue true))
  (if (Math|Boolean|ANDBoolean (> (.x _screenposition) 0.0) (> (.y _screenposition) 0.0) (< (.x _screenposition) (.x _returnvalue_2)) (< (.y _screenposition) (.y _returnvalue_2)))
    (Utilities|Time|SetTimerbyEvent (delegate Custom|Check%20if%20on%20Camera) 0.0)
    (CallFunction|PlayExcitedAnimation)))

(event Custom|Play%20Excited%20Animation
  (Components|Animation|PlayAnimation (Variables|Default|GetSkeletalMesh) "/Game/NeoKaiju/Pickups/BabyKaijuPickup/baby_kaiju_wow.baby_kaiju_wow" false))

(event EventBeginPlay
  (Utilities|Time|SetTimerbyEvent (delegate Custom|Check%20if%20on%20Camera) 0.3 true 1.0))

(event Collision|EventActorBeginOverlap
  (params (OtherActor :type Actor%20Object%20Reference)))

(event EventTick
  (params (DeltaSeconds :type Float%20%28single-precision%29)))

(event EventOnPickedUp
  (params (Character :type Kaiju%20Character%20Object%20Reference))
  (CallFunction|PlayEvent "/Game/Neokaiju/Audio/Events/Structures/KaijuRescue.KaijuRescue" (Transformation|GetActorLocation))
  (Effects|SpawnEmitteratLocation "/Game/NeoKaiju/Ability/StandardAbilities/JumpAbility/P_impact.P_Impact" (Transformation|GetActorLocation)))

(fn ConstructionScript)

(fn IsRootComponent
  (params (Actor :type Actor%20Object%20Reference) (Component :type Primitive%20Component%20Object%20Reference))
  (return (== (Variables|/Script/Engine.Actor|GetRootComponent Actor) Component)))