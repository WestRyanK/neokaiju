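; BP_Secret is a secret pickup with an animated icon plane and a sound or effect event on collection.
; Tick calls the parent, then drives Bob and Spin, which compute a sine vertical offset and a steady world-space yaw from game time.
; OnPickedUp plays the Pink_Block event at the actor's location.
; No overlap or collection logic is implemented in this Blueprint.
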(event EventBeginPlay
  (|CallParentFunction) ; This node is disabled and will not be called.\nDrag off pins to build functionality.
)

(event Collision|EventActorBeginOverlap
  (params (OtherActor :type Actor%20Object%20Reference))
  (|CallParentFunction OtherActor) ; This node is disabled and will not be called.\nDrag off pins to build functionality.
)

(event EventTick
  (params (DeltaSeconds :type Float%20%28single-precision%29))
  (|CallParentFunction DeltaSeconds)
  (CallFunction|Bob 1.0 1e+01)
  (CallFunction|Spin 3.0))

(event EventOnPickedUp
  (params (Character :type Kaiju%20Character%20Object%20Reference))
  (CallFunction|PlayEvent "/Game/Neokaiju/Audio/Events/Structures/Pink_Block.Pink_Block" (Transformation|GetActorLocation)))

(fn ConstructionScript
  (|CallParentFunction))

(fn Spin
  (params (Interval :type Float%20%28single-precision%29))
  (Transformation|SetWorldRotation (Variables|Default|GetIconPlane) (Math|Rotator|MakeRotator 9e+01 0.0 (/ (* (Utilities|Time|GetTimeSeconds) 3.6e+02) Interval)) false false))

(fn Bob
  (params (Interval :type Float%20%28single-precision%29) (Amplitude :type Float%20%28single-precision%29))
  (Transformation|SetRelativeLocation (Variables|Default|GetIconPlane) (Math|Vector|MakeVector 0.0 0.0 (* (Math|Trig|Sin(Radians) (/ (* (Utilities|Time|GetTimeSeconds) (* (Math|Trig|GetPI) 2.0)) Interval)) Amplitude)) false false))