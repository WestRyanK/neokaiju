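; Player Kaiju character Blueprint that handles camera-arm flipping, feedback and level-based visuals.
; Facing flips from KaijuMovement toggle left/right fire effects and rotate the spring arm, deferring rotation until landing when airborne.
; Landings play level-indexed sounds and velocity-scaled rumble, damage triggers montage, sound, rumble and material flash, and level changes swap fire Niagara systems.
; It also fits pooled spline meshes to a given spline and moves the audio listener onto the Kaiju.
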(event Custom|OnFacingDirectionFlipped
  (params (FacingDirection :type EFacingDirection%20Enum :default "RIGHT"))
  (bind _perpendiculartagawarespringarm (Variables|Default|GetPerpendicularTagAwareSpringArm))
  (CallFunction|EnableRightLeftFireEffects FacingDirection)
  ;[1 0.3599 0.01562] convert to c++ time permitting
  (if (AI|Components|NavMovement|IsFalling (Variables|Character|GetCharacterMovement))
    (Variables|Default|SetShouldFlipOnLand (not (Variables|Default|GetShouldFlipOnLand)))
    (else
      (Transformation|SetWorldRotation _perpendiculartagawarespringarm (Utilities|Select :Index FacingDirection :NONE (Transformation|GetWorldRotation _perpendiculartagawarespringarm) :RIGHT "0,180.000000, 0" :LEFT "0, 0, 0") false false))))

(event EventOnLanded
  (params (Hit :type Hit%20Result%20Structure%20%28by%20ref%29))
  (bind _perpendiculartagawarespringarm (Variables|Default|GetPerpendicularTagAwareSpringArm))
  ;[1 0.3599 0.01562] see below
  (if (Variables|Default|GetShouldFlipOnLand)
    ;[1 0.3599 0.01562] convert to c++ time permitting
    (Variables|Default|SetShouldFlipOnLand false)
    (Transformation|SetWorldRotation _perpendiculartagawarespringarm (Utilities|Select :Index (stale Custom|OnFacingDirectionFlipped FacingDirection) :NONE (Transformation|GetWorldRotation _perpendiculartagawarespringarm) :RIGHT "0,180.000000, 0" :LEFT "0, 0, 0") false false)
    (else
      (CallFunction|PlayLandSoundbyLevel)
      (Game|Feedback|PlayDynamicForceFeedback (Game|GetPlayerController 0) (CallFunction|LandForceIntensity) 0.25 true true true true))))

(event EventOnDamageTaken
  (params (OldHealth :type Float%20%28single-precision%29) (NewHealth :type Float%20%28single-precision%29))
  (Animation|PlayAnimMontage 0 4.0 "start")
  (Class|FMODBlueprintStatics|PlayEvent2D (Variables|Default|GetDamagedSoundEvent))
  (Game|Feedback|ClientPlayForceFeedback (Game|GetPlayerController 0) (Variables|Default|GetDamageTakenForceFeedback) "None" false false false)
  (Rendering|Material|SetScalarParameterValueonMaterials (Variables|Character|GetMesh) "Em_Color_Value" 1e+03)
  (Rendering|Material|SetScalarParameterValueonMaterials (Variables|Character|GetMesh) "Em_Hue_Shift" 0.3)
  (Utilities|FlowControl|Delay 0.3)
  (Rendering|Material|SetScalarParameterValueonMaterials (Variables|Character|GetMesh) "Em_Color_Value" 2.0)
  (Rendering|Material|SetScalarParameterValueonMaterials (Variables|Character|GetMesh) "Em_Hue_Shift" 0.0))

(event EventBeginPlay
  (|CallParentFunction)
  (EventDispatchers|AssignOnFacingDirectionFlipped (Variables|Default|GetKaijuMovement) (EventDispatchers|CreateEvent :!event Custom|OnFacingDirectionFlipped))
  (CallFunction|AttachAudioListenertoKaiju))

(event EventTick
  (params (DeltaSeconds :type Float%20%28single-precision%29)))

(event EventUpdateSplineMeshes
  (params (SplineRef :type Spline%20Component%20Object%20Reference))
  (bind _splinemeshlength (Variables|Default|GetSplineMeshLength))
  (bind _splinemeshlength_2 (Variables|Default|GetSplineMeshLength))
  (for (_array_element _array_index) (Variables|Default|GetSplineMeshes)
    (Rendering|SetVisibility _array_element (< (* _array_index _splinemeshlength_2) (Spline|GetSplineLength SplineRef)) false)
    (if (< (* _array_index _splinemeshlength_2) (Spline|GetSplineLength SplineRef))
      (SplineMesh|SetStartandEnd _array_element (Spline|GetLocationatDistanceAlongSpline SplineRef (* _array_index _splinemeshlength_2) "Local") (Math|Vector|ClampVectorSize (Spline|GetTangentatDistanceAlongSpline SplineRef (* _array_index _splinemeshlength_2) "Local") 0.0 _splinemeshlength) (Spline|GetLocationatDistanceAlongSpline SplineRef (* (+ _array_index 1) _splinemeshlength_2) "Local") (Math|Vector|ClampVectorSize (Spline|GetTangentatDistanceAlongSpline SplineRef (* (+ _array_index 1) _splinemeshlength_2) "Local") 0.0 _splinemeshlength) true :!class /Script/Engine.SplineMeshComponent))))

(event EventOnKaijuLevelChanged
  (params (OldLevel :type Float%20%28single-precision%29) (NewLevel :type Float%20%28single-precision%29))
  (CallFunction|SetNiagaraSystemsforLevel (Math|Float|Truncate NewLevel)))

(fn ConstructionScript
  (for _index (range 1 (Variables|Default|GetSplineCount))
    (bind _returnvalue (AddComponent|AddSplineMeshComponent false))
    (Utilities|Array|Add (Variables|Default|GetSplineMeshes) _returnvalue)
    (Rendering|SetVisibility _returnvalue false false)))

(fn LandForceIntensity
  (return (Math|Float|Clamp(Float) (Math|Float|NormalizetoRange (Math|Float|Square (- 0.0 (.z (Transformation|GetVelocity)))) 0.0 (Math|Float|Square (Math|Float|MakeLiteralFloat 4e+03))) 0.02)))

(fn EnableRightLeftFireEffects
  (params (FacingDirection :type EFacingDirection%20Enum :default "RIGHT"))
  (bind _returnvalue (Utilities|Select :Index FacingDirection :NONE false :RIGHT true :LEFT false))
  (LocalVariables|SetRightOn _returnvalue)
  (LocalVariables|SetLeftOn (not _returnvalue))
  (Rendering|SetVisibility (Variables|Default|GetFV_TailFire) (LocalVariables|GetRightOn) false)
  (Rendering|SetVisibility (Variables|Default|GetFV_BackFire) (LocalVariables|GetRightOn) false)
  (Rendering|SetVisibility (Variables|Default|GetBV_BackFire) (LocalVariables|GetLeftOn) false)
  (Rendering|SetVisibility (Variables|Default|GetBV_TailFire) (LocalVariables|GetLeftOn) false))

(fn PlayLandSoundbyLevel
  (Class|FMODBlueprintStatics|PlayEvent2D (Utilities|Array|Get(acopy) (Variables|Default|GetLandSoundEvent) (Math|Float|Truncate (.ReturnValue (Ability|Attribute|GetFloatAttribute self "(AttributeName=\"KaijuLevel\",Attribute=StructProperty'\"/Script/Neokaiju.KaijuAttributeSet:KaijuLevel\"',AttributeOwner=Class'\"/Script/Neokaiju.KaijuAttributeSet\"')"))))))

(fn ReinitNiagaraSystemwithAsset
  (params (ParticleSystem :type Niagara%20Component%20Object%20Reference) (Systems :type Array%20of%20Niagara%20System%20Object%20References) (Index :type Integer))
  (Class|NiagaraComponent|SetAsset ParticleSystem (Utilities|Array|Get(acopy) Systems Index))
  (Niagara|ReinitializeSystem ParticleSystem))

(fn SetNiagaraSystemsforLevel
  (params (Level :type Integer))
  (CallFunction|ReinitNiagaraSystemwithAsset (Variables|Default|GetFV_BackFire) (Variables|Default|GetFV_Back_Fire_Array) Level)
  (CallFunction|ReinitNiagaraSystemwithAsset (Variables|Default|GetBV_BackFire) (Variables|Default|GetBV_Back_Fire_Array) Level)
  (CallFunction|ReinitNiagaraSystemwithAsset (Variables|Default|GetFV_TailFire) (Variables|Default|GetFV_Tail_Fire_Array) Level)
  (CallFunction|ReinitNiagaraSystemwithAsset (Variables|Default|GetBV_TailFire) (Variables|Default|GetBV_Tail_Fire_Array) Level))

(fn AttachAudioListenertoKaiju
  ;[1 1 1] The Audio Listener (FMOD's "ear") is defaulted to the camera, which is far away. We're attaching it to the Kaiju itself so attenuation will work better
  (Class|PlayerController|SetAudioListenerOverride (Game|GetPlayerController 0) (Variables|Default|GetRotationScaleIndependentPoint) "0, 0, 0" "0, 0, 0"))