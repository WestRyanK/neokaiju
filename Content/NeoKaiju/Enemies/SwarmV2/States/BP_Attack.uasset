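; Attack state for a SwarmV2 enemy that lunges at the target kaiju along a direction locked on Enter.
; Update backs the swarm up, halting on overlap, then plays the stab sound and charges, switching to Dissassemble on timeout.
; Charge hits lead to Grab in claw mode, swarm death against a dashing kaiju (tag and attribute check), or GAS damage and Stuck.
; Building blocks take damage, static meshes just cause Stuck, and lasers damage the swarm.
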(event EventEnter
  (params (NewSwarm :type Swarm%20V2%20Object%20Reference))
  (bind _swarmref (Variables|Default|GetSwarmRef))
  (|CallParentFunction NewSwarm)
  (Variables|Default|Setattack_time 0.0)
  (Variables|Default|Setpre_attack_reverse_time 0.0)
  (Variables|Default|Setreversing true)
  (Variables|Default|Setstopped false)
  (bind _output_get (Variables|Default|SetattackVector (Math|Vector|Normalize (- (Transformation|GetActorLocation (Variables|/Script/Neokaiju.SwarmV2|GetTargetKaiju _swarmref)) (Transformation|GetActorLocation _swarmref)))))
  (Variables|/Script/Neokaiju.SwarmV2|SetLastDirection (Variables|Default|GetSwarmRef) _output_get))

(event EventUpdate
  (params (DeltaTime :type Float%20%28single-precision%29))
  (bind _swarmref (Variables|Default|GetSwarmRef))
  (bind _swarmref_2 (Variables|Default|GetSwarmRef))
  (bind _swarmref_3 (Variables|Default|GetSwarmRef))
  (bind _swarmref_4 (Variables|Default|GetSwarmRef))
  (if (Variables|/Script/Neokaiju.SwarmV2|GetbHitByLaser _swarmref_2)
    (bind _asbp_swarm_v2 (Utilities|Casting|CastToBP_SwarmV2 _swarmref_2)
      (:then
        (Default|LaserDamage _asbp_swarm_v2))
      (:CastFailed
        _)))
  (if (<= (Variables|Default|Getpre_attack_reverse_time) (Variables|/Script/Neokaiju.SwarmStats|GetPreAttackReverseTime (Variables|/Script/Neokaiju.SwarmV2|GetStats (Variables|Default|GetSwarmRef))))
    (Variables|Default|Setpre_attack_reverse_time (+ DeltaTime (Variables|Default|Getpre_attack_reverse_time)))
    (if (not (Variables|Default|Getstopped))
      (Class|SwarmV2|Move _swarmref_3 DeltaTime (Variables|/Script/Neokaiju.SwarmStats|GetPreAttackReverseSpeed (Variables|/Script/Neokaiju.SwarmV2|GetStats _swarmref_3)) (Math|Vector|NegateVector (Variables|Default|GetattackVector))))
    (else
      (if (Variables|Default|Getreversing)
        (Variables|Default|Setreversing false)
        (Class|FMODBlueprintStatics|PlayEventAttached "/Game/Neokaiju/Audio/Events/Environment/Swarm_Stab.Swarm_Stab" (Variables|/Script/Engine.Actor|GetRootComponent (Variables|Default|GetSwarmRef)) "None" "0, 0, 0" "KeepRelativeOffset"))
      (if (<= (Variables|Default|Getattack_time) (Variables|/Script/Neokaiju.SwarmStats|GetMaxAttackTime (Variables|/Script/Neokaiju.SwarmV2|GetStats (Variables|Default|GetSwarmRef))))
        (Variables|Default|Setattack_time (+ DeltaTime (Variables|Default|Getattack_time)))
        (Class|SwarmV2|Move _swarmref DeltaTime (Variables|/Script/Neokaiju.SwarmStats|GetAttackSpeed (Variables|/Script/Neokaiju.SwarmV2|GetStats _swarmref)) (Variables|Default|GetattackVector))
        (else
          (bind _returnvalue (Game|ConstructObjectfromClass "/Game/NeoKaiju/Enemies/SwarmV2/States/BP_Dissassemble.BP_Dissassemble_C" _swarmref_4))
          (Class|SwarmV2|ChangeState _swarmref_4 _returnvalue))))))

(event EventOnInnerBeginOverlap
  (params (OverlappedComponent :type Primitive%20Component%20Object%20Reference) (OtherActor :type Actor%20Object%20Reference) (OtherComp :type Primitive%20Component%20Object%20Reference) (OtherBodyIndex :type Integer) (FromSweep :type Boolean) (SweepResult :type Hit%20Result%20Structure))
  (bind _swarmref (Variables|Default|GetSwarmRef))
  (bind _swarmref_2 (Variables|Default|GetSwarmRef))
  (bind _swarmref_3 (Variables|Default|GetSwarmRef))
  (bind _swarmref_4 (Variables|Default|GetSwarmRef))
  (bind _targetkaiju (Variables|/Script/Neokaiju.SwarmV2|GetTargetKaiju _swarmref_3))
  (bind _targetkaiju_2 (Variables|/Script/Neokaiju.SwarmV2|GetTargetKaiju _swarmref_4))
  (bind _returnvalue (Ability|GetAbilitySystemComponent _targetkaiju))
  (bind _returnvalue_2 (Ability|GetAbilitySystemComponent _targetkaiju_2))
  (if (Variables|Default|Getreversing)
    (Variables|Default|Setstopped true)
    (elif (== OtherActor (Variables|/Script/Neokaiju.SwarmV2|GetTargetKaiju (Variables|Default|GetSwarmRef)))
      (if (Variables|/Script/Neokaiju.SwarmV2|GetClawMode _swarmref_3)
        (bind _returnvalue_3 (Game|ConstructObjectfromClass "/Game/NeoKaiju/Enemies/SwarmV2/States/BP_Grab.BP_Grab_C" _swarmref_2))
        (Class|SwarmV2|ChangeState _swarmref_2 _returnvalue_3)
        (elif (and (GameplayTags|HasMatchingGameplayTag _returnvalue_2 "(TagName=\"Cooldown.Ability.Standard.Dash\")") (== (.ReturnValue (Ability|Attribute|GetFloatAttributefromAbilitySystemComponent _returnvalue_2 "(AttributeName=\"KaijuLevel\",Attribute=StructProperty'\"/Script/Neokaiju.KaijuAttributeSet:KaijuLevel\"',AttributeOwner=Class'\"/Script/Neokaiju.KaijuAttributeSet\"')")) 4.0))
          (Class|SwarmV2|KillSwarm (Variables|Default|GetSwarmRef))
          (else
            (Utilities|FlowControl|DoOnce false
              (:Completed
                (GameplayEffects|ApplyGameplayEffectToSelf _returnvalue "/Game/NeoKaiju/Enemies/Swarm/GE_SwarmDamageKaiju.GE_SwarmDamageKaiju_C" 0.0 (GameplayEffects|MakeEffectContext _returnvalue))
                (bind _returnvalue_4 (Game|ConstructObjectfromClass "/Game/NeoKaiju/Enemies/SwarmV2/States/BP_Stuck.BP_Stuck_C" _swarmref :!label _label))
                (Class|SwarmV2|ChangeState _swarmref _returnvalue_4))))))
      (else
        (bind _asbuilding_block (Utilities|Casting|CastToBuildingBlock OtherActor)
          (:then
            (GameplayEffects|ApplyGameplayEffectToSelf (Ability|GetAbilitySystemComponent _asbuilding_block) "/Game/NeoKaiju/Enemies/Swarm/GE_SwarmDamageBlock.GE_SwarmDamageBlock_C" 0.0 (GameplayEffects|MakeEffectContext (Ability|GetAbilitySystemComponent _asbuilding_block)))
            (goto _label))
          (:CastFailed
            (Utilities|Casting|CastToStaticMeshActor OtherActor)
            (goto _label)))))))

(event EventExit
  (Collision|SetCollisionResponsetoChannel (Variables|/Script/Neokaiju.SwarmV2|GetInnerRadius (Variables|Default|GetSwarmRef)) "ECC_Pawn" "ECR_Overlap"))

(event EventOnBeginHitbyLaser
  (bind _asbp_swarm_v2 (Utilities|Casting|CastToBP_SwarmV2 (Variables|Default|GetSwarmRef)))
  (Default|ShowHealthBar _asbp_swarm_v2))

(fn OnMeshBeginOverlap
  (params (OverlappedComponent :type Primitive%20Component%20Object%20Reference) (OtherActor :type Actor%20Object%20Reference) (OtherComp :type Primitive%20Component%20Object%20Reference) (OtherBodyIndex :type Integer) (FromSweep :type Boolean) (SweepResult :type Hit%20Result%20Structure)))