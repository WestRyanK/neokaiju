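; Idle state for the V2 swarm enemy, waiting for its target Kaiju to come within range.
; On entry it sizes the outer sphere to the idle radius and switches to Chase immediately if the Kaiju is already inside, or later on overlap.
; An inner overlap while the Kaiju has the Dash cooldown tag switches to Scatter.
; Laser events are empty, and the laser-triggered Scatter nodes never run.
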(event EventEnter
  (params (NewSwarm :type Swarm%20V2%20Object%20Reference))
  (bind _swarmref (Variables|Default|GetSwarmRef))
  (bind _swarmref_2 (Variables|Default|GetSwarmRef))
  (|CallParentFunction NewSwarm)
  (Components|Sphere|SetSphereRadius (Variables|/Script/Neokaiju.SwarmV2|GetOuterRadius _swarmref) (Variables|/Script/Neokaiju.SwarmStats|GetIdleOuterRadius (Variables|/Script/Neokaiju.SwarmV2|GetStats _swarmref)) true)
  ;[1 1 1] if it's already close enough go straight to the point
  (if (<= (Transformation|GetDistanceTo (Variables|/Script/Neokaiju.SwarmV2|GetTargetKaiju _swarmref_2) _swarmref_2) (Variables|/Script/Neokaiju.SwarmStats|GetIdleOuterRadius (Variables|/Script/Neokaiju.SwarmV2|GetStats _swarmref_2)))
    (Class|SwarmState|OnOuterBeginOverlap 0 (Variables|/Script/Neokaiju.SwarmV2|GetTargetKaiju (Variables|Default|GetSwarmRef)) 0 0 false)))

(event EventOnOuterBeginOverlap
  (params (OverlappedComponent :type Primitive%20Component%20Object%20Reference) (OtherActor :type Actor%20Object%20Reference) (OtherComp :type Primitive%20Component%20Object%20Reference) (OtherBodyIndex :type Integer) (FromSweep :type Boolean) (SweepResult :type Hit%20Result%20Structure))
  (bind _swarmref (Variables|Default|GetSwarmRef))
  (if (== OtherActor (Variables|/Script/Neokaiju.SwarmV2|GetTargetKaiju _swarmref))
    (bind _returnvalue (Game|ConstructObjectfromClass "/Game/NeoKaiju/Enemies/SwarmV2/States/BP_Chase.BP_Chase_C" _swarmref))
    (Class|SwarmV2|ChangeState _swarmref _returnvalue)))

(event EventOnBeginHitbyLaser)

(event EventOnBeginOverlapbyLaser)

(event EventOnInnerBeginOverlap
  (params (OverlappedComponent :type Primitive%20Component%20Object%20Reference) (OtherActor :type Actor%20Object%20Reference) (OtherComp :type Primitive%20Component%20Object%20Reference) (OtherBodyIndex :type Integer) (FromSweep :type Boolean) (SweepResult :type Hit%20Result%20Structure))
  (bind _swarmref (Variables|Default|GetSwarmRef))
  (bind _swarmref_2 (Variables|Default|GetSwarmRef))
  (bind _targetkaiju (Variables|/Script/Neokaiju.SwarmV2|GetTargetKaiju _swarmref))
  (if (and (== OtherActor _targetkaiju) (GameplayTags|HasMatchingGameplayTag (Ability|GetAbilitySystemComponent _targetkaiju) "(TagName=\"Cooldown.Ability.Standard.Dash\")"))
    (bind _returnvalue (Game|ConstructObjectfromClass "/Game/NeoKaiju/Enemies/SwarmV2/States/BP_Scatter.BP_Scatter_C" _swarmref_2))
    (Variables|/Game/NeoKaiju/Enemies/SwarmV2/States/BP_Scatter.BP_Scatter_C|SetscatterByLazer _returnvalue false)
    (Class|SwarmV2|ChangeState _swarmref_2 _returnvalue)))