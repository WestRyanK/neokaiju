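; Swarm enemy state that strafes around the target kaiju for a timed period, then switches to Assemble.
; Each update it moves along a tangent from a cross product, adjusted by an open-space search, and reverses when deflected over 20 degrees.
; It returns to Chase if the kaiju leaves the strafe radius.
; Inner overlap with a kaiju on dash cooldown triggers Scatter; laser events do nothing.
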(event EventEnter
  (params (NewSwarm :type Swarm%20V2%20Object%20Reference))
  (bind _swarmref (Variables|Default|GetSwarmRef))
  (|CallParentFunction NewSwarm)
  (Variables|/Script/Neokaiju.SwarmV2|SetLastDirection _swarmref "0, 0, 0")
  (Components|Sphere|SetSphereRadius (Variables|/Script/Neokaiju.SwarmV2|GetOuterRadius _swarmref) (Variables|/Script/Neokaiju.SwarmStats|GetStrafeOuterRadius (Variables|/Script/Neokaiju.SwarmV2|GetStats _swarmref)) true)
  (Variables|Default|SetStrafe_time 0.0)
  (Variables|Default|SetdirectionVector (Class|KismetMathLibrary|VectorRight)))

(event EventUpdate
  (params (DeltaTime :type Float%20%28single-precision%29))
  (bind _swarmref (Variables|Default|GetSwarmRef))
  (bind _swarmref_2 (Variables|Default|GetSwarmRef))
  (bind _swarmref_3 (Variables|Default|GetSwarmRef))
  (bind _swarmref_4 (Variables|Default|GetSwarmRef))
  (bind _swarmref_5 (Variables|Default|GetSwarmRef))
  (bind _returnvalue (Transformation|GetActorLocation _swarmref_3))
  (bind _targetkaiju (Variables|/Script/Neokaiju.SwarmV2|GetTargetKaiju _swarmref_3))
  (bind _returnvalue_2 (Transformation|GetActorLocation _targetkaiju))
  (bind _returnvalue_3 (- _returnvalue_2 _returnvalue))
  (bind _returnvalue_4 (Math|Vector|VectorLength _returnvalue_3))
  (if (> (Variables|/Script/Neokaiju.SwarmStats|GetStrafeTime (Variables|/Script/Neokaiju.SwarmV2|GetStats (Variables|Default|GetSwarmRef))) (Variables|Default|GetStrafe_time))
    (Variables|Default|SetStrafe_time (+ DeltaTime (Variables|Default|GetStrafe_time)))
    ;[1 1 1] go back to chase if the player gets too far away
    (if (< _returnvalue_4 (Variables|/Script/Neokaiju.SwarmStats|GetStrafeOuterRadius (Variables|/Script/Neokaiju.SwarmV2|GetStats (Variables|Default|GetSwarmRef))))
      (bind _returnvalue_5 (Class|SwarmV2|FindOpenSpaceFrontBack (Variables|Default|GetSwarmRef) (Math|Vector|Normalize (Math|Vector|CrossProduct _returnvalue_3 (Variables|Default|GetdirectionVector))) _returnvalue_4))
      ;[1 1 1] reverse direction of strafing if the desired direction was not returned
      (if (>= (Math|Vector|DotProduct _returnvalue_5 (Math|Vector|Normalize (Math|Vector|CrossProduct _returnvalue_3 (Variables|Default|GetdirectionVector)))) (Math|Trig|Cos(Degrees) 2e+01))
        _
        (else
          (Variables|Default|SetdirectionVector (Math|Vector|NegateVector (Variables|Default|GetdirectionVector)))))
      (bind _output_get (Variables|/Script/Neokaiju.SwarmV2|SetLastDirection _swarmref_5 _returnvalue_5))
      (Class|SwarmV2|Move _swarmref_5 DeltaTime (Variables|/Script/Neokaiju.SwarmStats|GetStrafeSpeed (Variables|/Script/Neokaiju.SwarmV2|GetStats _swarmref_5)) _output_get)
      (Class|SwarmV2|OrientSwarm _swarmref (Math|Rotator|MakeRotfromZ _returnvalue_3))
      (Class|SwarmV2|RotateSwarm _swarmref DeltaTime)
      (else
        (bind _returnvalue_6 (Game|ConstructObjectfromClass "/Game/NeoKaiju/Enemies/SwarmV2/States/BP_Chase.BP_Chase_C" _swarmref_4))
        (Class|SwarmV2|ChangeState _swarmref_4 _returnvalue_6)))
    (else
      (bind _returnvalue_7 (Game|ConstructObjectfromClass "/Game/NeoKaiju/Enemies/SwarmV2/States/BP_Assemble.BP_Assemble_C" _swarmref_2))
      (Class|SwarmV2|ChangeState _swarmref_2 _returnvalue_7))))

(event EventOnBeginOverlapbyLaser)

(event EventOnBeginHitbyLaser)

(event EventOnInnerBeginOverlap
  (params (OverlappedComponent :type Primitive%20Component%20Object%20Reference) (OtherActor :type Actor%20Object%20Reference) (OtherComp :type Primitive%20Component%20Object%20Reference) (OtherBodyIndex :type Integer) (FromSweep :type Boolean) (SweepResult :type Hit%20Result%20Structure))
  (bind _swarmref (Variables|Default|GetSwarmRef))
  (bind _swarmref_2 (Variables|Default|GetSwarmRef))
  (bind _targetkaiju (Variables|/Script/Neokaiju.SwarmV2|GetTargetKaiju _swarmref))
  (if (and (== OtherActor _targetkaiju) (GameplayTags|HasMatchingGameplayTag (Ability|GetAbilitySystemComponent _targetkaiju) "(TagName=\"Cooldown.Ability.Standard.Dash\")"))
    (bind _returnvalue (Game|ConstructObjectfromClass "/Game/NeoKaiju/Enemies/SwarmV2/States/BP_Scatter.BP_Scatter_C" _swarmref_2))
    (Variables|/Game/NeoKaiju/Enemies/SwarmV2/States/BP_Scatter.BP_Scatter_C|SetscatterByLazer _returnvalue false)
    (Class|SwarmV2|ChangeState _swarmref_2 _returnvalue)))