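; BP_Stuck is the SwarmV2 enemy state for a swarm that is stuck.
; It waits out the stuck time, reverses against the swarm's last direction for a set time, then switches to BP_Dissassemble.
; Inner overlaps with anything but the target kaiju halt the reversing, while overlapping the kaiju kills the swarm if an attribute check and Dash cooldown tag match.
; Laser hits apply damage throughout.
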(event EventEnter
  (params (NewSwarm :type Swarm%20V2%20Object%20Reference))
  (|CallParentFunction NewSwarm)
  (Variables|Default|Setstuck_time 0.0)
  (Variables|Default|Setreversing_time 0.0)
  (Variables|Default|Setstuck_dir (Variables|/Script/Neokaiju.SwarmV2|GetLastDirection (Variables|Default|GetSwarmRef)))
  (Variables|Default|Setstop false)
  (Variables|Default|SetlazerHitTime 0.0))

(event EventUpdate
  (params (DeltaTime :type Float%20%28single-precision%29))
  (bind _swarmref (Variables|Default|GetSwarmRef))
  (bind _swarmref_2 (Variables|Default|GetSwarmRef))
  (bind _swarmref_3 (Variables|Default|GetSwarmRef))
  (Variables|Default|SetDeltaTime DeltaTime)
  (if (Variables|/Script/Neokaiju.SwarmV2|GetbHitByLaser _swarmref)
    (bind _asbp_swarm_v2 (Utilities|Casting|CastToBP_SwarmV2 _swarmref)
      (:then
        (Default|LaserDamage _asbp_swarm_v2))
      (:CastFailed
        _)))
  (if (<= (Variables|Default|Getstuck_time) (Variables|/Script/Neokaiju.SwarmStats|GetStuckTime (Variables|/Script/Neokaiju.SwarmV2|GetStats (Variables|Default|GetSwarmRef))))
    (Variables|Default|Setstuck_time (+ (Variables|Default|GetDeltaTime) (Variables|Default|Getstuck_time)))
    (elif (<= (Variables|Default|Getreversing_time) (Variables|/Script/Neokaiju.SwarmStats|GetReverseTime (Variables|/Script/Neokaiju.SwarmV2|GetStats (Variables|Default|GetSwarmRef))))
      (Variables|Default|Setreversing_time (+ (Variables|Default|Getreversing_time) (Variables|Default|GetDeltaTime)))
      (if (not (Variables|Default|Getstop))
        (Transformation|SetActorLocation _swarmref_3 (- (Transformation|GetActorLocation _swarmref_3) (* (Variables|Default|Getstuck_dir) (* (Variables|/Script/Neokaiju.SwarmStats|GetReverseSpeed (Variables|/Script/Neokaiju.SwarmV2|GetStats (Variables|Default|GetSwarmRef))) (Variables|Default|GetDeltaTime)))) false false))
      (else
        (bind _returnvalue (Game|ConstructObjectfromClass "/Game/NeoKaiju/Enemies/SwarmV2/States/BP_Dissassemble.BP_Dissassemble_C" _swarmref_2))
        (Class|SwarmV2|ChangeState _swarmref_2 _returnvalue)))))

(event EventOnInnerBeginOverlap
  (params (OverlappedComponent :type Primitive%20Component%20Object%20Reference) (OtherActor :type Actor%20Object%20Reference) (OtherComp :type Primitive%20Component%20Object%20Reference) (OtherBodyIndex :type Integer) (FromSweep :type Boolean) (SweepResult :type Hit%20Result%20Structure))
  (bind _swarmref (Variables|Default|GetSwarmRef))
  (bind _targetkaiju (Variables|/Script/Neokaiju.SwarmV2|GetTargetKaiju _swarmref))
  (bind _returnvalue (Ability|GetAbilitySystemComponent _targetkaiju))
  (if (== OtherActor _targetkaiju)
    (if (and (== (.ReturnValue (Ability|Attribute|GetFloatAttributefromAbilitySystemComponent _returnvalue "(AttributeName=\"KaijuLevel\",Attribute=StructProperty'\"/Script/Neokaiju.KaijuAttributeSet:KaijuLevel\"',AttributeOwner=Class'\"/Script/Neokaiju.KaijuAttributeSet\"')")) 4.0) (GameplayTags|HasMatchingGameplayTag _returnvalue "(TagName=\"Cooldown.Ability.Standard.Dash\")"))
      (Class|SwarmV2|KillSwarm (Variables|Default|GetSwarmRef)))
    (else
      (Variables|Default|Setstop true))))