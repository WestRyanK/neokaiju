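; BP_Aim is the aim state of the SwarmV2 enemy, turning the swarm toward its target kaiju before it attacks.
; Enter picks the claw or bullet pointer hook and hides the aiming pointer, which is disabled by request.
; Update orients swarm and pointer and applies laser damage when hit, switching to a new BP_Attack once aim time expires.
; An inner overlap kills the swarm if the kaiju has the dash cooldown tag and passes an attribute check.
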(event EventEnter
  (params (NewSwarm :type Swarm%20V2%20Object%20Reference))
  (|CallParentFunction NewSwarm)
  (Variables|Default|SetAim_Time 0.0)
  (Variables|Default|Setlazer_kill_time 0.0)
  (bind _asbp_swarm_v2 (Utilities|Casting|CastToBP_SwarmV2 (Variables|Default|GetSwarmRef)))
  ;[1 1 1] turned off at jordan's request, turn back on for aiming lazer
  (Rendering|SetVisibility (Variables|/Game/NeoKaiju/Enemies/SwarmV2/BP_SwarmV2.BP_SwarmV2_C|Getpointer _asbp_swarm_v2) false false)
  (if (Variables|/Script/Neokaiju.SwarmV2|GetClawMode (Variables|Default|GetSwarmRef))
    (Variables|Default|Setpointer_hook (Variables|/Game/NeoKaiju/Enemies/SwarmV2/BP_SwarmV2.BP_SwarmV2_C|GetclawPointerHook _asbp_swarm_v2))
    (else
      (Variables|Default|Setpointer_hook (Variables|/Game/NeoKaiju/Enemies/SwarmV2/BP_SwarmV2.BP_SwarmV2_C|GetbulletPointerHook _asbp_swarm_v2)))))

(event EventUpdate
  (params (DeltaTime :type Float%20%28single-precision%29))
  (bind _swarmref (Variables|Default|GetSwarmRef))
  (bind _swarmref_2 (Variables|Default|GetSwarmRef))
  (bind _returnvalue (Transformation|GetActorLocation _swarmref))
  (bind _targetkaiju (Variables|/Script/Neokaiju.SwarmV2|GetTargetKaiju _swarmref))
  (bind _returnvalue_2 (Transformation|GetActorLocation _targetkaiju))
  (bind _returnvalue_3 (- _returnvalue_2 _returnvalue))
  (if (<= (Variables|Default|GetAim_Time) (Variables|/Script/Neokaiju.SwarmStats|GetAimTime (Variables|/Script/Neokaiju.SwarmV2|GetStats (Variables|Default|GetSwarmRef))))
    (Variables|Default|SetAim_Time (+ DeltaTime (Variables|Default|GetAim_Time)))
    (if (Variables|/Script/Neokaiju.SwarmV2|GetbHitByLaser (Variables|Default|GetSwarmRef))
      (bind _asbp_swarm_v2 (Utilities|Casting|CastToBP_SwarmV2 (Variables|Default|GetSwarmRef))
        (:then
          (Default|LaserDamage _asbp_swarm_v2))
        (:CastFailed
          _)))
    (Class|SwarmV2|OrientSwarm (Variables|Default|GetSwarmRef) (Math|Rotator|MakeRotfromZ _returnvalue_3))
    (bind _asbp_swarm_v2_2 (Utilities|Casting|CastToBP_SwarmV2 (Variables|Default|GetSwarmRef)))
    (Default|OrientPointer _asbp_swarm_v2_2 (Variables|Default|Getpointer_hook) (Math|Vector|Normalize _returnvalue_3))
    (else
      (bind _returnvalue_4 (Game|ConstructObjectfromClass "/Game/NeoKaiju/Enemies/SwarmV2/States/BP_Attack.BP_Attack_C" _swarmref_2))
      (Class|SwarmV2|ChangeState _swarmref_2 _returnvalue_4))))

(event EventExit
  (bind _asbp_swarm_v2 (Utilities|Casting|CastToBP_SwarmV2 (Variables|Default|GetSwarmRef)))
  (Rendering|SetVisibility (Variables|/Game/NeoKaiju/Enemies/SwarmV2/BP_SwarmV2.BP_SwarmV2_C|Getpointer _asbp_swarm_v2) false false))

(event EventOnInnerBeginOverlap
  (params (OverlappedComponent :type Primitive%20Component%20Object%20Reference) (OtherActor :type Actor%20Object%20Reference) (OtherComp :type Primitive%20Component%20Object%20Reference) (OtherBodyIndex :type Integer) (FromSweep :type Boolean) (SweepResult :type Hit%20Result%20Structure))
  (bind _swarmref (Variables|Default|GetSwarmRef))
  (bind _targetkaiju (Variables|/Script/Neokaiju.SwarmV2|GetTargetKaiju _swarmref))
  (bind _returnvalue (Ability|GetAbilitySystemComponent _targetkaiju))
  (if (Math|Boolean|ANDBoolean (== OtherActor _targetkaiju) (GameplayTags|HasMatchingGameplayTag _returnvalue "(TagName=\"Cooldown.Ability.Standard.Dash\")") (== (.ReturnValue (Ability|Attribute|GetFloatAttributefromAbilitySystemComponent _returnvalue "(AttributeName=\"KaijuLevel\",Attribute=StructProperty'\"/Script/Neokaiju.KaijuAttributeSet:KaijuLevel\"',AttributeOwner=Class'\"/Script/Neokaiju.KaijuAttributeSet\"')")) 4.0))
    (Class|SwarmV2|KillSwarm (Variables|Default|GetSwarmRef))))