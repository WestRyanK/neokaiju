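; Swarm enemy state that captures the target kaiju and holds it on a spring until it struggles free.
; An analytically solved damped spring moves it along world X; struggles add velocity and weaken the spring, and outer-sphere collisions zero velocity.
; SwarmGrabManager shares motion between grabbers, so only the commanding swarm moves the kaiju while each follows at its offset.
; On escape the swarm spins briefly, then switches to BP_Dissassemble.
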(event Custom|OnCapturedActorStruggle
  (params (StruggleAttemptNum :type Integer) (StrugglesRemainingToEscape :type Integer) (TimeSinceCaptureStarted :type Float%20%28single-precision%29) (ToRight :type Boolean))
  ;[1 1 1] struggle
  (CallFunction|Shake StruggleAttemptNum (+ StruggleAttemptNum StrugglesRemainingToEscape) ToRight))

(event Custom|OnCapturedActorEscape
  (params (StruggleAttemptNum :type Integer) (TimeSinceCaptureStarted :type Float%20%28single-precision%29) (ToRight :type Boolean))
  ;[1 1 1] escaped
  (Variables|spin|SetangularVelocity (/ (* (Variables|spin|GetkaijuDashSpeed) (* (Math|Float|SelectFloat 1.0 -1.0 ToRight) (Math|Float|SelectFloat 1.0 -1.0 (>= (.Z (Math|Vector|BreakVector (Variables|capture|GetgrabOffset))) 0.0)))) (Variables|spin|Getclaw%20radius)))
  (Variables|capture|Setescaped true)
  (Variables|spin|SetspinTime 0.0)
  (Variables|spin|SetmaxSpinTime (Math|Random|RandomFloatinRange 0.5 2.5))
  (bind _returnvalue (Class|SwarmV2|GetEnemySubsystem (Variables|Default|GetSwarmRef)))
  (Class|SwarmGrabManager|ReleaseGrabNumber (Variables|/Script/Neokaiju.EnemySubsystem|GetSwarmGrabManager _returnvalue) (Variables|capture|GetgrabNum))
  (CallFunction|StopGrabSound))

(event Custom|Shake
  (params (NumAttempts :type Integer) (MaxAttempts :type Integer) (ToRight :type Boolean))
  (bind _swarmref (Variables|Default|GetSwarmRef))
  (bind _targetkaiju (Variables|/Script/Neokaiju.SwarmV2|GetTargetKaiju _swarmref))
  (bind _returnvalue (Ability|GetAbilitySystemComponent _targetkaiju))
  ;[1 1 1] shake
  (Variables|spring|SetKweakness (/ (Math|Conversions|ToFloat(Integer) NumAttempts) (Math|Conversions|ToFloat(Integer) MaxAttempts)))
  (bind _output_get (Variables|spin|SetkaijuDashSpeed (* (/ (.ReturnValue (Ability|Attribute|GetFloatAttributefromAbilitySystemComponent _returnvalue "(AttributeName=\"DashDistance\",Attribute=StructProperty'\"/Script/Neokaiju.KaijuAttributeSet:DashDistance\"',AttributeOwner=Class'\"/Script/Neokaiju.KaijuAttributeSet\"')")) (.ReturnValue (Ability|Attribute|GetFloatAttributefromAbilitySystemComponent _returnvalue "(AttributeName=\"DashDuration\",Attribute=StructProperty'\"/Script/Neokaiju.KaijuAttributeSet:DashDuration\"',AttributeOwner=Class'\"/Script/Neokaiju.KaijuAttributeSet\"')"))) (Variables|/Script/Neokaiju.SwarmStats|GetGrabVelocityMultiplier (Variables|/Script/Neokaiju.SwarmV2|GetStats (Variables|Default|GetSwarmRef))))))
  (bind _returnvalue_2 (Class|SwarmV2|GetEnemySubsystem (Variables|Default|GetSwarmRef)))
  ;;[1 1 1] new v_0
  (bind _newvelocity (CallFunction|CalcCurrentVelocity (Variables|/Script/Neokaiju.SwarmGrabManager|GetcapturedTime (Variables|/Script/Neokaiju.EnemySubsystem|GetSwarmGrabManager _returnvalue_2))))
  (Class|SwarmGrabManager|SetCaptureVelocity (Variables|/Script/Neokaiju.EnemySubsystem|GetSwarmGrabManager _returnvalue_2) (+ _newvelocity (* _output_get (Math|Float|SelectFloat 1.0 -1.0 ToRight))) (Variables|capture|GetgrabNum))
  (Variables|spring|Setomega%20W (/ (Math|Float|Sqrt (- (* 4.0 (Variables|spring|Getkaiju%20M) (* (Variables|spring|Getgrab%20K) (Math|Float|Lerp 1.0 0.5 (Variables|spring|GetKweakness)))) (Math|Float|Square (Variables|spring|Getdrag%20D)))) (* 2 (Variables|spring|Getkaiju%20M))))
  (bind _returnvalue_3 (Class|SwarmV2|GetEnemySubsystem (Variables|Default|GetSwarmRef)))
  ;;[1 1 1] c1 = x_0
  (Variables|spring|Setc1 (Variables|/Script/Neokaiju.SwarmGrabManager|GetcapturedPosition (Variables|/Script/Neokaiju.EnemySubsystem|GetSwarmGrabManager _returnvalue_3)))
  ;;[1 1 1] c2  =  (v_0 - x_0 * a) / w
  (Variables|spring|Setc2 (/ (- (Variables|/Script/Neokaiju.SwarmGrabManager|GetcapturedVelocity (Variables|/Script/Neokaiju.EnemySubsystem|GetSwarmGrabManager _returnvalue_3)) (* (Variables|/Script/Neokaiju.SwarmGrabManager|GetcapturedPosition (Variables|/Script/Neokaiju.EnemySubsystem|GetSwarmGrabManager _returnvalue_3)) (Variables|spring|Getalpha%20A))) (Variables|spring|Getomega%20W)))
  (Class|SwarmGrabManager|SetCaptureTime (Variables|/Script/Neokaiju.EnemySubsystem|GetSwarmGrabManager _returnvalue_3) 0.0 (Variables|capture|GetgrabNum)))

(event EventEnter
  (params (NewSwarm :type Swarm%20V2%20Object%20Reference))
  (bind _swarmref (Variables|Default|GetSwarmRef))
  (bind _returnvalue (Transformation|GetActorTransform _swarmref))
  (bind _outerradius (Variables|/Script/Neokaiju.SwarmV2|GetOuterRadius _swarmref))
  (bind _targetkaiju (Variables|/Script/Neokaiju.SwarmV2|GetTargetKaiju _swarmref))
  ;[1 1 1] enter
  (|CallParentFunction NewSwarm)
  (CallFunction|InitCaptureVars)
  (bind _asbp_swarm_v2 (Utilities|Casting|CastToBP_SwarmV2 _swarmref)
    (:then
      (Transformation|SetRelativeLocation (Variables|/Game/NeoKaiju/Enemies/SwarmV2/BP_SwarmV2.BP_SwarmV2_C|GetCapturePoint _asbp_swarm_v2) (Math|Transform|InverseTransformLocation _returnvalue (Transformation|GetWorldLocation (Variables|/Script/Neokaiju.KaijuCharacter|GetAttachPosition _targetkaiju))) false false))
    (:CastFailed
      _))
  (Transformation|SetRelativeLocation _outerradius (Math|Transform|InverseTransformLocation _returnvalue (Transformation|GetActorLocation _targetkaiju)) false false)
  (Components|Sphere|SetSphereRadius _outerradius (Components|Capsule|GetScaledCapsuleRadius (Variables|/Script/Engine.Character|GetCapsuleComponent (Variables|/Script/Neokaiju.SwarmV2|GetTargetKaiju _swarmref))) true)
  (CallFunction|InitSpringVars)
  (bind _returnvalue_2 (Class|CaptureAbility|CaptureActor "/Game/NeoKaiju/Ability/EnvironmentAbilities/CaptureAbility/GA_CaptureAbility.GA_CaptureAbility_C" _swarmref (Variables|/Script/Neokaiju.SwarmV2|GetTargetKaiju _swarmref) (Variables|/Script/Neokaiju.SwarmStats|GetDashesToEscapeGrab (Variables|/Script/Neokaiju.SwarmV2|GetStats _swarmref))))
  (Variables|capture|Setescaped (not _returnvalue_2))
  (CallFunction|PlayGrabSound))

(event EventUpdate
  (params (DeltaTime :type Float%20%28single-precision%29))
  (bind _swarmref (Variables|Default|GetSwarmRef))
  ;[1 1 1] update
  (if (not (Variables|capture|Getescaped))
    (bind _returnvalue (Class|SwarmV2|GetEnemySubsystem (Variables|Default|GetSwarmRef)))
    ;;[1 1 1] If we don't have control skip to end (ensures only one swarm updates the position of the player)
    (if (!= (Variables|/Script/Neokaiju.SwarmGrabManager|GetcommandingSwarm (Variables|/Script/Neokaiju.EnemySubsystem|GetSwarmGrabManager _returnvalue)) (Variables|capture|GetgrabNum))
      _
      (else
        (bind _returnvalue_2 (Class|SwarmGrabManager|SetCaptureTime (Variables|/Script/Neokaiju.EnemySubsystem|GetSwarmGrabManager _returnvalue) (+ DeltaTime (Variables|/Script/Neokaiju.SwarmGrabManager|GetcapturedTime (Variables|/Script/Neokaiju.EnemySubsystem|GetSwarmGrabManager _returnvalue))) (Variables|capture|GetgrabNum)))
        (Class|SwarmGrabManager|SetCapturePosition (Variables|/Script/Neokaiju.EnemySubsystem|GetSwarmGrabManager _returnvalue) (* (Class|KismetMathLibrary|Exp (* _returnvalue_2 (Variables|spring|Getalpha%20A))) (+ (* (Math|Trig|Cos(Radians) (* _returnvalue_2 (Variables|spring|Getomega%20W))) (Variables|spring|Getc1)) (* (Math|Trig|Sin(Radians) (* _returnvalue_2 (Variables|spring|Getomega%20W))) (Variables|spring|Getc2)))) (Variables|capture|GetgrabNum))
        ;;[1 1 1] get new absolute position of kaiju
        (Transformation|SetActorLocation (Variables|/Script/Neokaiju.SwarmV2|GetTargetKaiju (Variables|Default|GetSwarmRef)) (+ (Variables|capture|GetinitGrabVector) (Math|Vector|MakeVector (Variables|/Script/Neokaiju.SwarmGrabManager|GetcapturedPosition (Variables|/Script/Neokaiju.EnemySubsystem|GetSwarmGrabManager _returnvalue)) 0.0 0.0)) false false)))
    ;;[1 1 1] set our new position
    (Transformation|SetActorLocation (Variables|Default|GetSwarmRef) (+ (+ (Variables|capture|GetinitGrabVector) (Math|Vector|MakeVector (Variables|/Script/Neokaiju.SwarmGrabManager|GetcapturedPosition (Variables|/Script/Neokaiju.EnemySubsystem|GetSwarmGrabManager _returnvalue)) 0.0 0.0)) (Variables|capture|GetgrabOffset)) false false)
    (elif (<= (Variables|spin|GetspinTime) (Variables|spin|GetmaxSpinTime))
      (Variables|spin|SetspinTime (+ (Variables|spin|GetspinTime) DeltaTime))
      (Class|Actor|AddActorWorldRotation (Variables|Default|GetSwarmRef) (Math|Rotator|MakeRotator 0.0 (* DeltaTime (Variables|spin|GetangularVelocity)) 0.0))
      (else
        (bind _returnvalue_3 (Game|ConstructObjectfromClass "/Game/NeoKaiju/Enemies/SwarmV2/States/BP_Dissassemble.BP_Dissassemble_C" _swarmref))
        (Class|SwarmV2|ChangeState _swarmref _returnvalue_3)))))

(event EventExit
  (bind _swarmref (Variables|Default|GetSwarmRef))
  ;[1 1 1] exit
  (Transformation|SetRelativeLocation (Variables|/Script/Neokaiju.SwarmV2|GetOuterRadius (Variables|Default|GetSwarmRef)) "0, 0, 0" false false)
  (if (not (Variables|capture|Getescaped))
    (Class|CaptureAbility|ReleaseActor _swarmref (Variables|/Script/Neokaiju.SwarmV2|GetTargetKaiju _swarmref))
    (bind _returnvalue (Class|SwarmV2|GetEnemySubsystem (Variables|Default|GetSwarmRef)))
    (Class|SwarmGrabManager|ReleaseGrabNumber (Variables|/Script/Neokaiju.EnemySubsystem|GetSwarmGrabManager _returnvalue) (Variables|capture|GetgrabNum))))

(event EventOnInnerBeginOverlap
  (params (OverlappedComponent :type Primitive%20Component%20Object%20Reference) (OtherActor :type Actor%20Object%20Reference) (OtherComp :type Primitive%20Component%20Object%20Reference) (OtherBodyIndex :type Integer) (FromSweep :type Boolean) (SweepResult :type Hit%20Result%20Structure))
  ;[1 1 1] character slammed swarm into wall
  (if (not (== OtherActor (Variables|/Script/Neokaiju.SwarmV2|GetTargetKaiju (Variables|Default|GetSwarmRef))))
    _))

(event EventOnOuterBeginOverlap
  (params (OverlappedComponent :type Primitive%20Component%20Object%20Reference) (OtherActor :type Actor%20Object%20Reference) (OtherComp :type Primitive%20Component%20Object%20Reference) (OtherBodyIndex :type Integer) (FromSweep :type Boolean) (SweepResult :type Hit%20Result%20Structure))
  ;[1 1 1] character slammed themselves into wall
  (if (not (== OtherActor (Variables|/Script/Neokaiju.SwarmV2|GetTargetKaiju (Variables|Default|GetSwarmRef))))
    (bind _returnvalue (Class|SwarmV2|GetEnemySubsystem (Variables|Default|GetSwarmRef)))
    ;[1 1 1] set velocity and time to 0, then recalc c1 and c2
    (Class|SwarmGrabManager|SetCaptureVelocity (Variables|/Script/Neokaiju.EnemySubsystem|GetSwarmGrabManager _returnvalue) 0.0 (Variables|capture|GetgrabNum))
    ;[1 1 1] c1 = x_0
    (Variables|spring|Setc1 (Variables|/Script/Neokaiju.SwarmGrabManager|GetcapturedPosition (Variables|/Script/Neokaiju.EnemySubsystem|GetSwarmGrabManager _returnvalue)))
    ;[1 1 1] c2  =  (v_0 - x_0 * a) / w
    (Variables|spring|Setc2 (/ (- 0.0 (* (Variables|/Script/Neokaiju.SwarmGrabManager|GetcapturedPosition (Variables|/Script/Neokaiju.EnemySubsystem|GetSwarmGrabManager _returnvalue)) (Variables|spring|Getalpha%20A))) (Variables|spring|Getomega%20W)))
    (Class|SwarmGrabManager|SetCaptureTime (Variables|/Script/Neokaiju.EnemySubsystem|GetSwarmGrabManager _returnvalue) 0.0 (Variables|capture|GetgrabNum))))

(fn InitSpringVars
  (Variables|spring|Setdrag%20D (* 0.5 (Variables|drag|GetDragCoeficient) (Variables|drag|GetdensityOfAir) (Variables|drag|GetdragOffsetCoeficient)))
  (Variables|spring|Setgrab%20K (Variables|/Script/Neokaiju.SwarmStats|GetGrabKValue (Variables|/Script/Neokaiju.SwarmV2|GetStats (Variables|Default|GetSwarmRef))))
  (Variables|spring|Setalpha%20A (/ (* -1.0 (Variables|spring|Getdrag%20D)) (* 2 (Variables|spring|Getkaiju%20M))))
  (Variables|spring|SetKweakness 0.0)
  (Variables|spring|Setomega%20W (/ (Math|Float|Sqrt (- (* 4.0 (Variables|spring|Getkaiju%20M) (* (Variables|spring|Getgrab%20K) (Math|Float|Lerp 1.0 0.5 (Variables|spring|GetKweakness)))) (Math|Float|Square (Variables|spring|Getdrag%20D)))) (* 2 (Variables|spring|Getkaiju%20M))))
  (bind _returnvalue (Class|SwarmV2|GetEnemySubsystem (Variables|Default|GetSwarmRef)))
  ;[1 1 1] c1 = x_0
  (Variables|spring|Setc1 (Variables|/Script/Neokaiju.SwarmGrabManager|GetcapturedPosition (Variables|/Script/Neokaiju.EnemySubsystem|GetSwarmGrabManager _returnvalue)))
  ;[1 1 1] c2  =  (v_0 - x_0 * a) / w
  (Variables|spring|Setc2 (/ (- (Variables|/Script/Neokaiju.SwarmGrabManager|GetcapturedVelocity (Variables|/Script/Neokaiju.EnemySubsystem|GetSwarmGrabManager _returnvalue)) (* (Variables|/Script/Neokaiju.SwarmGrabManager|GetcapturedPosition (Variables|/Script/Neokaiju.EnemySubsystem|GetSwarmGrabManager _returnvalue)) (Variables|spring|Getalpha%20A))) (Variables|spring|Getomega%20W)))
  (return false))

(fn InitCaptureVars
  (bind _swarmref (Variables|Default|GetSwarmRef))
  (bind _targetkaiju (Variables|/Script/Neokaiju.SwarmV2|GetTargetKaiju _swarmref))
  (bind _returnvalue (Transformation|GetActorLocation _targetkaiju))
  (bind _returnvalue_2 (Class|SwarmV2|GetEnemySubsystem (Variables|Default|GetSwarmRef)))
  (bind _returnvalue_3 (Class|SwarmGrabManager|ObtainGrabNumber (Variables|/Script/Neokaiju.EnemySubsystem|GetSwarmGrabManager _returnvalue_2)))
  (bind _output_get (Variables|capture|SetgrabNum _returnvalue_3))
  (bind _returnvalue_4 (Class|SwarmGrabManager|SetCaptureInitPosition (Variables|/Script/Neokaiju.EnemySubsystem|GetSwarmGrabManager _returnvalue_2) _returnvalue _output_get))
  (Variables|capture|SetinitGrabVector _returnvalue_4)
  (Variables|capture|SetgrabOffset (- (Transformation|GetActorLocation _swarmref) _returnvalue))
  ;[1 1 1] x_0
  (Class|SwarmGrabManager|SetCapturePosition (Variables|/Script/Neokaiju.EnemySubsystem|GetSwarmGrabManager _returnvalue_2) 0.0 (Variables|capture|GetgrabNum))
  ;[1 1 1] v_0
  (Class|SwarmGrabManager|SetCaptureVelocity (Variables|/Script/Neokaiju.EnemySubsystem|GetSwarmGrabManager _returnvalue_2) 0.0 (Variables|capture|GetgrabNum))
  ;[1 1 1] a_0
  (Class|SwarmGrabManager|SetCaptureAcceleration (Variables|/Script/Neokaiju.EnemySubsystem|GetSwarmGrabManager _returnvalue_2) 0.0 (Variables|capture|GetgrabNum))
  ;[1 1 1] t
  (Class|SwarmGrabManager|SetCaptureTime (Variables|/Script/Neokaiju.EnemySubsystem|GetSwarmGrabManager _returnvalue_2) 0.0 (Variables|capture|GetgrabNum))
  (return false))

(fn CalcCurrentVelocity
  (params (currentTime :type Float%20%28single-precision%29))
  (bind _omega_w (Variables|spring|Getomega%20W))
  (bind _returnvalue (* currentTime _omega_w))
  (return (* (Class|KismetMathLibrary|Exp (* currentTime (Variables|spring|Getalpha%20A))) (+ (* (Math|Trig|Cos(Radians) _returnvalue) (+ (* (Variables|spring|Getc1) (Variables|spring|Getalpha%20A)) (* (Variables|spring|Getc2) (Variables|spring|Getomega%20W)))) (* (Math|Trig|Sin(Radians) _returnvalue) (+ (* -1.0 (Variables|spring|Getc1) (Variables|spring|Getomega%20W)) (* (Variables|spring|Getc2) (Variables|spring|Getalpha%20A))))))))

(fn PlayGrabSound
  (if (not (Variables|capture|Getescaped))
    (bind _returnvalue (Class|FMODBlueprintStatics|PlayEventatLocation "/Game/Neokaiju/Audio/Events/Environment/Swarm_GrabHold.Swarm_GrabHold" (Math|Conversions|ToTransform(Vector) (Transformation|GetActorLocation (Variables|Default|GetSwarmRef)))))
    (Variables|Default|SetGrabSound _returnvalue)))

(fn StopGrabSound
  (bind _returnvalue (Class|FMODBlueprintStatics|EventInstanceIsValid (Variables|Default|GetGrabSound)))
  (if _returnvalue
    (Class|FMODBlueprintStatics|EventInstanceStop (Variables|Default|GetGrabSound) true)))