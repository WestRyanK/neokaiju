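; Chase state for the V2 enemy swarm, which pursues the target kaiju until it can circle it.
; Each update steers by averaging the last direction with the direction to the kaiju, passes it through FindOpenSpace, then moves, orients and rotates the swarm.
; It switches to Circle at the outer radius, Idle beyond pursuit range, or Scatter when the kaiju enters the inner radius with its Dash cooldown tag.
; Laser events are empty.
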(event EventEnter
  (params (NewSwarm :type Swarm%20V2%20Object%20Reference))
  (bind _swarmref (Variables|Default|GetSwarmRef))
  (bind _stats (Variables|/Script/Neokaiju.SwarmV2|GetStats _swarmref))
  (bind _chasebegincircleradius (Variables|/Script/Neokaiju.SwarmStats|GetChaseBeginCircleRadius _stats))
  (|CallParentFunction NewSwarm)
  ;[1 1 1] if it's already close enough go straight to the point
  (if (<= (Transformation|GetDistanceTo (Variables|/Script/Neokaiju.SwarmV2|GetTargetKaiju _swarmref) _swarmref) _chasebegincircleradius)
    (Class|SwarmState|OnOuterBeginOverlap 0 (Variables|/Script/Neokaiju.SwarmV2|GetTargetKaiju (Variables|Default|GetSwarmRef)) 0 0 false))
  (Components|Sphere|SetSphereRadius (Variables|/Script/Neokaiju.SwarmV2|GetOuterRadius _swarmref) _chasebegincircleradius true))

(event EventUpdate
  (params (DeltaTime :type Float%20%28single-precision%29))
  (bind _swarmref (Variables|Default|GetSwarmRef))
  (bind _swarmref_2 (Variables|Default|GetSwarmRef))
  (bind _swarmref_3 (Variables|Default|GetSwarmRef))
  (bind _swarmref_4 (Variables|Default|GetSwarmRef))
  (bind _returnvalue (Transformation|GetActorLocation _swarmref_2))
  (bind _targetkaiju (Variables|/Script/Neokaiju.SwarmV2|GetTargetKaiju _swarmref_2))
  (bind _returnvalue_2 (Transformation|GetActorLocation _targetkaiju))
  (bind _returnvalue_3 (- _returnvalue_2 _returnvalue))
  (bind _returnvalue_4 (Math|Vector|VectorLength _returnvalue_3))
  ;[1 1 1] go back to idle if the player gets too far away
  (if (< _returnvalue_4 (Variables|/Script/Neokaiju.SwarmStats|GetChaseEndPursuitRadius (Variables|/Script/Neokaiju.SwarmV2|GetStats (Variables|Default|GetSwarmRef))))
    (bind _returnvalue_5 (Class|SwarmV2|FindOpenSpace (Variables|Default|GetSwarmRef) (/ (+ (Variables|/Script/Neokaiju.SwarmV2|GetLastDirection (Variables|Default|GetSwarmRef)) (Math|Vector|Normalize _returnvalue_3)) (Math|Float|SelectFloat 1.0 2.0 (Math|Vector|Equal(Vector) (Variables|/Script/Neokaiju.SwarmV2|GetLastDirection (Variables|Default|GetSwarmRef)) "0, 0, 0" 0.001))) _returnvalue_4))
    (bind _output_get (Variables|/Script/Neokaiju.SwarmV2|SetLastDirection _swarmref_4 _returnvalue_5))
    (Class|SwarmV2|Move _swarmref_4 DeltaTime (Variables|/Script/Neokaiju.SwarmStats|GetChaseSpeed (Variables|/Script/Neokaiju.SwarmV2|GetStats _swarmref_4)) _output_get)
    (Class|SwarmV2|OrientSwarm _swarmref_3 (Math|Rotator|MakeRotfromZ _returnvalue_3))
    (Class|SwarmV2|RotateSwarm _swarmref_3 DeltaTime)
    (else
      (bind _returnvalue_6 (Game|ConstructObjectfromClass "/Game/NeoKaiju/Enemies/SwarmV2/States/BP_Idle.BP_Idle_C" _swarmref))
      (Class|SwarmV2|ChangeState _swarmref _returnvalue_6))))

(event EventOnOuterBeginOverlap
  (params (OverlappedComponent :type Primitive%20Component%20Object%20Reference) (OtherActor :type Actor%20Object%20Reference) (OtherComp :type Primitive%20Component%20Object%20Reference) (OtherBodyIndex :type Integer) (FromSweep :type Boolean) (SweepResult :type Hit%20Result%20Structure))
  (bind _swarmref (Variables|Default|GetSwarmRef))
  (if (== OtherActor (Variables|/Script/Neokaiju.SwarmV2|GetTargetKaiju _swarmref))
    (bind _returnvalue (Game|ConstructObjectfromClass "/Game/NeoKaiju/Enemies/SwarmV2/States/BP_Circle.BP_Circle_C" _swarmref))
    (Class|SwarmV2|ChangeState _swarmref _returnvalue)))

(event EventOnBeginHitbyLaser)

(event EventOnInnerBeginOverlap
  (params (OverlappedComponent :type Primitive%20Component%20Object%20Reference) (OtherActor :type Actor%20Object%20Reference) (OtherComp :type Primitive%20Component%20Object%20Reference) (OtherBodyIndex :type Integer) (FromSweep :type Boolean) (SweepResult :type Hit%20Result%20Structure))
  (bind _swarmref (Variables|Default|GetSwarmRef))
  (bind _swarmref_2 (Variables|Default|GetSwarmRef))
  (bind _targetkaiju (Variables|/Script/Neokaiju.SwarmV2|GetTargetKaiju _swarmref))
  (if (and (== OtherActor _targetkaiju) (GameplayTags|HasMatchingGameplayTag (Ability|GetAbilitySystemComponent _targetkaiju) "(TagName=\"Cooldown.Ability.Standard.Dash\")"))
    (bind _returnvalue (Game|ConstructObjectfromClass "/Game/NeoKaiju/Enemies/SwarmV2/States/BP_Scatter.BP_Scatter_C" _swarmref_2))
    (Variables|/Game/NeoKaiju/Enemies/SwarmV2/States/BP_Scatter.BP_Scatter_C|SetscatterByLazer _returnvalue false)
    (Class|SwarmV2|ChangeState _swarmref_2 _returnvalue)))

(event EventOnBeginOverlapbyLaser)

(event EventOnEndOverlapbyLaser)

(event EventExit)