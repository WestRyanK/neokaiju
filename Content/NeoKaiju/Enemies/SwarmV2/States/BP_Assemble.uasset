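; BP_Assemble is a SwarmV2 enemy state that assembles the swarm into its bullet form before handing off to aiming.
; Enter turns off claw mode, shows the bullet mesh with a glow material and sets the spin multiplier.
; Update rotates and assembles the swarm over the stats-driven transform time, then switches to a new BP_Aim state.
; Exit restores the enemy material and makes the inner radius block a custom trace channel.
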(event EventEnter
  (params (NewSwarm :type Swarm%20V2%20Object%20Reference))
  (bind _swarmref (Variables|Default|GetSwarmRef))
  (bind _swarmref_2 (Variables|Default|GetSwarmRef))
  (|CallParentFunction NewSwarm)
  (Variables|Default|SettransformTime 0.0)
  (Variables|/Script/Neokaiju.SwarmV2|SetClawMode (Variables|Default|GetSwarmRef) false)
  (Rendering|SetVisibility (select (Variables|/Script/Neokaiju.SwarmV2|GetClawMode _swarmref_2) (Variables|/Script/Neokaiju.SwarmV2|GetClawMesh _swarmref_2) (Variables|/Script/Neokaiju.SwarmV2|GetBulletMesh _swarmref_2)) true false)
  (bind _asstatic_mesh_component (Utilities|Casting|CastToStaticMeshComponent (select (Variables|/Script/Neokaiju.SwarmV2|GetClawMode _swarmref_2) (Variables|/Script/Neokaiju.SwarmV2|GetClawMesh _swarmref_2) (Variables|/Script/Neokaiju.SwarmV2|GetBulletMesh _swarmref_2)))
    (:then
      (Rendering|Material|SetMaterial _asstatic_mesh_component 0 "/Game/NeoKaiju/Enemies/Swarm/M_swarmGlow.M_swarmGlow"))
    (:CastFailed
      _))
  (bind _asbp_swarm_v2 (Utilities|Casting|CastToBP_SwarmV2 _swarmref))
  (Variables|/Game/NeoKaiju/Enemies/SwarmV2/BP_SwarmV2.BP_SwarmV2_C|SetRotationMultiplier _asbp_swarm_v2 (Variables|/Script/Neokaiju.SwarmStats|GetLazerReactionSpin (Variables|/Script/Neokaiju.SwarmV2|GetStats _swarmref))))

(event EventUpdate
  (params (DeltaTime :type Float%20%28single-precision%29))
  (bind _swarmref (Variables|Default|GetSwarmRef))
  (bind _swarmref_2 (Variables|Default|GetSwarmRef))
  (if (<= (Variables|Default|GettransformTime) (Variables|/Script/Neokaiju.SwarmStats|GetTransformTime (Variables|/Script/Neokaiju.SwarmV2|GetStats (Variables|Default|GetSwarmRef))))
    (Class|SwarmV2|RotateSwarm _swarmref_2 DeltaTime)
    (Class|SwarmV2|AssembleSwarm _swarmref_2 (Variables|Default|GettransformTime) (Variables|/Script/Neokaiju.SwarmStats|GetTransformTime (Variables|/Script/Neokaiju.SwarmV2|GetStats _swarmref_2)))
    (Variables|Default|SettransformTime (+ (Variables|Default|GettransformTime) DeltaTime))
    (else
      (bind _returnvalue (Game|ConstructObjectfromClass "/Game/NeoKaiju/Enemies/SwarmV2/States/BP_Aim.BP_Aim_C" _swarmref))
      (Class|SwarmV2|ChangeState _swarmref _returnvalue))))

(event EventExit
  (bind _swarmref (Variables|Default|GetSwarmRef))
  (bind _asstatic_mesh_component (Utilities|Casting|CastToStaticMeshComponent (select (Variables|/Script/Neokaiju.SwarmV2|GetClawMode _swarmref) (Variables|/Script/Neokaiju.SwarmV2|GetClawMesh _swarmref) (Variables|/Script/Neokaiju.SwarmV2|GetBulletMesh _swarmref))))
  (Rendering|Material|SetMaterial _asstatic_mesh_component 0 "/Game/NeoKaiju/Structures/Textures/M_Enemies.M_Enemies")
  (Collision|SetCollisionResponsetoChannel (Variables|/Script/Neokaiju.SwarmV2|GetInnerRadius (Variables|Default|GetSwarmRef)) "ECC_GameTraceChannel2" "ECR_Block"))