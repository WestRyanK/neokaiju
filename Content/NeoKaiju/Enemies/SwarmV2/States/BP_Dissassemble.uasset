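; BP_Dissassemble is a swarm enemy state that breaks the swarm out of its claw or bullet form, then switches to BP_Chase.
; Enter applies a glow material to the active form's mesh.
; Update rotates and dissembles the swarm over the stats' transform time before constructing the chase state.
; Exit sets inner-radius collision to overlap, hides the mesh, restores its enemy material and resets spin to normal.
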(event EventEnter
  (params (NewSwarm :type Swarm%20V2%20Object%20Reference))
  (bind _swarmref (Variables|Default|GetSwarmRef))
  (|CallParentFunction NewSwarm)
  (Variables|Default|SettransformTime 0.0)
  (bind _asstatic_mesh_component (Utilities|Casting|CastToStaticMeshComponent (select (Variables|/Script/Neokaiju.SwarmV2|GetClawMode _swarmref) (Variables|/Script/Neokaiju.SwarmV2|GetClawMesh _swarmref) (Variables|/Script/Neokaiju.SwarmV2|GetBulletMesh _swarmref))))
  (Rendering|Material|SetMaterial _asstatic_mesh_component 0 "/Game/NeoKaiju/Enemies/Swarm/M_swarmGlow.M_swarmGlow"))

(event EventUpdate
  (params (DeltaTime :type Float%20%28single-precision%29))
  (bind _swarmref (Variables|Default|GetSwarmRef))
  (bind _swarmref_2 (Variables|Default|GetSwarmRef))
  (if (<= (Variables|Default|GettransformTime) (Variables|/Script/Neokaiju.SwarmStats|GetTransformTime (Variables|/Script/Neokaiju.SwarmV2|GetStats (Variables|Default|GetSwarmRef))))
    (Class|SwarmV2|RotateSwarm _swarmref_2 DeltaTime)
    (Class|SwarmV2|DissembleSwarm _swarmref_2 (Variables|Default|GettransformTime) (Variables|/Script/Neokaiju.SwarmStats|GetTransformTime (Variables|/Script/Neokaiju.SwarmV2|GetStats _swarmref_2)))
    (Variables|Default|SettransformTime (+ (Variables|Default|GettransformTime) DeltaTime))
    (else
      (bind _returnvalue (Game|ConstructObjectfromClass "/Game/NeoKaiju/Enemies/SwarmV2/States/BP_Chase.BP_Chase_C" _swarmref))
      (Class|SwarmV2|ChangeState _swarmref _returnvalue))))

(event EventExit
  (bind _swarmref (Variables|Default|GetSwarmRef))
  (bind _swarmref_2 (Variables|Default|GetSwarmRef))
  (bind _clawmesh (Variables|/Script/Neokaiju.SwarmV2|GetClawMesh _swarmref))
  (bind _bulletmesh (Variables|/Script/Neokaiju.SwarmV2|GetBulletMesh _swarmref))
  (bind _clawmode (Variables|/Script/Neokaiju.SwarmV2|GetClawMode _swarmref))
  (bind _returnvalue (select _clawmode _clawmesh _bulletmesh))
  (Collision|SetCollisionResponsetoChannel (Variables|/Script/Neokaiju.SwarmV2|GetInnerRadius (Variables|Default|GetSwarmRef)) "ECC_GameTraceChannel2" "ECR_Overlap")
  (Rendering|SetVisibility _returnvalue false false)
  (bind _asstatic_mesh_component (Utilities|Casting|CastToStaticMeshComponent _returnvalue)
    (:then
      (Rendering|Material|SetMaterial _asstatic_mesh_component 0 "/Game/NeoKaiju/Structures/Textures/M_Enemies.M_Enemies"))
    (:CastFailed
      _))
  (bind _asbp_swarm_v2 (Utilities|Casting|CastToBP_SwarmV2 _swarmref_2))
  (Variables|/Game/NeoKaiju/Enemies/SwarmV2/BP_SwarmV2.BP_SwarmV2_C|SetRotationMultiplier _asbp_swarm_v2 (Variables|/Script/Neokaiju.SwarmStats|GetNormalSpin (Variables|/Script/Neokaiju.SwarmV2|GetStats _swarmref_2))))