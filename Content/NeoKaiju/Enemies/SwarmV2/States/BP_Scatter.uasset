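; BP_Scatter is a swarm enemy state that scatters the swarm outward, holds it, reassembles it, then switches to BP_Chase.
; Update runs the disperse, wait and assemble phases on timers against the swarm's Stats, driving ScatterSwarmOut and ScatterSwarmIn.
; Laser hit or overlap pauses the wait until it ends.
; A new laser contact restarts the wait, or converts assembly progress into dispersal time to reverse mid-assembly.
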(event EventEnter
  (params (NewSwarm :type Swarm%20V2%20Object%20Reference))
  (|CallParentFunction NewSwarm)
  (Variables|Default|Setscatter_out_time 0.0)
  (Variables|Default|Setlaser_ended (not (Variables|Default|GetscatterByLazer)))
  (Variables|Default|Setscatter_time 0.0)
  (Variables|Default|Setscatter_in_time 0.0))

(event EventOnEndHitbyLaser
  (Variables|Default|Setlaser_ended true))

(event EventUpdate
  (params (DeltaTime :type Float%20%28single-precision%29))
  (bind _swarmref (Variables|Default|GetSwarmRef))
  (bind _swarmref_2 (Variables|Default|GetSwarmRef))
  (bind _swarmref_3 (Variables|Default|GetSwarmRef))
  (bind _stats (Variables|/Script/Neokaiju.SwarmV2|GetStats _swarmref))
  (bind _stats_2 (Variables|/Script/Neokaiju.SwarmV2|GetStats _swarmref_3))
  (bind _scatterassembletime (Variables|/Script/Neokaiju.SwarmStats|GetScatterAssembleTime _stats))
  (bind _scatterdispersetime (Variables|/Script/Neokaiju.SwarmStats|GetScatterDisperseTime _stats_2))
  ;[1 1 1] scatter out
  (bind _output_get (Variables|Default|SetDeltaTime DeltaTime))
  (if (<= (Variables|Default|Getscatter_out_time) _scatterdispersetime)
    (Class|SwarmV2|ScatterSwarmOut (Variables|Default|GetSwarmRef) (Variables|Default|Getscatter_out_time) _scatterdispersetime)
    (Variables|Default|Setscatter_out_time (+ (Variables|Default|Getscatter_out_time) _output_get))
    (else
      ;[1 1 1] scatter wait
      (if (Variables|Default|Getlaser_ended)
        (if (<= (Variables|Default|Getscatter_time) (Variables|/Script/Neokaiju.SwarmStats|GetScatterTime (Variables|/Script/Neokaiju.SwarmV2|GetStats (Variables|Default|GetSwarmRef))))
          (Variables|Default|Setscatter_time (+ (Variables|Default|Getscatter_time) (Variables|Default|GetDeltaTime)))
          (else
            ;[1 1 1] scatter in
            (if (<= (Variables|Default|Getscatter_in_time) _scatterassembletime)
              (Class|SwarmV2|ScatterSwarmin (Variables|Default|GetSwarmRef) (Variables|Default|Getscatter_in_time) _scatterassembletime)
              (Variables|Default|Setscatter_in_time (+ (Variables|Default|Getscatter_in_time) (Variables|Default|GetDeltaTime)))
              (else
                (bind _returnvalue (Game|ConstructObjectfromClass "/Game/NeoKaiju/Enemies/SwarmV2/States/BP_Chase.BP_Chase_C" _swarmref_2))
                (Class|SwarmV2|ChangeState _swarmref_2 _returnvalue)))))))))

(event EventOnBeginHitbyLaser
  (bind _swarmref (Variables|Default|GetSwarmRef))
  (bind _stats (Variables|/Script/Neokaiju.SwarmV2|GetStats _swarmref))
  (bind _scatterassembletime (Variables|/Script/Neokaiju.SwarmStats|GetScatterAssembleTime _stats))
  (Variables|Default|Setlaser_ended false)
  (if (not (<= (Variables|Default|Getscatter_out_time) (Variables|/Script/Neokaiju.SwarmStats|GetScatterDisperseTime _stats)))
    (if (<= (Variables|Default|Getscatter_time) (Variables|/Script/Neokaiju.SwarmStats|GetScatterTime _stats))
      (Variables|Default|Setscatter_time 0.0)
      (elif (<= (Variables|Default|Getscatter_in_time) _scatterassembletime)
        (Variables|Default|Setscatter_time 0.0)
        (Variables|Default|Setscatter_out_time (* (/ (Variables|Default|Getscatter_in_time) _scatterassembletime) (Variables|/Script/Neokaiju.SwarmStats|GetScatterDisperseTime _stats)))
        (Variables|Default|Setscatter_in_time 0.0)))))

(event EventOnBeginOverlapbyLaser
  (bind _swarmref (Variables|Default|GetSwarmRef))
  (bind _stats (Variables|/Script/Neokaiju.SwarmV2|GetStats _swarmref))
  (bind _scatterassembletime (Variables|/Script/Neokaiju.SwarmStats|GetScatterAssembleTime _stats))
  (Variables|Default|Setlaser_ended false)
  (if (not (<= (Variables|Default|Getscatter_out_time) (Variables|/Script/Neokaiju.SwarmStats|GetScatterDisperseTime _stats)))
    (if (<= (Variables|Default|Getscatter_time) (Variables|/Script/Neokaiju.SwarmStats|GetScatterTime _stats))
      (Variables|Default|Setscatter_time 0.0)
      (elif (<= (Variables|Default|Getscatter_in_time) _scatterassembletime)
        (Variables|Default|Setscatter_time 0.0)
        (Variables|Default|Setscatter_out_time (* (/ (Variables|Default|Getscatter_in_time) _scatterassembletime) (Variables|/Script/Neokaiju.SwarmStats|GetScatterDisperseTime _stats)))
        (Variables|Default|Setscatter_in_time 0.0)))))

(event EventOnEndOverlapbyLaser
  (Variables|Default|Setlaser_ended true))