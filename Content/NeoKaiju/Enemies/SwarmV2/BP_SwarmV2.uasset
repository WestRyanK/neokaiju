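; Swarm enemy that targets the player's Kaiju, built from randomized orbiting particle clusters on a spinning hook.
; State objects (starting at BP_Idle) receive forwarded overlap, laser and grab-struggle events.
; Helpers scatter the swarm, scale-morph it into a bullet or claw mesh, and sphere-trace candidate directions for open space.
; Laser damage scales with a player ability attribute, updates the health bar and triggers exploding death at zero health.
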(event OnComponentBeginOverlap(OuterRadius)
  (params (OverlappedComponent :type Primitive%20Component%20Object%20Reference) (OtherActor :type Actor%20Object%20Reference) (OtherComp :type Primitive%20Component%20Object%20Reference) (OtherBodyIndex :type Integer) (bFromSweep :type Boolean) (SweepResult :type Hit%20Result%20Structure%20%28by%20ref%29))
  (bind _currentstate (Variables|Default|GetCurrentState))
  (Utilities|IsValid _currentstate
    (:Is%20Valid
      (Class|SwarmState|OnOuterBeginOverlap _currentstate OverlappedComponent OtherActor OtherComp OtherBodyIndex bFromSweep SweepResult))))

(event OnComponentEndOverlap(OuterRadius)
  (params (OverlappedComponent :type Primitive%20Component%20Object%20Reference) (OtherActor :type Actor%20Object%20Reference) (OtherComp :type Primitive%20Component%20Object%20Reference) (OtherBodyIndex :type Integer))
  (bind _currentstate (Variables|Default|GetCurrentState))
  (Utilities|IsValid _currentstate
    (:Is%20Valid
      (Class|SwarmState|OnOuterEndOverlap _currentstate OverlappedComponent OtherActor OtherComp OtherBodyIndex))))

(event OnComponentBeginOverlap(InnerRadius)
  (params (OverlappedComponent :type Primitive%20Component%20Object%20Reference) (OtherActor :type Actor%20Object%20Reference) (OtherComp :type Primitive%20Component%20Object%20Reference) (OtherBodyIndex :type Integer) (bFromSweep :type Boolean) (SweepResult :type Hit%20Result%20Structure%20%28by%20ref%29))
  (bind _currentstate (Variables|Default|GetCurrentState))
  (Utilities|IsValid _currentstate
    (:Is%20Valid
      (Class|SwarmState|OnInnerBeginOverlap _currentstate OverlappedComponent OtherActor OtherComp OtherBodyIndex bFromSweep SweepResult))))

(event OnComponentEndOverlap(InnerRadius)
  (params (OverlappedComponent :type Primitive%20Component%20Object%20Reference) (OtherActor :type Actor%20Object%20Reference) (OtherComp :type Primitive%20Component%20Object%20Reference) (OtherBodyIndex :type Integer))
  (bind _currentstate (Variables|Default|GetCurrentState))
  (Utilities|IsValid _currentstate
    (:Is%20Valid
      (Class|SwarmState|OnInnerEndOverlap _currentstate OverlappedComponent OtherActor OtherComp OtherBodyIndex))))

(event OnComponentBeginOverlap(BulletMesh)
  (params (OverlappedComponent :type Primitive%20Component%20Object%20Reference) (OtherActor :type Actor%20Object%20Reference) (OtherComp :type Primitive%20Component%20Object%20Reference) (OtherBodyIndex :type Integer) (bFromSweep :type Boolean) (SweepResult :type Hit%20Result%20Structure%20%28by%20ref%29))
  ;[1 1 1] only one mesh should be set to have collision on at a time (if any are)
  (bind _asbp_attack (Utilities|Casting|CastToBP_Attack (Variables|Default|GetCurrentState)))
  (Default|OnMeshBeginOverlap _asbp_attack OverlappedComponent OtherActor OtherComp OtherBodyIndex bFromSweep SweepResult))

(event OnComponentBeginOverlap(ClawMesh)
  (params (OverlappedComponent :type Primitive%20Component%20Object%20Reference) (OtherActor :type Actor%20Object%20Reference) (OtherComp :type Primitive%20Component%20Object%20Reference) (OtherBodyIndex :type Integer) (bFromSweep :type Boolean) (SweepResult :type Hit%20Result%20Structure%20%28by%20ref%29))
  ;[1 1 1] only one mesh should be set to have collision on at a time (if any are)
  (bind _asbp_attack (Utilities|Casting|CastToBP_Attack (Variables|Default|GetCurrentState)))
  (Default|OnMeshBeginOverlap _asbp_attack OverlappedComponent OtherActor OtherComp OtherBodyIndex bFromSweep SweepResult))

(event Custom|DealDamage
  (params (Damage :type Float%20%28single-precision%29))
  (bind _output_get (Variables|Default|SetHealth (- (Variables|Default|GetHealth) Damage)))
  (Default|UpdateHealth (Variables|Default|GetHealthBarRef) (/ _output_get (Variables|/Script/Neokaiju.SwarmStats|GetTimeForLazerToKill (Variables|Default|GetStats))))
  (CallFunction|ShowHealthBar)
  (if (<= _output_get 0.0)
    (Class|SwarmV2|KillSwarm)))

(event Custom|HideHealthBar
  (Rendering|SetVisibility (Variables|Default|GetHealthBar) false false))

(event Custom|ShowHealthBar
  (Rendering|SetVisibility (Variables|Default|GetHealthBar) true false))

(event EventBeginPlay
  (Variables|Default|SetHealth (Variables|/Script/Neokaiju.SwarmStats|GetTimeForLazerToKill (Variables|Default|GetStats)))
  (bind _asswarm_healthbar (Utilities|Casting|CastToSwarm_Healthbar (UserInterface|GetUserWidgetObject (Variables|Default|GetHealthBar))))
  (bind _output_get (Variables|Default|SetHealthBarRef _asswarm_healthbar))
  (Default|UpdateHealth _output_get 1.0))

(event Collision|EventActorBeginOverlap
  (params (OtherActor :type Actor%20Object%20Reference)))

(event EventDissembleSwarm
  (params (transformTime :type Float%20%28single-precision%29) (totalTransformTime :type Float%20%28single-precision%29))
  (bind _returnvalue (/ transformTime totalTransformTime))
  (bind _returnvalue_2 (- 1.0 _returnvalue))
  ;[1 1 1] dissemble swarm
  (Transformation|SetRelativeScale3D (Variables|Default|GetswarmHook) (Math|Vector|MakeVector _returnvalue _returnvalue _returnvalue))
  (Transformation|SetRelativeScale3D (select (Variables|Default|GetClawMode) (Variables|Default|GetClawMesh) (Variables|Default|GetBulletMesh)) (Math|Vector|MakeVector _returnvalue_2 _returnvalue_2 _returnvalue_2)))

(event EventScatterSwarmOut
  (params (scatterTime :type Float%20%28single-precision%29) (totalScatterTime :type Float%20%28single-precision%29))
  (bind _returnvalue (/ scatterTime totalScatterTime))
  (bind _stats (Variables|Default|GetStats))
  (bind _swarmenemies (Variables|Default|GetSwarmEnemies))
  ;[1 1 1] scatter out
  (for (_ _array_index) _swarmenemies
    (Utilities|Struct|SetmembersinSwarmV2_Struct (Utilities|Array|Get(acopy) _swarmenemies _array_index) (* (.init_rel_pos (Utilities|Struct|BreakSwarmV2_Struct (Utilities|Array|Get(acopy) _swarmenemies _array_index))) (Math|Vector|MakeVector 1.0 (Math|Float|Lerp 1.0 (Variables|/Script/Neokaiju.SwarmStats|GetScatterDisperseY _stats) _returnvalue) (Math|Float|Lerp 1.0 (Variables|/Script/Neokaiju.SwarmStats|GetScatterDisperseZ _stats) _returnvalue))))
    (Transformation|SetRelativeLocation (.scene_component (Utilities|Struct|BreakSwarmV2_Struct (Utilities|Array|Get(acopy) _swarmenemies _array_index))) (* (.init_rel_pos (Utilities|Struct|BreakSwarmV2_Struct (Utilities|Array|Get(acopy) _swarmenemies _array_index))) (Math|Vector|MakeVector 1.0 (Math|Float|Lerp 1.0 (Variables|/Script/Neokaiju.SwarmStats|GetScatterDisperseY _stats) _returnvalue) (Math|Float|Lerp 1.0 (Variables|/Script/Neokaiju.SwarmStats|GetScatterDisperseZ _stats) _returnvalue))) false false)))

(event EventScatterSwarmin
  (params (scatterTime :type Float%20%28single-precision%29) (totalScatterTime :type Float%20%28single-precision%29))
  (bind _returnvalue (/ scatterTime totalScatterTime))
  (bind _stats (Variables|Default|GetStats))
  (bind _swarmenemies (Variables|Default|GetSwarmEnemies))
  ;[1 1 1] scatter in
  (for (_ _array_index) _swarmenemies
    (Utilities|Struct|SetmembersinSwarmV2_Struct (Utilities|Array|Get(acopy) _swarmenemies _array_index) (* (.init_rel_pos (Utilities|Struct|BreakSwarmV2_Struct (Utilities|Array|Get(acopy) _swarmenemies _array_index))) (Math|Vector|MakeVector 1.0 (Math|Float|Lerp (Variables|/Script/Neokaiju.SwarmStats|GetScatterDisperseY _stats) 1.0 _returnvalue) (Math|Float|Lerp (Variables|/Script/Neokaiju.SwarmStats|GetScatterDisperseZ _stats) 1.0 _returnvalue))))
    (Transformation|SetRelativeLocation (.scene_component (Utilities|Struct|BreakSwarmV2_Struct (Utilities|Array|Get(acopy) _swarmenemies _array_index))) (* (.init_rel_pos (Utilities|Struct|BreakSwarmV2_Struct (Utilities|Array|Get(acopy) _swarmenemies _array_index))) (Math|Vector|MakeVector 1.0 (Math|Float|Lerp (Variables|/Script/Neokaiju.SwarmStats|GetScatterDisperseY _stats) 1.0 _returnvalue) (Math|Float|Lerp (Variables|/Script/Neokaiju.SwarmStats|GetScatterDisperseZ _stats) 1.0 _returnvalue))) false false)))

(event EventBeginOverlapbyLaser
  (bind _currentstate (Variables|Default|GetCurrentState))
  ;[1 1 1] Laser events
  (Utilities|IsValid _currentstate
    (:Is%20Valid
      (Class|SwarmState|OnBeginOverlapbyLaser _currentstate)
      (Variables|Default|SetRotationMultiplier (Variables|/Script/Neokaiju.SwarmStats|GetLazerReactionSpin (Variables|Default|GetStats))))))

(event EventEndOverlapbyLaser
  (bind _currentstate (Variables|Default|GetCurrentState))
  ;[1 1 1] Laser events
  (Utilities|IsValid _currentstate
    (:Is%20Valid
      (Class|SwarmState|OnEndOverlapbyLaser _currentstate)
      (Variables|Default|SetRotationMultiplier (Variables|/Script/Neokaiju.SwarmStats|GetNormalSpin (Variables|Default|GetStats))))))

(event EventRotateSwarm
  (params (deltaTime :type Float%20%28single-precision%29))
  (bind _swarmhook (Variables|Default|GetswarmHook))
  (bind _relativerotation (Variables|/Script/Engine.SceneComponent|GetRelativeRotation _swarmhook))
  (bind (_roll _pitch _yaw) (Math|Rotator|BreakRotator _relativerotation))
  ;[1 1 1] Rotate
  (Transformation|SetRelativeRotation _swarmhook (Math|Rotator|MakeRotator _roll _pitch (+ _yaw (* deltaTime (Variables|Default|GetRotationMultiplier)))) false false))

(event EventTick
  (params (DeltaSeconds :type Float%20%28single-precision%29)))

(event EventInit
  (bind _askaiju_character (Utilities|Casting|CastToKaijuCharacter (Game|GetPlayerCharacter 0))
    (:then
      (Variables|Default|SetTargetKaiju _askaiju_character)
      (CallFunction|InitSwarmEnemies)
      (Rendering|Material|SetMaterial (Variables|Default|GetBulletMesh) 0 "/Game/NeoKaiju/Enemies/Swarm/M_SwarmShield1.M_SwarmShield1")
      (Rendering|Material|SetMaterial (Variables|Default|GetClawMesh) 0 "/Game/NeoKaiju/Enemies/Swarm/M_SwarmShield1.M_SwarmShield1")
      (Variables|Default|SetRotationMultiplier (Variables|/Script/Neokaiju.SwarmStats|GetNormalSpin (Variables|Default|GetStats)))
      (bind _returnvalue (Game|ConstructObjectfromClass "/Game/NeoKaiju/Enemies/SwarmV2/States/BP_Idle.BP_Idle_C" self))
      (Class|SwarmV2|ChangeState self _returnvalue))
    (:CastFailed
      (Development|PrintString "The wrong character class is being used."))))

(event EventKillSwarm
  (bind _currentstate (Variables|Default|GetCurrentState))
  (bind _innerradius (Variables|Default|GetInnerRadius))
  ;[1 1 1] kill
  (Utilities|FlowControl|Delay (Math|Random|RandomFloatinRange 0.05 0.4))
  (for _array_element (Variables|Default|GetSwarmEnemies)
    (Effects|SpawnEmitteratLocation "/Game/NeoKaiju/Particles/StarterContent/Particles/P_Explosion.P_Explosion" (Transformation|GetWorldLocation (.scene_component (Utilities|Struct|BreakSwarmV2_Struct _array_element))) (Math|Random|RandomRotator true) (* (Transformation|GetWorldScale (.scene_component (Utilities|Struct|BreakSwarmV2_Struct _array_element))) 2)))
  (Effects|SpawnEmitteratLocation "/Game/NeoKaiju/Particles/StarterContent/Particles/P_Explosion.P_Explosion" (Transformation|GetWorldLocation _innerradius) (Math|Random|RandomRotator true) (* (Transformation|GetWorldScale _innerradius) 2))
  (Class|EnemySubsystem|EnemyDestroyed (Subsystems|GetEnemySubsystem) self)
  (CallFunction|PlayEvent "/Game/Neokaiju/Audio/Events/Environment/Swarm_Destroyed.Swarm_Destroyed" (Transformation|GetActorLocation))
  (Utilities|IsValid _currentstate
    (:Is%20Valid
      (Class|SwarmState|Exit _currentstate))
    (:Is%20Not%20Valid
      _))
  (Actor|DestroyActor))

(event EventBeginHitbyLaser
  ;[1 1 1] Laser events
  (Variables|Default|SetbHitByLaser true))

(event EventOnCapturedActorEscape
  (params (StruggleAttemptNum :type Integer) (TimeSinceCaptureStarted :type Float%20%28single-precision%29))
  (bind _returnvalue (Class|Actor|GetInputAxisKeyValue))
  ;[1 1 1] Actor struggling
  (bind _asbp_grab (Utilities|Casting|CastToBP_Grab (Variables|Default|GetCurrentState)))
  (Default|OnCapturedActorEscape _asbp_grab StruggleAttemptNum TimeSinceCaptureStarted (or (> _returnvalue 0.0) (and (== _returnvalue 0.0) (Utilities|Enum|Equal(Enum) (Variables|/Script/Neokaiju.KaijuMovementComponent|GetFacingDirection (Variables|/Script/Neokaiju.KaijuCharacter|GetKaijuMovement (Variables|Default|GetTargetKaiju))) "RIGHT")))))

(event EventOnCapturedActorStruggle
  (params (StruggleAttemptNum :type Integer) (StrugglesRemainingToEscape :type Integer) (TimeSinceCaptureStarted :type Float%20%28single-precision%29))
  (bind _returnvalue (Class|Actor|GetInputAxisKeyValue))
  ;[1 1 1] Actor struggling
  (bind _asbp_grab (Utilities|Casting|CastToBP_Grab (Variables|Default|GetCurrentState)))
  (Default|OnCapturedActorStruggle _asbp_grab StruggleAttemptNum StrugglesRemainingToEscape TimeSinceCaptureStarted (or (> _returnvalue 0.0) (and (== _returnvalue 0.0) (Utilities|Enum|Equal(Enum) (Variables|/Script/Neokaiju.KaijuMovementComponent|GetFacingDirection (Variables|/Script/Neokaiju.KaijuCharacter|GetKaijuMovement (Variables|Default|GetTargetKaiju))) "RIGHT")))))

(event EventEndHitbyLaser
  ;[1 1 1] Laser events
  (Variables|Default|SetbHitByLaser false))

(event EventAssembleSwarm
  (params (transformTime :type Float%20%28single-precision%29) (totalTransformTime :type Float%20%28single-precision%29))
  (bind _returnvalue (/ transformTime totalTransformTime))
  (bind _returnvalue_2 (- 1.0 _returnvalue))
  ;[1 1 1] assemble swarm
  (Transformation|SetRelativeScale3D (select (Variables|Default|GetClawMode) (Variables|Default|GetClawMesh) (Variables|Default|GetBulletMesh)) (Math|Vector|MakeVector _returnvalue _returnvalue _returnvalue))
  (Transformation|SetRelativeScale3D (Variables|Default|GetswarmHook) (Math|Vector|MakeVector _returnvalue_2 _returnvalue_2 _returnvalue_2)))

(fn ConstructionScript
  (Components|Sphere|SetSphereRadius (Variables|Default|GetOuterRadius) (Variables|/Script/Neokaiju.SwarmStats|GetIdleOuterRadius (Variables|Default|GetStats)) false))

(fn FindOpenSpace
  (params (Target :type Vector :default "0, 0, 0") (MaxDist :type Float%20%28single-precision%29))
  (bind _returnvalue (Transformation|GetActorLocation))
  (bind _innerradius (Variables|Default|GetInnerRadius))
  (bind _defaultmaxdist (LocalVariables|GetDefaultMaxDist))
  (bind _returnvalue_2 (Components|Sphere|GetScaledSphereRadius _innerradius))
  (bind _returnvalue_3 (* _returnvalue_2 2.0))
  (bind _returnvalue_4 (- MaxDist _returnvalue_3))
  (bind _returnvalue_5 (Math|Float|Truncate _returnvalue_4))
  (|CallParentFunction Target MaxDist)
  (for _array_element (Variables|Default|GetDirections)
    (LocalVariables|SetFinalDirection (Math|Vector|RotateVector Target _array_element))
    (bind _returnvalue_6 (Collision|SphereTraceForObjects (+ _returnvalue (* (Math|Vector|RotateVector Target _array_element) (* 0.5 _returnvalue_2))) (+ _returnvalue (* (Math|Vector|RotateVector Target _array_element) (select (> _defaultmaxdist _returnvalue_5) _returnvalue_5 _defaultmaxdist))) _returnvalue_2 (Utilities|Array|MakeArray "ObjectTypeQuery1" "ObjectTypeQuery2" "ObjectTypeQuery5") false 0 "None"))
    ;[1 1 1] return the current direction if clear
    (if (not _returnvalue_6)
      (return (Math|Vector|Normalize (LocalVariables|GetFinalDirection)))))
  (return "0, 0, 0"))

(fn OrientPointer
  (params (pointerHook :type Scene%20Component%20Object%20Reference) (direction :type Vector))
  (bind _returnvalue (Transformation|GetWorldLocation pointerHook))
  (bind _pointer (Variables|Default|Getpointer))
  (bind _pointer_2 (Variables|Default|Getpointer))
  (bind _relativescale3d (Variables|/Script/Engine.SceneComponent|GetRelativeScale3D _pointer_2))
  (bind _relativelocation (Variables|/Script/Engine.SceneComponent|GetRelativeLocation _pointer))
  (bind (_outhit _returnvalue_2) (Collision|LineTraceForObjects _returnvalue (+ _returnvalue (* direction 2e+03)) (Utilities|Array|MakeArray "ObjectTypeQuery1" "ObjectTypeQuery2" "ObjectTypeQuery3") false 0 "None"))
  (Transformation|SetRelativeScale3D _pointer_2 (Math|Vector|MakeVector (.x _relativescale3d) (.y _relativescale3d) (/ (+ (Math|Float|SelectFloat (.Distance (Collision|BreakHitResult _outhit)) 1e+03 _returnvalue_2) 1e+02) 1e+02)))
  (Transformation|SetRelativeLocation _pointer (Math|Vector|MakeVector (.x _relativelocation) (.y _relativelocation) (+ (/ (Math|Float|SelectFloat (.Distance (Collision|BreakHitResult _outhit)) 1e+03 _returnvalue_2) 2.0) (.z (Math|Transform|InverseTransformLocation (Transformation|GetActorTransform) (Transformation|GetWorldLocation pointerHook))))) false false))

(fn SetSwarmVisibility
  (params (NewVisibility :type Boolean))
  (for _array_element (Variables|Default|GetSwarmEnemies)
    (Rendering|SetVisibility (.scene_component (Utilities|Struct|BreakSwarmV2_Struct _array_element)) NewVisibility true)))

(fn InitSwarmEnemies
  (for _index (range 0 (- (Math|Conversions|ToInteger(Byte) (Variables|Default|GetmaxSwarmAmount)) 1))
    (bind _enemyradiussquared (CallFunction|AddSwarmEnemy))
    (if (> _enemyradiussquared (LocalVariables|GetswarmRadiusSquared))
      (LocalVariables|SetswarmRadiusSquared _enemyradiussquared)))
  (Components|Sphere|SetSphereRadius (Variables|Default|GetInnerRadius) (/ (Math|Float|Sqrt (LocalVariables|GetswarmRadiusSquared)) 1.25) true)
  (Rendering|SetVisibility (Variables|Default|GetBulletMesh) false false))

(fn AddSwarmEnemy
  (bind _returnvalue (AddComponent|AddSceneComponent false (Math|Transform|MakeTransform (Math|Random|RandomPointinBoundingBox "0, 0, 0" (Variables|Default|GetmaxSwarmBound)) "0, 0, 0" (Variables|Default|GetenemyScale))))
  (Transformation|AttachComponentToComponent _returnvalue (Variables|Default|GetswarmHook) "None" "KeepRelative" "KeepRelative" "KeepRelative" true)
  (bind _rot (CallFunction|ProcessNewRotator))
  (LocalVariables|SetparticleRadiusSquared (Math|Vector|VectorLengthSquared (Variables|/Script/Engine.SceneComponent|GetRelativeLocation _returnvalue)))
  (Utilities|Array|Add (Variables|Default|GetSwarmEnemies) (Utilities|Struct|MakeSwarmV2_Struct _returnvalue (Variables|/Script/Engine.SceneComponent|GetRelativeLocation _returnvalue) (Variables|/Script/Engine.SceneComponent|GetRelativeLocation _returnvalue) _rot))
  (bind _returnvalue_2 (Effects|SpawnEmitterAttached "/Game/NeoKaiju/Particles/Cones_Spinning2.Cones_Spinning2" _returnvalue "None" "0, 0, 0" "0, 0, 0" "4.000000,4.000000,4.000000"))
  (CallFunction|SetParticleRandBehaviour _returnvalue_2)
  (return (LocalVariables|GetparticleRadiusSquared)))

(fn ProcessNewRotator
  (bind _returnvalue (Math|Random|RandomRotator true))
  (bind (_roll _pitch _yaw) (Math|Rotator|BreakRotator _returnvalue))
  (bind _returnvalue_2 (/ _roll 3.6e+02))
  (bind _returnvalue_3 (/ _pitch 3.6e+02))
  (bind _returnvalue_4 (/ _yaw 3.6e+02))
  (return (Math|Rotator|MakeRotator (Math|Float|SelectFloat (- 3.6e+02 _returnvalue_2) _returnvalue_2 (> _roll 1.8e+02)) (Math|Float|SelectFloat (- 3.6e+02 _returnvalue_3) _returnvalue_3 (> _pitch 1.8e+02)) (Math|Float|SelectFloat (- 3.6e+02 _returnvalue_4) _returnvalue_4 (> _yaw 1.8e+02)))))

(fn SetParticleRandBehaviour
  (params (swarmParticle :type Particle%20System%20Component%20Object%20Reference))
  (bind _maxparticlebound (Variables|Default|GetmaxParticleBound))
  (bind _maxparticlerate (Variables|Default|GetmaxParticleRate))
  (Variables|/Script/Engine.ParticleSystemComponent|SetInstanceParameters swarmParticle (Utilities|Array|MakeArray (Utilities|Struct|MakeParticleSysParam "orbitOffset1" "PSPT_Vector" 0.0 0.0 (Math|Random|RandomPointinBoundingBox "0, 0, 0" _maxparticlebound)) (Utilities|Struct|MakeParticleSysParam "orbitOffset2" "PSPT_Vector" 0.0 0.0 (Math|Random|RandomPointinBoundingBox "0, 0, 0" _maxparticlebound)) (Utilities|Struct|MakeParticleSysParam "orbitOffset3" "PSPT_Vector" 0.0 0.0 (Math|Random|RandomPointinBoundingBox "0, 0, 0" _maxparticlebound)) (Utilities|Struct|MakeParticleSysParam "orbitOffset4" "PSPT_Vector" 0.0 0.0 (Math|Random|RandomPointinBoundingBox "0, 0, 0" _maxparticlebound)) (Utilities|Struct|MakeParticleSysParam "orbitRate1" "PSPT_Vector" 0.0 0.0 (Math|Random|RandomPointinBoundingBox "0, 0, 0" _maxparticlerate)) (Utilities|Struct|MakeParticleSysParam "orbitRate2" "PSPT_Vector" 0.0 0.0 (Math|Random|RandomPointinBoundingBox "0, 0, 0" _maxparticlerate)) (Utilities|Struct|MakeParticleSysParam "orbitRate3" "PSPT_Vector" 0.0 0.0 (Math|Random|RandomPointinBoundingBox "0, 0, 0" _maxparticlerate)) (Utilities|Struct|MakeParticleSysParam "orbitRate4" "PSPT_Vector" 0.0 0.0 (Math|Random|RandomPointinBoundingBox "0, 0, 0" _maxparticlerate)))))

(fn FindOpenSpaceFrontBack
  (params (Target :type Vector :default "0, 0, 0") (MaxDist :type Float%20%28single-precision%29))
  (bind _returnvalue (Transformation|GetActorLocation))
  (bind _directions (Variables|Default|GetDirections))
  (bind _defaultmaxdist (LocalVariables|GetDefaultMaxDist))
  (bind _innerradius (Variables|Default|GetInnerRadius))
  (bind _returnvalue_2 (Utilities|Array|Length _directions))
  (bind _returnvalue_3 (Components|Sphere|GetScaledSphereRadius _innerradius))
  (bind _returnvalue_4 (* _returnvalue_3 2.0))
  (bind _returnvalue_5 (- MaxDist _returnvalue_4))
  (bind _returnvalue_6 (Math|Float|Truncate _returnvalue_5))
  (|CallParentFunction Target MaxDist)
  (LocalVariables|SetfourthLength (/ (Utilities|Array|Length (Variables|Default|GetDirections)) 4))
  ;[1 1 1] get the first part of the array (the direction requested)
  (LocalVariables|SetloopValue 0)
  (for _index (range 0 (- (LocalVariables|GetfourthLength) 1))
    (LocalVariables|SetFinalDirection (Math|Vector|RotateVector Target (Utilities|Array|Get(acopy) (Variables|Default|GetDirections) (Utilities|Select :Index (LocalVariables|GetloopValue) :Option%200 _index :Option%201 (stale _index_2) :Option%202 (stale _index_3) :Option%203 0))))
    (bind _returnvalue_7 (Collision|SphereTraceForObjects (+ _returnvalue (* (Math|Vector|RotateVector Target (Utilities|Array|Get(acopy) (Variables|Default|GetDirections) (Utilities|Select :Index (LocalVariables|GetloopValue) :Option%200 _index :Option%201 (stale _index_2) :Option%202 (stale _index_3) :Option%203 0))) (* 0.5 _returnvalue_3))) (+ _returnvalue (* (Math|Vector|RotateVector Target (Utilities|Array|Get(acopy) (Variables|Default|GetDirections) (Utilities|Select :Index (LocalVariables|GetloopValue) :Option%200 _index :Option%201 (stale _index_2) :Option%202 (stale _index_3) :Option%203 0))) (select (> _defaultmaxdist _returnvalue_6) _returnvalue_6 _defaultmaxdist))) _returnvalue_3 (Utilities|Array|MakeArray "ObjectTypeQuery1" "ObjectTypeQuery2" "ObjectTypeQuery5") false 0 "None"))
    ;[1 1 1] return the current direction if clear
    (if (not _returnvalue_7)
      (return (Math|Vector|Normalize (LocalVariables|GetFinalDirection)))))
  ;[1 1 1] get the end of the array (the opposite direction)
  (LocalVariables|SetloopValue 0)
  (for _index_2 (range (- _returnvalue_2 (LocalVariables|GetfourthLength)) (- _returnvalue_2 1))
    (LocalVariables|SetFinalDirection (Math|Vector|RotateVector Target (Utilities|Array|Get(acopy) (Variables|Default|GetDirections) (Utilities|Select :Index (LocalVariables|GetloopValue) :Option%200 _index :Option%201 _index_2 :Option%202 (stale _index_3) :Option%203 0))))
    (bind _returnvalue_8 (Collision|SphereTraceForObjects (+ _returnvalue (* (Math|Vector|RotateVector Target (Utilities|Array|Get(acopy) (Variables|Default|GetDirections) (Utilities|Select :Index (LocalVariables|GetloopValue) :Option%200 _index :Option%201 _index_2 :Option%202 (stale _index_3) :Option%203 0))) (* 0.5 _returnvalue_3))) (+ _returnvalue (* (Math|Vector|RotateVector Target (Utilities|Array|Get(acopy) (Variables|Default|GetDirections) (Utilities|Select :Index (LocalVariables|GetloopValue) :Option%200 _index :Option%201 _index_2 :Option%202 (stale _index_3) :Option%203 0))) (select (> _defaultmaxdist _returnvalue_6) _returnvalue_6 _defaultmaxdist))) _returnvalue_3 (Utilities|Array|MakeArray "ObjectTypeQuery1" "ObjectTypeQuery2" "ObjectTypeQuery5") false 0 "None"))
    (if (not _returnvalue_8)
      (return (Math|Vector|Normalize (LocalVariables|GetFinalDirection)))))
  ;[1 1 1] get the middle of the array if all else fails (perpendicular to direction wanted)
  (LocalVariables|SetloopValue 2)
  (for _index_3 (range (LocalVariables|GetfourthLength) (- (- (Utilities|Array|Length (Variables|Default|GetDirections)) (LocalVariables|GetfourthLength)) 1))
    (LocalVariables|SetFinalDirection (Math|Vector|RotateVector Target (Utilities|Array|Get(acopy) (Variables|Default|GetDirections) (Utilities|Select :Index (LocalVariables|GetloopValue) :Option%200 _index :Option%201 _index_2 :Option%202 _index_3 :Option%203 0))))
    (bind _returnvalue_9 (Collision|SphereTraceForObjects (+ _returnvalue (* (Math|Vector|RotateVector Target (Utilities|Array|Get(acopy) (Variables|Default|GetDirections) (Utilities|Select :Index (LocalVariables|GetloopValue) :Option%200 _index :Option%201 _index_2 :Option%202 _index_3 :Option%203 0))) (* 0.5 _returnvalue_3))) (+ _returnvalue (* (Math|Vector|RotateVector Target (Utilities|Array|Get(acopy) (Variables|Default|GetDirections) (Utilities|Select :Index (LocalVariables|GetloopValue) :Option%200 _index :Option%201 _index_2 :Option%202 _index_3 :Option%203 0))) (select (> _defaultmaxdist _returnvalue_6) _returnvalue_6 _defaultmaxdist))) _returnvalue_3 (Utilities|Array|MakeArray "ObjectTypeQuery1" "ObjectTypeQuery2" "ObjectTypeQuery5") false 0 "None"))
    (if (not _returnvalue_9)
      (return (Math|Vector|Normalize (LocalVariables|GetFinalDirection)))))
  (return "0, 0, 0"))

(fn LaserDamage
  (CallFunction|DealDamage (* (Utilities|Time|GetWorldDeltaSeconds) (Utilities|Select :Index (Math|Float|Ceil (.ReturnValue (Ability|Attribute|GetFloatAttributefromAbilitySystemComponent (Ability|GetAbilitySystemComponent (Variables|Default|GetTargetKaiju)) "(AttributeName=\"KaijuLevel\",Attribute=StructProperty'\"/Script/Neokaiju.KaijuAttributeSet:KaijuLevel\"',AttributeOwner=Class'\"/Script/Neokaiju.KaijuAttributeSet\"')"))) :Option%200 0.1 :Option%201 0.5 :Option%202 1.0 :Option%203 1.5 :Option%204 2.0))))