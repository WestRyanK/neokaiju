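; BP_Prop is a structure prop Blueprint that adds sound and particle effects when the prop is destroyed.
; Its PlayonDestroyedFX override calls the parent, then plays DestroyedSound and spawns a PS_JParticleBurst system at the actor's location.
; The burst scales uniformly from the largest dimension of the mesh's local bounds divided by 100, so it fits the prop's size.
; An unconnected SpawnEmitterAttached node never runs, and the construction script is empty.
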(event EventPlayonDestroyedFX
  (bind _returnvalue (Transformation|GetActorLocation))
  (bind _mesh (Variables|Character|GetMesh))
  (bind (_min _max) (Components|StaticMesh|GetLocalBounds _mesh))
  (bind _returnvalue_2 (- _max _min))
  (bind _returnvalue_3 (Math|Float|Max(Float) (.x _returnvalue_2) (.y _returnvalue_2) (.z _returnvalue_2)))
  (bind _returnvalue_4 (/ _returnvalue_3 1e+02))
  (|CallParentFunction)
  (CallFunction|PlayEvent (Variables|Default|GetDestroyedSound) _returnvalue)
  (Niagara|SpawnSystematLocation "/Game/NeoKaiju/Particles/John_Particles/PS_JParticleBurst.PS_JParticleBurst" _returnvalue "90.000000, 0, 0" (Math|Vector|MakeVector _returnvalue_4 _returnvalue_4 _returnvalue_4)))

(fn ConstructionScript)