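; Exploding building block that gives visual and audio feedback before and during its explosion.
; On BeginPlay it applies the exploding barrel material and caches the mesh's initial scale.
; When about to explode, it shakes the actor and swells it through a timeline relative to that scale.
; On explosion it plays a sound event and spawns particles at the epicenter, sized by the maximum explosion radius.
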(event EventBeginPlay
  (Rendering|Material|SetMaterial (Variables|Character|GetMesh) 0 "/Game/NeoKaiju/Structures/Textures/ExplodingBarrel.ExplodingBarrel")
  (Variables|Default|Setinitial_scale (Variables|/Script/Engine.SceneComponent|GetRelativeScale3D (Variables|Character|GetMesh))))

(event Collision|EventActorBeginOverlap
  (params (OtherActor :type Actor%20Object%20Reference)))

(event EventOnAbouttoExplode
  (params (TimeUntilExplosion :type Float%20%28single-precision%29))
  (Class|ShakerComponent|PlayShakeonActor (Variables|Default|GetShaker))
  (bind _scale (Timeline|ExpandTimeline Play)
    (:Update
      (Transformation|SetActorScale3D (* (Variables|Default|Getinitial_scale) _scale)))))

(event EventOnExplode
  (params (Epicenter :type Vector :default "0, 0, 0"))
  (CallFunction|PlayExplosionParticleEffect Epicenter)
  (CallFunction|PlayExplosionSoundEffect Epicenter))

(fn ConstructionScript)

(fn PlayExplosionParticleEffect
  (params (Epicenter :type Vector))
  (Effects|SpawnEmitteratLocation (Variables|Default|GetExplosionParticleEffect) Epicenter "0, 0, 0" (Math|Conversions|ToVector(Float) (/ (Class|ExplodingBuildingBlock|GetMaxExplodeRadius) 5e+01))))

(fn PlayExplosionSoundEffect
  (params (Epicenter :type Vector))
  (CallFunction|PlayEvent (Variables|Default|GetExplosionSound) Epicenter))