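; Destructible building block actor that plays damage and destruction feedback and can auto-size its bounds to its mesh at construction.
; Damage plays a level-indexed FMOD sound and a shake; destruction plays a sound and spawns rubble.
; Rubble is a BP_BuildingJiblets actor scaled to mesh bounds, with crumble particles.
; Its see-through material copies textures and tint from the mesh's first or second dynamic material, otherwise reusing that material.
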(event EventBeginPlay)

(event Collision|EventActorBeginOverlap
  (params (OtherActor :type Actor%20Object%20Reference)))

(event EventTick
  (params (DeltaSeconds :type Float%20%28single-precision%29)))

(event EventPlayonDamagedFX
  (params (OldHealth :type Float%20%28single-precision%29) (NewHealth :type Float%20%28single-precision%29))
  (bind _shouldplay (CallFunction|ShouldPlayDamageFX OldHealth NewHealth self))
  (if _shouldplay
    (CallFunction|PlayFMODSoundbyLevel (Variables|Default|GetDamageSoundsByLevel))
    (Class|ShakerComponent|PlayShakeonActor (Variables|Default|GetShaker))))

(event EventPlayonDestroyedFX
  (CallFunction|PlayFMODSoundbyLevel (Variables|Default|GetDestroyedSoundsByLevel))
  (CallFunction|SpawnRubble))

(fn ConstructionScript
  (if (Variables|Default|GetUseAutoScaleToMesh)
    (Class|BreakableStructure|ResizeBounds)))

(fn PlayFMODSoundbyLevel
  (params (SoundByLevel :type Array%20of%20FMOD%20Event%20Object%20References))
  (CallFunction|PlayEvent (Utilities|Array|Get(acopy) SoundByLevel (Math|Float|Truncate (.ReturnValue (Ability|Attribute|GetFloatAttribute self "(AttributeName=\"Tier\",Attribute=StructProperty'\"/Script/Neokaiju.BreakableStructureAttributeSet:Tier\"',AttributeOwner=Class'\"/Script/Neokaiju.BreakableStructureAttributeSet\"')")))) (Transformation|GetActorLocation)))

(fn SpawnRubble
  (bind _mesh (Variables|Character|GetMesh))
  (bind _mesh_2 (Variables|Character|GetMesh))
  (bind (_origin _boxextent) (Collision|GetComponentBounds _mesh))
  (bind _returnvalue (Rendering|Material|GetMaterial _mesh_2 1))
  (bind _returnvalue_2 (Rendering|Material|GetMaterial _mesh_2 0))
  (Utilities|IsValid (Variables|Character|GetMesh)
    (:Is%20Valid
      (Utilities|IsValid (Rendering|Material|GetMaterial (Variables|Character|GetMesh) 0)
        (:Is%20Valid
          (bind _returnvalue_3 (Game|SpawnActorfromClass "/Game/NeoKaiju/Structures/Blocks/BP_BuildingJiblets.BP_BuildingJiblets_C" (Math|Transform|MakeTransform _origin (.Rotation (Math|Transform|BreakTransform (Transformation|GetActorTransform))) (/ _boxextent 5e+01)) "Undefined" self (Variables|Default|GetDestructibleMesh) 5e+03 0))
          (LocalVariables|SetDestructibleComponent (Variables|/Script/ApexDestruction.DestructibleActor|GetDestructibleComponent _returnvalue_3))
          (Utilities|IsValid (LocalVariables|GetDestructibleComponent)
            (:Is%20Valid
              (Niagara|SpawnSystemAttached "/Game/NeoKaiju/Particles/PS_BlockCrumble.PS_BlockCrumble" (LocalVariables|GetDestructibleComponent) "None" "0.000000, 0,50.000000" "0, 0, 0" "SnapToTarget" true)
              (if (not (Variables|Default|GetrubbleUseSecondMaterial))
                (bind _asmaterial_instance_dynamic (Utilities|Casting|CastToMaterialInstanceDynamic _returnvalue_2 :!label _label)
                  (:then
                    (bind _returnvalue_4 (Rendering|Material|CreateDynamicMaterialInstance (LocalVariables|GetDestructibleComponent) 0 "/Game/NeoKaiju/Structures/Blocks/Art/destructibleMeshes/destructibleMeshSeeThrough_M.destructibleMeshSeeThrough_M" "None" :!class /Script/Engine.PrimitiveComponent))
                    (Rendering|Material|SetVectorParameterValue _returnvalue_4 "baseColor" (.ParameterValue (Utilities|Struct|BreakVectorParameterValue (Utilities|Array|Get(acopy) (Variables|/Script/Engine.MaterialInstance|GetVectorParameterValues (Variables|Default|GetBaseMatSource))))) :!class /Script/Engine.MaterialInstanceDynamic)
                    (CallFunction|SetRubbleMaterial _asmaterial_instance_dynamic _returnvalue_4)
                    (Rendering|Material|SetMaterial (LocalVariables|GetDestructibleComponent) 0 _returnvalue_4)
                    (Rendering|Material|SetMaterial (LocalVariables|GetDestructibleComponent) 1 _returnvalue_4))
                  (:CastFailed
                    (bind _returnvalue_5 (Rendering|Material|CreateDynamicMaterialInstance (LocalVariables|GetDestructibleComponent) 1 _returnvalue_2 "bob" :!class /Script/Engine.PrimitiveComponent))
                    (Rendering|Material|SetMaterial (LocalVariables|GetDestructibleComponent) 0 _returnvalue_5)
                    (Rendering|Material|SetMaterial (LocalVariables|GetDestructibleComponent) 1 _returnvalue_5)))
                (else
                  (Utilities|IsValid _returnvalue
                    (:Is%20Valid
                      (bind _asmaterial_instance_dynamic_2 (Utilities|Casting|CastToMaterialInstanceDynamic _returnvalue)
                        (:then
                          (bind _returnvalue_6 (Rendering|Material|CreateDynamicMaterialInstance (LocalVariables|GetDestructibleComponent) 0 "/Game/NeoKaiju/Structures/Blocks/Art/destructibleMeshes/destructibleMeshSeeThrough_M.destructibleMeshSeeThrough_M" "None" :!class /Script/Engine.PrimitiveComponent))
                          (Rendering|Material|SetVectorParameterValue _returnvalue_6 "baseColor" (.ParameterValue (Utilities|Struct|BreakVectorParameterValue (Utilities|Array|Get(acopy) (Variables|/Script/Engine.MaterialInstance|GetVectorParameterValues (Variables|Default|GetWindowMatSource))))) :!class /Script/Engine.MaterialInstanceDynamic)
                          (CallFunction|SetRubbleMaterial _asmaterial_instance_dynamic_2 _returnvalue_6)
                          (Rendering|Material|SetMaterial (LocalVariables|GetDestructibleComponent) 0 _returnvalue_6)
                          (Rendering|Material|SetMaterial (LocalVariables|GetDestructibleComponent) 1 _returnvalue_6))
                        (:CastFailed
                          (bind _returnvalue_7 (Rendering|Material|CreateDynamicMaterialInstance (LocalVariables|GetDestructibleComponent) 1 _returnvalue "bob" :!class /Script/Engine.PrimitiveComponent))
                          (Rendering|Material|SetMaterial (LocalVariables|GetDestructibleComponent) 0 _returnvalue_7)
                          (Rendering|Material|SetMaterial (LocalVariables|GetDestructibleComponent) 1 _returnvalue_7))))
                    (:Is%20Not%20Valid
                      (goto _label))))))))))))

(fn SetRubbleMaterial
  (params (baseMaterial :type Material%20Instance%20Dynamic%20Object%20Reference) (newMaterial :type Material%20Instance%20Dynamic%20Object%20Reference))
  (bind _returnvalue (Rendering|Material|GetTextureParameterValue baseMaterial "BaseColor" :!class /Script/Engine.MaterialInstanceDynamic))
  (Rendering|Material|SetTextureParameterValue newMaterial "BaseTex" _returnvalue)
  (bind _returnvalue_2 (Rendering|Material|GetTextureParameterValue baseMaterial "Metalness/Roughness" :!class /Script/Engine.MaterialInstanceDynamic))
  (Rendering|Material|SetTextureParameterValue newMaterial "Metal/Rough" _returnvalue_2)
  (bind _returnvalue_3 (Rendering|Material|GetTextureParameterValue baseMaterial "EmmisiveColor" :!class /Script/Engine.MaterialInstanceDynamic))
  (Rendering|Material|SetTextureParameterValue newMaterial "EmmisiveColor" _returnvalue_3)
  (bind _returnvalue_4 (Rendering|Material|GetScalarParameterValue baseMaterial "Em_Color_Whiten" :!class /Script/Engine.MaterialInstanceDynamic))
  (Rendering|Material|SetScalarParameterValue newMaterial "Em_Color_Whiten" _returnvalue_4 :!class /Script/Engine.MaterialInstanceDynamic)
  (bind _returnvalue_5 (Rendering|Material|GetScalarParameterValue baseMaterial "Em_Color_Value" :!class /Script/Engine.MaterialInstanceDynamic))
  (Rendering|Material|SetScalarParameterValue newMaterial "Em_Color_Value" _returnvalue_5 :!class /Script/Engine.MaterialInstanceDynamic)
  (bind _returnvalue_6 (Rendering|Material|GetScalarParameterValue baseMaterial "Em_Color_Desaturation" :!class /Script/Engine.MaterialInstanceDynamic))
  (Rendering|Material|SetScalarParameterValue newMaterial "Em_Color_Desaturation" _returnvalue_6 :!class /Script/Engine.MaterialInstanceDynamic)
  (bind _returnvalue_7 (Rendering|Material|GetScalarParameterValue baseMaterial "Em_Tint_Alpha" :!class /Script/Engine.MaterialInstanceDynamic))
  (Rendering|Material|SetScalarParameterValue newMaterial "Em_Tint_Alpha" _returnvalue_7 :!class /Script/Engine.MaterialInstanceDynamic)
  (bind _returnvalue_8 (Rendering|Material|GetScalarParameterValue baseMaterial "Em_Hue_Shift" :!class /Script/Engine.MaterialInstanceDynamic))
  (Rendering|Material|SetScalarParameterValue newMaterial "Em_Hue_Shift" _returnvalue_8 :!class /Script/Engine.MaterialInstanceDynamic)
  (bind _returnvalue_9 (Rendering|Material|GetVectorParameterValue baseMaterial "Em_Tint" :!class /Script/Engine.MaterialInstanceDynamic))
  (Rendering|Material|SetVectorParameterValue newMaterial "Em_Tint" _returnvalue_9 :!class /Script/Engine.MaterialInstanceDynamic)
  (bind _returnvalue_10 (Rendering|Material|GetScalarParameterValue baseMaterial "Base_Color_Whiten" :!class /Script/Engine.MaterialInstanceDynamic))
  (Rendering|Material|SetScalarParameterValue newMaterial "Base_Color_Whiten" _returnvalue_10 :!class /Script/Engine.MaterialInstanceDynamic)
  (bind _returnvalue_11 (Rendering|Material|GetScalarParameterValue baseMaterial "Base_Color_Value" :!class /Script/Engine.MaterialInstanceDynamic))
  (Rendering|Material|SetScalarParameterValue newMaterial "Base_Color_Value" _returnvalue_11 :!class /Script/Engine.MaterialInstanceDynamic)
  (bind _returnvalue_12 (Rendering|Material|GetScalarParameterValue baseMaterial "Base_Color_Desaturation" :!class /Script/Engine.MaterialInstanceDynamic))
  (Rendering|Material|SetScalarParameterValue newMaterial "Base_Color_Desaturation" _returnvalue_12 :!class /Script/Engine.MaterialInstanceDynamic)
  (bind _returnvalue_13 (Rendering|Material|GetScalarParameterValue baseMaterial "Base_Tint_Alpha" :!class /Script/Engine.MaterialInstanceDynamic))
  (Rendering|Material|SetScalarParameterValue newMaterial "Base_Tint_Alpha" _returnvalue_13 :!class /Script/Engine.MaterialInstanceDynamic)
  (bind _returnvalue_14 (Rendering|Material|GetScalarParameterValue baseMaterial "Base_Hue_Shift" :!class /Script/Engine.MaterialInstanceDynamic))
  (Rendering|Material|SetScalarParameterValue newMaterial "Base_Hue_Shift" _returnvalue_14 :!class /Script/Engine.MaterialInstanceDynamic)
  (bind _returnvalue_15 (Rendering|Material|GetVectorParameterValue baseMaterial "Base_Tint" :!class /Script/Engine.MaterialInstanceDynamic))
  (Rendering|Material|SetVectorParameterValue newMaterial "Base_Tint" _returnvalue_15 :!class /Script/Engine.MaterialInstanceDynamic))