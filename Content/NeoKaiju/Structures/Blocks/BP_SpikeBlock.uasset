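; BP_SpikeBlock is a spike block structure that adds damage and destruction feedback to its parent block behavior.
; The construction script fits SpikeOverlapBox to the mesh's local bounds, centering it and matching its extent.
; Damage that passes the ShouldPlayDamageFX check plays a tier 2 stress event and shakes the actor, while destruction plays a tier 2 smash event.
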(event EventBeginPlay)

(event Collision|EventActorBeginOverlap
  (params (OtherActor :type Actor%20Object%20Reference)))

(event EventTick
  (params (DeltaSeconds :type Float%20%28single-precision%29)))

(event EventPlayonDamagedFX
  (params (OldHealth :type Float%20%28single-precision%29) (NewHealth :type Float%20%28single-precision%29))
  (bind _shouldplay (CallFunction|ShouldPlayDamageFX OldHealth NewHealth self))
  (if _shouldplay
    (CallFunction|PlayEvent "/Game/Neokaiju/Audio/Events/Structures/Stress_Tier2.Stress_Tier2" (Transformation|GetActorLocation))
    (Class|ShakerComponent|PlayShakeonActor (Variables|Default|GetShaker))))

(event EventPlayonDestroyedFX
  (CallFunction|PlayEvent "/Game/Neokaiju/Audio/Events/Structures/Smash_Tier2.Smash_Tier2" (Transformation|GetActorLocation)))

(fn ConstructionScript
  (bind _mesh (Variables|Character|GetMesh))
  (bind (_min _max) (Components|StaticMesh|GetLocalBounds _mesh))
  (|CallParentFunction)
  (bind _output_get (LocalVariables|Setcenter (/ (+ _min _max) 2.0)))
  (LocalVariables|Setextent (- _max _output_get))
  (Transformation|SetRelativeLocation (Variables|Default|GetSpikeOverlapBox) (LocalVariables|Getcenter) false false)
  (Components|Box|SetBoxExtent (Variables|Default|GetSpikeOverlapBox) (LocalVariables|Getextent) true))