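; Short-lived destructible debris actor for buildings that shatters as soon as it spawns.
; The construction script applies the configured DestructibleMesh to its DestructibleComponent.
; On BeginPlay it applies full radius damage from a point offset along world Y within its bounds, pushing the pieces with a configurable impulse.
; The actor destroys itself after DestroyDelay.
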(event EventBeginPlay
  (bind (_origin _boxextent) (Collision|GetActorBounds false))
  (Class|DestructibleComponent|ApplyRadiusDamage (Variables|Default|GetDestructibleComponent) 1.0 (+ _origin (Math|Vector|MakeVector 0.0 (* (.Y (Math|Vector|BreakVector _boxextent)) 0.75) 0.0)) 5e+02 (Variables|Default|GetImpulse) true)
  (Utilities|FlowControl|Delay (Variables|Default|GetdestroyDelay))
  (Actor|DestroyActor))

(event Collision|EventActorBeginOverlap
  (params (OtherActor :type Actor%20Object%20Reference)))

(event EventTick
  (params (DeltaSeconds :type Float%20%28single-precision%29)))

(fn ConstructionScript
  (Class|SkinnedMeshComponent|SetSkeletalMesh (Variables|Default|GetDestructibleComponent) (Variables|Default|GetDestructibleMesh) true))