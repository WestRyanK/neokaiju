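; Destructible powercore structure block that plays an explosion audio event at its location and spawns rubble when its destroyed FX fire.
; Its SetRubbleMaterial override copies surface parameters such as base color, emissive, metallic, roughness and opacity from the base material into the rubble material, enabling flat-value switches without calling the parent version.
; Unconnected leftover logic covers a louder 2D explosion sound and captive baby kaiju pickup; neither runs.
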(event EventBeginPlay
  (|CallParentFunction))

(event Collision|EventActorBeginOverlap
  (params (OtherActor :type Actor%20Object%20Reference))
  (|CallParentFunction OtherActor) ; This node is disabled and will not be called.\nDrag off pins to build functionality.
)

(event EventTick
  (params (DeltaSeconds :type Float%20%28single-precision%29))
  (|CallParentFunction DeltaSeconds) ; This node is disabled and will not be called.\nDrag off pins to build functionality.
)

(event EventPlayonDestroyedFX
  (CallFunction|PlayEvent "/Game/Neokaiju/Audio/Events/Structures/PowerCore_Explosion.PowerCore_Explosion" (Transformation|GetActorLocation))
  (CallFunction|SpawnRubble))

(fn ConstructionScript
  (|CallParentFunction))

(fn SetRubbleMaterial
  (params (baseMaterial :type Material%20Instance%20Dynamic%20Object%20Reference) (newMaterial :type Material%20Instance%20Dynamic%20Object%20Reference))
  (bind _returnvalue (Rendering|Material|GetVectorParameterValue baseMaterial "Base Color" :!class /Script/Engine.MaterialInstanceDynamic))
  (Rendering|Material|SetScalarParameterValue newMaterial "useFlatBaseColor" 1.0 :!class /Script/Engine.MaterialInstanceDynamic)
  (Rendering|Material|SetVectorParameterValue newMaterial "baseColor" _returnvalue :!class /Script/Engine.MaterialInstanceDynamic)
  (bind _returnvalue_2 (Rendering|Material|GetVectorParameterValue baseMaterial "Emissive Color" :!class /Script/Engine.MaterialInstanceDynamic))
  (Rendering|Material|SetScalarParameterValue newMaterial "useFlatEmissive" 1.0 :!class /Script/Engine.MaterialInstanceDynamic)
  (Rendering|Material|SetVectorParameterValue newMaterial "Emisive Color" _returnvalue_2 :!class /Script/Engine.MaterialInstanceDynamic)
  (bind _returnvalue_3 (Rendering|Material|GetVectorParameterValue baseMaterial "Metallic" :!class /Script/Engine.MaterialInstanceDynamic))
  (Rendering|Material|SetScalarParameterValue newMaterial "useFlatMetalic/Rough/Occlusion" 1.0 :!class /Script/Engine.MaterialInstanceDynamic)
  (Rendering|Material|SetVectorParameterValue newMaterial "Metalic" _returnvalue_3 :!class /Script/Engine.MaterialInstanceDynamic)
  (bind _returnvalue_4 (Rendering|Material|GetVectorParameterValue baseMaterial "Roughness" :!class /Script/Engine.MaterialInstanceDynamic))
  (Rendering|Material|SetVectorParameterValue newMaterial "Roughness" _returnvalue_4 :!class /Script/Engine.MaterialInstanceDynamic)
  (bind _returnvalue_5 (Rendering|Material|GetVectorParameterValue baseMaterial "Opacity" :!class /Script/Engine.MaterialInstanceDynamic))
  (Rendering|Material|SetVectorParameterValue newMaterial "OpacityAft" _returnvalue_5 :!class /Script/Engine.MaterialInstanceDynamic))