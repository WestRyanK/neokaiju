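; BP_Claww is a claw structure attachment that traps the kaiju, providing its animation, sound and struggle feedback.
; Ready, capture, extend and release events drive montages and audio, with capture also notifying the kaiju character event subsystem.
; CanReady and NeedsReady flags stop repeated readying and queue it until the break animation's notify.
; Captured struggles shake the mesh sideways through a DoOnce-gated timeline, directed by player input or kaiju facing.
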(event EventBeginPlay)

(event EventPlayonCaptureFX
  (Class|KaijuCharacterEventSubsystem|KaijuTrappedbyClaw (Subsystems|GetKaijuCharacterEventSubsystem))
  (CallFunction|PlayEventAttached (Variables|Default|GetClawGrabSoundEvent) (Variables|Default|GetClawMesh))
  (Animation|Montage|PlayMontage (Variables|Default|GetClawMesh) "/Game/NeoKaiju/Structures/Attachments/Claw/Art/Animations/AM_ClawGrab.AM_ClawGrab" 3.0 0.0 "Default"))

(event EventOnCapturedActorStruggle
  (params (StruggleAttemptNum :type Integer) (StrugglesRemainingToEscape :type Integer) (TimeSinceCaptureStarted :type Float%20%28single-precision%29))
  (bind _returnvalue (Class|Actor|GetInputAxisKeyValue))
  (bind _clawmesh (Variables|Default|GetClawMesh))
  (bind _returnvalue_2 (> _returnvalue 0.0))
  (bind _relativelocation (Variables|/Script/Engine.SceneComponent|GetRelativeLocation _clawmesh))
  (bind (_x _y _z) (Math|Vector|BreakVector _relativelocation))
  (Utilities|FlowControl|DoOnce false :!label _label
    (:Completed
      (Variables|Default|Setinit%20y (.Y (Math|Vector|BreakVector (Variables|/Script/Engine.SceneComponent|GetRelativeLocation (Variables|Default|GetClawMesh)))))
      (bind _asbp_kaiju_character (Utilities|Casting|CastToBP_KaijuCharacter (Game|GetPlayerCharacter 0))
        (:then
          (Variables|Default|Setto%20right (or _returnvalue_2 (and (== _returnvalue 0.0) (Utilities|Enum|Equal(Enum) (Variables|/Script/Neokaiju.KaijuMovementComponent|GetFacingDirection (Variables|/Script/Neokaiju.KaijuCharacter|GetKaijuMovement _asbp_kaiju_character)) "RIGHT"))))
          (bind _x_alpha (Timeline|Timeline_0 PlayFromStart)
            (:Update
              (Transformation|SetRelativeLocation _clawmesh (Math|Vector|MakeVector _x (+ (* _x_alpha (Variables|Default|Getshake%20amplitude) (Math|Float|SelectFloat 1.0 -1.0 (Variables|Default|Getto%20right))) (Variables|Default|Getinit%20y)) _z) false false))
            (:Finished
              (goto _label Reset))))
        (:CastFailed
          (Variables|Default|Setto%20right _returnvalue_2)
          (Timeline|Timeline_0 PlayFromStart))))))

(event EventPlayonReleaseFX
  (Class|Claw|StartPauseforAnimations)
  (Variables|Default|SetCanReady false)
  (Animation|Montage|PlayMontage (Variables|Default|GetClawMesh) "/Game/NeoKaiju/Structures/Attachments/Claw/Art/Animations/AM_ClawBreak.AM_ClawBreak" 1.5 0.0 "Default"
    (:OnNotifyBegin
      (Variables|Default|SetCanReady true)
      (if (Variables|Default|GetNeedsReady)
        (Class|Claw|PlayonReadyFX)))))

(event EventPlayonClawExtendFX
  (CallFunction|PlayEventAttached (Variables|Default|GetClawExtendSoundEvent) (Variables|Default|GetClawMesh)))

(event EventPlayonClawMoveFX)

(event EventStoponClawMoveFX)

(event EventTick
  (params (DeltaSeconds :type Float%20%28single-precision%29)))

(event Collision|EventActorBeginOverlap
  (params (OtherActor :type Actor%20Object%20Reference)))

(event EventPlayonReadyFX
  ;[1 1 1] Don't want to ready over and over if player goes back and forth over bounding box. Also if we are told to ready but we are still in break animation, tell release event we need to be readied when its done
  (if (Variables|Default|GetCanReady)
    (Variables|Default|SetCanReady false)
    (Class|Claw|StartPauseforAnimations)
    (Animation|Montage|PlayMontage (Variables|Default|GetClawMesh) "/Game/NeoKaiju/Structures/Attachments/Claw/Art/Animations/AM_ClawReady.AM_ClawReady" 1.0 0.0 "Default"
      (:OnNotifyBegin
        (Animation|Montage|PlayMontage (Variables|Default|GetClawMesh) "/Game/NeoKaiju/Structures/Attachments/Claw/Art/Animations/AM_ClawGrab.AM_ClawGrab" 3.0 0.0 "Default"
          (:OnNotifyBegin
            (Animation|Montage|PlayMontage (Variables|Default|GetClawMesh) "/Game/NeoKaiju/Structures/Attachments/Claw/Art/Animations/AM_ClawGrab.AM_ClawGrab" -1.0 1.0 "Default"
              (:OnNotifyBegin
                (Utilities|FlowControl|Delay 0.2)
                (Variables|Default|SetCanReady true)
                (Variables|Default|SetNeedsReady false)
                (Class|Claw|StopPauseforAnimations)))))))
    (else
      (Variables|Default|SetNeedsReady true))))

(fn ConstructionScript)