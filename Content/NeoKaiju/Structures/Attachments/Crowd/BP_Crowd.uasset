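; Structure attachment that spawns a fleeing crowd Niagara effect the first time a kaiju enters its detection box, sized in blocks unless customized.
; The effect receives crowd size and lifetime, and Tick, disabled until then, slides it along X away from the player kaiju.
; When the kaiju changes sides, movement reverses and a mirrored vector is sent to the effect.
; The actor destroys itself once the effect is no longer valid.
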(event OnComponentBeginOverlap(KaijuDetectionBox)
  (params (OverlappedComponent :type Primitive%20Component%20Object%20Reference) (OtherActor :type Actor%20Object%20Reference) (OtherComp :type Primitive%20Component%20Object%20Reference) (OtherBodyIndex :type Integer) (bFromSweep :type Boolean) (SweepResult :type Hit%20Result%20Structure%20%28by%20ref%29))
  (bind _defaultsceneroot (Variables|Default|GetDefaultSceneRoot))
  (bind _returnvalue (Transformation|GetWorldLocation _defaultsceneroot))
  (Utilities|Casting|CastToBP_KaijuCharacter OtherActor)
  (Utilities|FlowControl|DoOnce false
    (:Completed
      (bind _returnvalue_2 (Niagara|SpawnSystematLocation "/Game/NeoKaiju/Structures/Attachments/Crowd/PS_Crowd.PS_Crowd" (Math|Vector|MakeVector (.x _returnvalue) (.y _returnvalue) (+ (.z _returnvalue) 15.0)) "0, 0, 0" "1.000000,1.000000,1.000000" true false))
      (Variables|Default|SetNS_Crowd _returnvalue_2)
      (Class|NiagaraComponent|SetVariableInt (Variables|Default|GetNS_Crowd) "User.CrowdSize" (Variables|Default|GetCrowdSize))
      (Niagara|SetNiagaraVariable(Float) (Variables|Default|GetNS_Crowd) "User.CrowdLifetime" (Variables|Default|GetCrowdLifetime%28inSeconds%29))
      (Components|Activation|Activate (Variables|Default|GetNS_Crowd) false)
      (bind _iskaijuonleft (CallFunction|KaijuonLeft))
      (Variables|Default|SetIsKaijuOnLeft _iskaijuonleft)
      (Niagara|SetNiagaraVariable(Vector3) (Variables|Default|GetNS_Crowd) "None" (select _iskaijuonleft (Math|Vector|MakeVector 1.0 1.0 0.0) (Math|Vector|MakeVector 1.0 -1.0 0.0)))
      (Actor|Tick|SetActorTickEnabled true))))

(event EventBeginPlay
  (Actor|Tick|SetActorTickEnabled false)
  (if (not (Variables|Default|GetCustomizedDetectionBox))
    (Components|Box|SetBoxExtent (Variables|Default|GetKaijuDetectionBox) (Math|Vector|MakeVector (* (Variables|Default|GetKaijuDetectionDistance%28inNumBlocks%29) 1e+02) 2e+02 5e+01) true)))

(event EventTick
  (params (DeltaSeconds :type Float%20%28single-precision%29))
  (bind _ns_crowd (Variables|Default|GetNS_Crowd))
  (bind _returnvalue (Transformation|GetWorldLocation _ns_crowd))
  (Utilities|IsValid (Variables|Default|GetNS_Crowd)
    (:Is%20Valid
      (Transformation|SetWorldLocation (Variables|Default|GetNS_Crowd) (Math|Vector|MakeVector (+ (.x _returnvalue) (* DeltaSeconds (Variables|Default|GetCrowdSpeed) (select (Variables|Default|GetIsKaijuOnLeft) (Math|Float|MakeLiteralFloat -1.0) (Math|Float|MakeLiteralFloat 1.0)))) (.y _returnvalue) (.z _returnvalue)) false true)
      (bind _iskaijuonleft (CallFunction|KaijuonLeft))
      (if (Math|Boolean|NotEqual(Boolean) _iskaijuonleft (Variables|Default|GetIsKaijuOnLeft))
        (Variables|Default|SetIsKaijuOnLeft _iskaijuonleft)
        (Niagara|SetNiagaraVariable(Vector3) (Variables|Default|GetNS_Crowd) "None" (select _iskaijuonleft (Math|Vector|MakeVector 1.0 1.0 0.0) (Math|Vector|MakeVector 1.0 -1.0 0.0)))))
    (:Is%20Not%20Valid
      (Actor|DestroyActor))))

(fn ConstructionScript)

(fn KaijuonLeft
  (bind _askaiju_character (Utilities|Casting|CastToKaijuCharacter (Game|GetPlayerCharacter 0)))
  (if (> (- (.x (Transformation|GetWorldLocation (Variables|/Script/Engine.Character|GetMesh _askaiju_character))) (.x (Transformation|GetWorldLocation (Variables|Default|GetNS_Crowd)))) 0.0)
    (return true)
    (else
      (return false))))