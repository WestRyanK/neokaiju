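; Gameplay ability that lets the kaiju character grab and throw, with rubble chomp and throw feedback events.
; Activation plays the grab montage, and OnGrab fires the chomp event at the avatar's location.
; OnThrow plays an upward or downward throw montage based on the vertical aim direction, then fires the throw event.
; A timer-driven mesh spin for throwing remains in the graph but its starting logic is disconnected.
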(event Custom|ThrowAnimationTick
  (bind _duration (Variables|Default|GetDuration))
  (bind _tickspeed (Variables|Default|GetTickSpeed))
  (bind _returnvalue (/ _duration _tickspeed))
  (Transformation|AddRelativeRotation (Variables|/Script/Engine.Character|GetMesh (Variables|Default|GetCharacter)) (Math|Rotator|MakeRotator 0.0 0.0 (/ (Variables|Default|GetRotateDegrees) _returnvalue)) false false)
  (Math|Integer|IncrementInt (Variables|Default|GetTickCount)
    (:%20%20
      (if (< _returnvalue (Math|Conversions|ToFloat(Integer) (Variables|Default|GetTickCount)))
        (Utilities|Time|ClearandInvalidateTimerbyHandle (Variables|Default|GetThrowAnimationTimerHandle))
        (Transformation|SetRelativeRotation (Variables|/Script/Engine.Character|GetMesh (Variables|Default|GetCharacter)) "0, 0, 0" false false)))))

(event Ability|EventActivateAbility
  (CallFunction|PlayGrabAM))

(event Ability|EventOnEndAbility
  (params (bWasCancelled :type Boolean)))

(event EventOnThrow
  (CallFunction|PlayThrowAM)
  (CallFunction|PlayEvent "/Game/Neokaiju/Audio/Events/Abilities/Throw_Rubble.Throw_Rubble" (Transformation|GetActorLocation (Ability|GetAvatarActorfromActorInfo))))

(event EventOnGrab
  (CallFunction|PlayEvent "/Game/Neokaiju/Audio/Events/Abilities/Chomp_Rubble.Chomp_Rubble" (Transformation|GetActorLocation (Ability|GetAvatarActorfromActorInfo))))

(fn PlayGrabAM
  (bind _askaiju_character (Utilities|Casting|CastToKaijuCharacter (Ability|GetAvatarActorfromActorInfo)))
  (Animation|PlayAnimMontage _askaiju_character "/Game/NeoKaiju/Ability/StandardAbilities/GrabAbility/KaijuCharacter_grab_2_Montage.KaijuCharacter_grab_2_Montage" 1.0 "start")
  (return))

(fn PlayThrowAM
  (bind _askaiju_character (Utilities|Casting|CastToKaijuCharacter (Ability|GetAvatarActorfromActorInfo)))
  (if (>= (.z (Variables|Default|GetAimDirection)) 0.0)
    (Animation|PlayAnimMontage _askaiju_character "/Game/NeoKaiju/Ability/StandardAbilities/GrabAbility/KaijuCharacter_throw_up_Montage.KaijuCharacter_throw_up_Montage" 1.0 "default")
    (else
      (Animation|PlayAnimMontage _askaiju_character "/Game/NeoKaiju/Ability/StandardAbilities/GrabAbility/KaijuCharacter_throw_down_Montage.KaijuCharacter_throw_down_Montage" 1.0 "Default")))
  (return))