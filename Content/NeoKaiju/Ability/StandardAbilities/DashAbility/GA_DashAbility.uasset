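; Kaiju dash Gameplay Ability that handles the dash's feedback and facing through start, tick, hit, impede and complete events.
; Start plays sound, alternates montages by chain-count parity, and spawns Niagara smoke and speed lines chosen by direction and an attribute-indexed tier.
; Tick turns the character's rotation point toward the dash with safe pitch rotation; hit triggers force feedback.
; Impede adds bonk effects; both endings stop particle spawning before delayed cleanup.
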(event Custom|OnFacingDirectionFlipped
  (params (FacingDirection :type EFacingDirection%20Enum :default "RIGHT"))
  (switch Utilities|FlowControl|Switch|SwitchonEFacingDirection FacingDirection
    (:RIGHT
      (Variables|Ability|Dash|SetDashSystem_Lines "/Game/NeoKaiju/Ability/StandardAbilities/DashAbility/Particles/PS_Dash_Lines_Right_LVL1.PS_Dash_Lines_Right_LVL1")
      (Variables|Ability|Dash|SetDashSystem "/Game/NeoKaiju/Ability/StandardAbilities/DashAbility/Particles/PS_Dash_Smoke_Right_LVL1.PS_Dash_Smoke_Right_LVL1"))
    (:LEFT
      (Variables|Ability|Dash|SetDashSystem_Lines "/Game/NeoKaiju/Ability/StandardAbilities/DashAbility/Particles/OldAssets/PS_Dash_Lines_Left.PS_Dash_Lines_Left")
      (Variables|Ability|Dash|SetDashSystem "/Game/NeoKaiju/Ability/StandardAbilities/DashAbility/Particles/PS_Dash_Smoke_Left_LVL1.PS_Dash_Smoke_Left_LVL1"))))

(event Ability|EventActivateAbility)

(event Ability|EventOnEndAbility
  (params (bWasCancelled :type Boolean)))

(event EventOnDashStart
  (params (DashDirection :type Vector :default "0, 0, 0") (ChainedDashCountOfDash :type Integer))
  (Variables|Ability|Dash|SetDashDirection DashDirection)
  (bind _askaiju_character (Utilities|Casting|CastToKaijuCharacter (Ability|GetAvatarActorfromActorInfo)))
  (Variables|Default|SetRotationPoint (Variables|/Script/Neokaiju.KaijuCharacter|GetCharacterRotationPoint _askaiju_character))
  (CallFunction|PlayDashSound)
  (CallFunction|SpawnDashParticles)
  (CallFunction|PlayDashAM ChainedDashCountOfDash))

(event EventOnDashComplete
  (CallFunction|StopDashSystem)
  (CallFunction|DestroySystemsDelayed 5.0))

(event EventOnDashImpede
  (CallFunction|PlayImpededSound)
  (CallFunction|StopDashSystem)
  (CallFunction|DestroySystemsDelayed 5.0)
  (CallFunction|PlayBonkAM))

(event EventOnDashTick
  (params (DeltaTime :type Float%20%28single-precision%29) (DashDirection :type Vector :default "0, 0, 0"))
  (CallFunction|FaceActortoDashDirection DeltaTime DashDirection))

(event EventOnDashHit
  (params (bWasImpeded :type Boolean))
  (Game|Feedback|ClientPlayForceFeedback (Game|GetPlayerController 0) (Variables|Ability|Dash|GetDashForceFeedback) "None" false true false))

(fn FaceActortoDashDirection
  (params (DeltaTime :type Float%20%28single-precision%29) (Dash%20Direction :type Vector))
  (bind _rotationpoint (Variables|Default|GetRotationPoint))
  (Transformation|SetWorldRotation (Variables|Default|GetRotationPoint) (Class|SafeDirectionUtility|GetSafePitchRotation (Math|Vector|GetRightVector _rotationpoint) (Math|Vector|GetForwardVector _rotationpoint) Dash%20Direction "0, 0, 0" "0, 0, 0" (Variables|Ability|Dash|GetDashRotateSpeed) DeltaTime false) false false))

(fn PlayImpededSound
  (Class|FMODBlueprintStatics|PlayEventAttached (Variables|Ability|Bounce|GetDashImpededSoundEvent) (Variables|/Script/Engine.Actor|GetRootComponent (Ability|GetAvatarActorfromActorInfo)) "None" "0, 0, 0" "KeepRelativeOffset")
  (Niagara|SpawnSystemAttached "/Game/NeoKaiju/Ability/StandardAbilities/DashAbility/Particles/PS_DashCollision.PS_DashCollision" (Class|GameplayAbility|GetOwningComponentfromActorInfo) "None" "0, 0, 0" "0,-90.000000, 0" "KeepRelativeOffset" false))

(fn StopDashSystem
  (CallFunction|DestroyifValid (Variables|Ability|Dash|GetSpawnedDashSystem_Point))
  (Utilities|IsValid (Variables|Ability|Dash|GetSpawnedDashSystem)
    (:Is%20Valid
      (Niagara|SetNiagaraVariable(Float) (Variables|Ability|Dash|GetSpawnedDashSystem) "SpawnRate" 0.0)
      (for _array_element (Actor|GetComponentsByClass (Ability|GetOwningActorfromActorInfo) "/Script/Niagara.NiagaraComponent")
        (Niagara|SetNiagaraVariable(Float) _array_element "SpawnDash" 0.0)
        (Niagara|SetNiagaraVariable(Vector3) _array_element "SpeedBoost" "0, 0, 0")))))

(fn PlayDashSound
  (Class|FMODBlueprintStatics|PlayEventAttached (Variables|Ability|Dash|GetDashSoundEvent) (Variables|Default|GetRotationPoint) "None" "0, 0, 0" "KeepRelativeOffset"))

(fn SpawnDashParticles
  (bind _returnvalue (Ability|GetOwningActorfromActorInfo))
  (bind _returnvalue_2 (Ability|GetAvatarActorfromActorInfo))
  (bind _dashdirection (Variables|Ability|Dash|GetDashDirection))
  (bind _x (Math|Vector|BreakVector _dashdirection))
  (bind _returnvalue_3 (Ability|GetAbilitySystemComponent _returnvalue_2))
  (bind _x_2 (Math|Vector|BreakVector _dashdirection))
  (bind _returnvalue_4 (Ability|GetAbilitySystemComponent _returnvalue))
  (bind _returnvalue_5 (Ability|Attribute|GetFloatAttributefromAbilitySystemComponent _returnvalue_4 "(AttributeName=\"KaijuLevel\",Attribute=StructProperty'\"/Script/Neokaiju.KaijuAttributeSet:KaijuLevel\"',AttributeOwner=Class'\"/Script/Neokaiju.KaijuAttributeSet\"')"))
  (bind _returnvalue_6 (GameplayTags|HasMatchingGameplayTag _returnvalue_3 "(TagName=\"Ability.Standard.Dash\")"))
  (bind _returnvalue_7 (Math|Float|Truncate _returnvalue_5))
  (bind _returnvalue_8 (- _returnvalue_7 1))
  (LocalVariables|SetMeshComponent (Utilities|Array|Get(acopy) (Actor|GetComponentsByClass (Ability|GetOwningActorfromActorInfo) "/Script/Engine.SkeletalMeshComponent")))
  (Variables|Ability|Dash|SetDashSystem "/Game/NeoKaiju/Ability/StandardAbilities/DashAbility/Particles/PS_Dash_Smoke_Right_LVL1.PS_Dash_Smoke_Right_LVL1")
  (Variables|Ability|Dash|SetDashSystem_Reverse "/Game/NeoKaiju/Ability/StandardAbilities/DashAbility/Particles/PS_Dash_Smoke_Left_LVL1.PS_Dash_Smoke_Left_LVL1")
  (Variables|Ability|Dash|SetDashSystem_Lines (Utilities|Array|Get(acopy) (Variables|Ability|Dash|GetDashSystem_Forward_Lines) _returnvalue_8))
  (Variables|Ability|Dash|SetDashSystem_Lines_Reverse (Utilities|Array|Get(acopy) (Variables|Ability|Dash|GetDashSystem_Backward_Lines) _returnvalue_8))
  (Variables|Ability|Dash|SetDashSystem (Utilities|Array|Get(acopy) (Variables|Ability|Dash|GetDashSystem_array) _returnvalue_8))
  (Variables|Ability|Dash|SetDashSystem_Reverse (Utilities|Array|Get(acopy) (Variables|Ability|Dash|GetDashSystem_Reverse_array) _returnvalue_8))
  (Utilities|FlowControl|Sequence
    (:then_0
      (if (Math|Boolean|ANDBoolean (>= _x 0.8) (<= _x 1.1) _returnvalue_6)
        (CallFunction|DestroyifValid (Variables|Ability|Dash|GetSpawnedDashSystem))
        (bind _returnvalue_9 (Niagara|SpawnSystemAttached (Variables|Ability|Dash|GetDashSystem) (LocalVariables|GetMeshComponent) "" "-75.000000,0.000000,5.000000" "0, 0, 0" "KeepRelativeOffset" true))
        (bind _output_get (Variables|Ability|Dash|SetSpawnedDashSystem _returnvalue_9))
        (Niagara|SetNiagaraVariable(Float) _output_get "SpawnRate" 4e+01)
        (elif (Math|Boolean|ANDBoolean (>= _x_2 -1.1) (<= _x_2 -0.8) _returnvalue_6)
          (CallFunction|DestroyifValid (Variables|Ability|Dash|GetSpawnedDashSystem))
          (bind _returnvalue_10 (Niagara|SpawnSystemAttached (Variables|Ability|Dash|GetDashSystem_Reverse) (LocalVariables|GetMeshComponent) "" "-75.000000,0.000000,5.000000" "0, 0, 0" "KeepRelativeOffset" true))
          (bind _output_get_2 (Variables|Ability|Dash|SetSpawnedDashSystem _returnvalue_10))
          (Niagara|SetNiagaraVariable(Float) _output_get_2 "SpawnRate" 4e+01))))
    (:then_1
      (if (>= (.X (Math|Vector|BreakVector (Variables|Ability|Dash|GetDashDirection))) 0.0)
        (CallFunction|DestroyifValid (Variables|Ability|Dash|GetSpawnedDashSystem_Lines))
        (bind _askaiju_character (Utilities|Casting|CastToKaijuCharacter (Ability|GetAvatarActorfromActorInfo)))
        (bind _returnvalue_11 (Niagara|SpawnSystemAttached (Variables|Ability|Dash|GetDashSystem_Lines) (Variables|/Script/Neokaiju.KaijuCharacter|GetCharacterRotationPoint _askaiju_character) "" "0.000000,10.000000,0.000000" "0, 0, 0" "SnapToTarget" false))
        (bind _output_get_3 (Variables|Ability|Dash|SetSpawnedDashSystem_Lines _returnvalue_11))
        (Niagara|SetNiagaraVariable(Float) _output_get_3 "SpawnRate" 45.0)
        (else
          (CallFunction|DestroyifValid (Variables|Ability|Dash|GetSpawnedDashSystem_Lines))
          (bind _askaiju_character_2 (Utilities|Casting|CastToKaijuCharacter (Ability|GetAvatarActorfromActorInfo)))
          (bind _returnvalue_12 (Niagara|SpawnSystemAttached (Variables|Ability|Dash|GetDashSystem_Lines_Reverse) (Variables|/Script/Neokaiju.KaijuCharacter|GetCharacterRotationPoint _askaiju_character_2) "" "0.000000,10.000000,0.000000" "0, 0, 0" "SnapToTarget" false))
          (bind _output_get_4 (Variables|Ability|Dash|SetSpawnedDashSystem_Lines _returnvalue_12))
          (Niagara|SetNiagaraVariable(Float) _output_get_4 "SpawnRate" 45.0))))
    (:then_3
      (for _array_element (Actor|GetComponentsByClass (Ability|GetOwningActorfromActorInfo) "/Script/Niagara.NiagaraComponent")
        (Niagara|SetNiagaraVariable(Float) _array_element "SpawnDash" 35.0)))))

(fn DestroySystemsDelayedEvent
  (CallFunction|DestroyifValid (Variables|Ability|Dash|GetSpawnedDashSystem))
  (CallFunction|DestroyifValid (Variables|Ability|Dash|GetSpawnedDashSystem_Lines)))

(fn DestroySystemsDelayed
  (params (Delay :type Float%20%28single-precision%29))
  (Utilities|IsValid (Variables|Ability|Dash|GetSpawnedDashSystem_Lines)
    (:Is%20Valid
      (Niagara|SetNiagaraVariable(Float) (Variables|Ability|Dash|GetSpawnedDashSystem_Lines) "SpawnRate" 0.0))
    (:Is%20Not%20Valid
      _))
  (Utilities|Time|SetTimerbyEvent (EventDispatchers|CreateEvent :!event DestroySystemsDelayedEvent) Delay))

(fn PlayDashAM
  (params (ChainedDashCount :type Integer))
  (bind _askaiju_character (Utilities|Casting|CastToKaijuCharacter (Ability|GetAvatarActorfromActorInfo)))
  (if (== (Math|Integer|%(Integer) ChainedDashCount 2) 0)
    (Animation|PlayAnimMontage _askaiju_character "/Game/NeoKaiju/Ability/StandardAbilities/DashAbility/AM_KaijuCharacter_dash_torpedo.AM_KaijuCharacter_dash_torpedo" 1.0 "start")
    (else
      (Animation|PlayAnimMontage _askaiju_character "/Game/NeoKaiju/Ability/StandardAbilities/DashAbility/AM_KaijuCharacter_dash.AM_KaijuCharacter_dash" 1.0 "start"))))

(fn PlayBonkAM
  (bind _askaiju_character (Utilities|Casting|CastToKaijuCharacter (Ability|GetAvatarActorfromActorInfo)))
  (Animation|PlayAnimMontage _askaiju_character "/Game/NeoKaiju/Ability/StandardAbilities/DashAbility/AM_KaijuCharacter_bonk.AM_KaijuCharacter_bonk" 1.0 "default"))