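; Older wall jump gameplay ability, named as OLD, that supplies the audio and visual feedback for each jump.
; The Blueprint only handles the OnJump event, leaving activation and end events empty.
; OnJump plays a sound event at the avatar's location and attaches a particle emitter to the supplied component socket, each if its asset is valid.
; A volume scale based on consecutive jump count is computed but left unconnected.
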(event Ability|EventActivateAbility)

(event Ability|EventOnEndAbility
  (params (bWasCancelled :type Boolean)))

(event EventOnJump
  (params (Component :type Scene%20Component%20Object%20Reference) (SocketName :type Name :default "None") (ConsecutiveJumpCount :type Integer))
  (CallFunction|PlayJumpSound ConsecutiveJumpCount)
  (CallFunction|PlayJumpParticleEffect Component SocketName))

(fn PlayJumpSound
  (params (ConsecutiveJumpCount :type Integer))
  (if (Utilities|IsValid (Variables|Ability|Jump|GetWallJumpSoundEvent))
    (CallFunction|PlayEvent (Variables|Ability|Jump|GetWallJumpSoundEvent) (Transformation|GetActorLocation (Ability|GetAvatarActorfromActorInfo)))))

(fn PlayJumpParticleEffect
  (params (FeetPosition :type Scene%20Component%20Object%20Reference) (AttachPointName :type Name))
  (if (Utilities|IsValid (Variables|Ability|Jump|GetJumpParticleEffect))
    (Effects|SpawnEmitterAttached (Variables|Ability|Jump|GetJumpParticleEffect) FeetPosition AttachPointName)))