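; Gameplay ability Blueprint that adds sound and visual feedback when a character jumps.
; OnJump plays a jump or double-jump sound event at the avatar's location, chosen by consecutive jump count and gated only on JumpSoundEvent validity.
; It also attaches the DoubleJump effect system to the supplied component socket on every jump.
; Activation and end events are empty, and an older emitter spawn is left disconnected.
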(event Ability|EventActivateAbility)

(event Ability|EventOnEndAbility
  (params (bWasCancelled :type Boolean)))

(event EventOnJump
  (params (Component :type Scene%20Component%20Object%20Reference) (SocketName :type Name :default "None") (ConsecutiveJumpCount :type Integer))
  (CallFunction|PlayJumpSound ConsecutiveJumpCount)
  (Niagara|SpawnSystemAttached "/Game/NeoKaiju/Particles/DoubleJump.DoubleJump" Component SocketName "0, 0, 0" "0, 0, 0" "KeepRelativeOffset" false))

(fn PlayJumpSound
  (params (ConsecutiveJumpCount :type Integer))
  (if (Utilities|IsValid (Variables|Ability|Jump|GetJumpSoundEvent))
    (CallFunction|PlayEvent (select (> ConsecutiveJumpCount 0) (Variables|Ability|Jump|GetDoubleJumpSoundEvent) (Variables|Ability|Jump|GetJumpSoundEvent)) (Transformation|GetActorLocation (Ability|GetAvatarActorfromActorInfo)))))