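; Gameplay ability for the gravity-altering jump, with this Blueprint supplying the jump's feedback through the OnJump event.
; Each jump spawns an attached Niagara effect on the given socket and plays controller force feedback on player 0.
; PlayJumpSound uses a double-jump event for consecutive jumps, otherwise indexing an array of sound events by a truncated attribute value from the avatar.
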(event Ability|EventActivateAbility)

(event Ability|EventOnEndAbility
  (params (bWasCancelled :type Boolean)))

(event EventOnJump
  (params (Component :type Scene%20Component%20Object%20Reference) (SocketName :type Name :default "None") (ConsecutiveJumpCount :type Integer))
  (CallFunction|PlayJumpSound ConsecutiveJumpCount)
  (Niagara|SpawnSystemAttached (Variables|Ability|Jump|GetJumpEffect) Component SocketName "-10.000000,0.000000,50.000000" "-20.000000, 0, 0" "KeepRelativeOffset" true)
  (Game|Feedback|ClientPlayForceFeedback (Game|GetPlayerController 0) (Variables|Ability|Jump|GetJumpForceFeedback) "None" false false false))

(fn PlayJumpSound
  (params (Consecutive%20Jump%20Count :type Integer))
  (CallFunction|PlayEvent (select (> Consecutive%20Jump%20Count 0) (Variables|Ability|Jump|GetDoubleJumpSoundEvent) (CallFunction|GetSoundEventfromLevel)) (Transformation|GetActorLocation (Ability|GetAvatarActorfromActorInfo))))

(fn GetSoundEventfromLevel
  (return (Utilities|Array|Get(acopy) (Variables|Ability|Jump|GetJumpSoundEvent) (Math|Float|Truncate (.ReturnValue (Ability|Attribute|GetFloatAttribute (Ability|GetAvatarActorfromActorInfo) "(AttributeName=\"KaijuLevel\",Attribute=StructProperty'\"/Script/Neokaiju.KaijuAttributeSet:KaijuLevel\"',AttributeOwner=Class'\"/Script/Neokaiju.KaijuAttributeSet\"')"))))))