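; Gameplay ability Blueprint for a curve-driven jump, adding the audio and visual feedback when the avatar jumps.
; On each jump event it plays a jump or double-jump sound at the avatar's location, chosen by the consecutive jump count.
; It also spawns the jump particle effect attached to the supplied component socket.
; The sound plays only when both sound events are set; activation and end events are unused.
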(event Ability|EventActivateAbility)

(event Ability|EventOnEndAbility
  (params (bWasCancelled :type Boolean)))

(event EventOnJump
  (params (Component :type Scene%20Component%20Object%20Reference) (SocketName :type Name :default "None") (ConsecutiveJumpCount :type Integer))
  (CallFunction|PlayJumpSound ConsecutiveJumpCount)
  (Effects|SpawnEmitterAttached (Variables|Ability|Jump|GetJump%20Effect) Component SocketName))

(fn PlayJumpSound
  (params (Consecutive%20Jump%20Count :type Integer))
  (if (and (Utilities|IsValid (Variables|Ability|Jump|GetJump%20Sound%20Event)) (Utilities|IsValid (Variables|Ability|Jump|GetDouble%20Jump%20Sound%20Event)))
    (CallFunction|PlayEvent (select (> Consecutive%20Jump%20Count 0) (Variables|Ability|Jump|GetDouble%20Jump%20Sound%20Event) (Variables|Ability|Jump|GetJump%20Sound%20Event)) (Transformation|GetActorLocation (Ability|GetAvatarActorfromActorInfo)))))