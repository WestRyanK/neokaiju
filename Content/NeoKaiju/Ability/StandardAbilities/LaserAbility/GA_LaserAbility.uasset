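; Gameplay Ability for the kaiju's charged laser, implementing montage, VFX, audio and rumble for charge and fire phase events.
; Charging picks a ground or air montage, attaches charge effects and levels the kaiju.
; Firing spawns socket-attached beam effects tiered by an ability attribute, then each tick updates beam, impact, random damage decals and the character's aim angle.
; Cleanup zeroes impact emitter rates before a delayed timer.
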(event EventOnFireLaserTick
  (params (LaserAimDirection :type Vector :default "0, 0, 0") (LaserHit :type Hit%20Result%20Structure))
  ;[1 1 1] Fire Laser
  (Fire|UpdateFireLaserBeam LaserAimDirection LaserHit)
  (Fire|UpdateFireLaserImpact LaserAimDirection LaserHit)
  (Fire|UpdateFireLaserDecals LaserHit)
  (CallFunction|SetAimDirectioninKaijuBP LaserAimDirection))

(event EventOnFireLaserComplete
  ;[1 1 1] Fire Laser
  (Fire|StopFireForceFeedback)
  (CallFunction|CleanUpFireLaser))

(event EventOnFireLaserStart
  (params (SocketName :type Name :default "None") (LaserSocketComponent :type Scene%20Component%20Object%20Reference))
  ;[1 1 1] Fire Laser
  (CallFunction|SaveSocketInfo SocketName LaserSocketComponent)
  (Variables|Default|SetbHasHit false)
  (Fire|PlayFireLaserSound)
  (Fire|PlayFireForceFeedback)
  (CallFunction|SpawnFireLaserBeam "10.000000, 0, 0"))

(event EventOnChargeLaserComplete
  ;[1 1 1] Charge Laser
  (Charge|CleanUpChargeLaser)
  (CallFunction|StopAnimMontage))

(event EventOnChargeLaserCancel
  ;[1 1 1] Charge Laser
  (CallFunction|StopAnimMontage)
  (Charge|CleanUpChargeLaser))

(event EventOnChargeLaserTick
  (params (TimeRemaining :type Float%20%28single-precision%29))
  ;[1 1 1] Charge Laser
  (Charge|UpdateChargeLaserSound 0 TimeRemaining))

(event EventOnChargeLaserStart
  (params (SocketName :type Name :default "None") (LaserSocketComponent :type Scene%20Component%20Object%20Reference))
  ;[1 1 1] Charge Laser
  (CallFunction|SaveSocketInfo SocketName LaserSocketComponent)
  (bind _asbp_kaiju_character (Utilities|Casting|CastToBP_KaijuCharacter (Ability|GetOwningActorfromActorInfo)))
  (bind _output_get (Variables|/Game/NeoKaiju/KaijuCharacter/BP_KaijuCharacter.BP_KaijuCharacter_C|SetlaserStartedInAir _asbp_kaiju_character (Variables|Default|GetbStartedInAir)))
  (if _output_get
    (CallFunction|PlayLaserMontage "/Game/NeoKaiju/Ability/StandardAbilities/LaserAbility/AM_KaijuCharacter_laser_air_charge.AM_KaijuCharacter_laser_air_charge")
    (else
      (CallFunction|PlayLaserMontage "/Game/NeoKaiju/Ability/StandardAbilities/LaserAbility/KaijuCharacter_Laser_Montage_v3.KaijuCharacter_Laser_Montage_v3")))
  (Charge|SpawnChargeLaserSystem)
  (CallFunction|LevelKaijutoGround))

(fn UpdateFireLaserBeam
  (params (Laser%20Aim%20Direction :type Vector) (Laser%20Hit :type Hit%20Result%20Structure))
  (bind (_bblockinghit _binitialoverlap _time _distance _location _impactpoint _normal _impactnormal _physmat _hitactor _hitcomponent _hitbonename _hititem _faceindex _tracestart _traceend) (Collision|BreakHitResult Laser%20Hit))
  (if (and (Utilities|IsValid (Variables|Fire|GetSpawnedFireLaserBeam)) (Utilities|IsValid (Variables|Fire|GetLaserStartSpawned)))
    (Transformation|SetWorldScale3D (Variables|Fire|GetSpawnedFireLaserBeam) (Math|Vector|VectorGetAbs (Transformation|GetWorldScale (Variables|Fire|GetSpawnedFireLaserBeam))))
    (Effects|Components|ParticleSystem|SetVectorParameter (Variables|Fire|GetSpawnedFireLaserBeam) "LaserTarget" (.ImpactPoint (Collision|BreakHitResult Laser%20Hit)))
    (Transformation|SetWorldRotation (Variables|Fire|GetLaserStartSpawned) (Math|Rotator|FindLookatRotation _traceend _tracestart) false false)))

(fn PlayFireLaserSound
  (bind _returnvalue (Class|FMODBlueprintStatics|EventInstanceIsValid (Variables|Fire|GetSpawnedFireLaserSoundEvent)))
  (if (and (not _returnvalue) (Utilities|IsValid (Variables|Fire|GetFireLaserSoundEvent)))
    (bind _eventinstance (CallFunction|PlayEvent (Variables|Fire|GetFireLaserSoundEvent) (Transformation|GetActorLocation (Ability|GetAvatarActorfromActorInfo))))
    (Variables|Fire|SetSpawnedFireLaserSoundEvent _eventinstance)))

(fn UpdateFireLaserImpact
  (params (Laser%20Aim%20Direction :type Vector) (Laser%20Hit :type Hit%20Result%20Structure))
  (bind (_bblockinghit _binitialoverlap _time _distance _location _impactpoint _normal _impactnormal) (Collision|BreakHitResult Laser%20Hit))
  (Utilities|FlowControl|Sequence
    (:then_0
      (if (.bBlockingHit (Collision|BreakHitResult Laser%20Hit))
        (Variables|Default|SetbHasHit true)))
    (:then_1
      (if (Variables|Default|GetbHasHit)
        ;[1 1 1] Start or Update Impact
        (Utilities|IsValid (Variables|Fire|GetSpawned%20Niagara%20Fire%20Laser%20Impact)
          (:Is%20Valid
            _)
          (:Is%20Not%20Valid
            (bind _returnvalue (Niagara|SpawnSystematLocation (Utilities|Array|Get(acopy) (Variables|Default|GetImpact_Particles) (- (Math|Float|Truncate (.ReturnValue (Ability|Attribute|GetFloatAttributefromAbilitySystemComponent (Ability|GetAbilitySystemComponent (Ability|GetAvatarActorfromActorInfo)) "(AttributeName=\"KaijuLevel\",Attribute=StructProperty'\"/Script/Neokaiju.KaijuAttributeSet:KaijuLevel\"',AttributeOwner=Class'\"/Script/Neokaiju.KaijuAttributeSet\"')"))) 1)) _impactpoint (Math|Conversions|RotationFromXVector _impactnormal)))
            (Variables|Fire|SetSpawned%20Niagara%20Fire%20Laser%20Impact _returnvalue)
            (CallFunction|SetNiagaraSystemValues (Variables|Fire|GetSpawned%20Niagara%20Fire%20Laser%20Impact) (Utilities|Map|MakeMap "CenterRate" 6.0 "DustSprayRate" 5e+01 "FireSprayRate" 25.0 "TrialSphere" 3e+01 "LineRate" 2e+01 "SphereEdge" 8e+01))))
        (Utilities|IsValid (Variables|Fire|GetSpawned%20Niagara%20Fire%20Laser%20Impact)
          (:Is%20Valid
            (Transformation|SetWorldLocation (Variables|Fire|GetSpawned%20Niagara%20Fire%20Laser%20Impact) (.ImpactPoint (Collision|BreakHitResult Laser%20Hit)) false false)
            (Transformation|SetWorldRotation (Variables|Fire|GetSpawned%20Niagara%20Fire%20Laser%20Impact) (Math|Rotator|MakeRotfromZ (.ImpactNormal (Collision|BreakHitResult Laser%20Hit))) false false)))))))

(fn UpdateChargeLaserSound
  (params (Laser%20Start :type Scene%20Component%20Object%20Reference) (Time%20Remaining :type Float%20%28single-precision%29))
  (if (Utilities|IsValid (Variables|Charge|GetChargeLaserSoundEvent))
    (bind _returnvalue (Class|FMODBlueprintStatics|EventInstanceIsValid (Variables|Charge|GetSpawnedChargeLaserSoundEvent)))
    (if (not _returnvalue)
      (bind _eventinstance (CallFunction|PlayEvent (Variables|Charge|GetChargeLaserSoundEvent) (Transformation|GetActorLocation (Ability|GetAvatarActorfromActorInfo))))
      (Variables|Charge|SetSpawnedChargeLaserSoundEvent _eventinstance))))

(fn CleanUpChargeLaser
  (bind _returnvalue (Class|FMODBlueprintStatics|EventInstanceIsValid (Variables|Charge|GetSpawnedChargeLaserSoundEvent)))
  (if _returnvalue
    (Class|FMODBlueprintStatics|EventInstanceStop (Variables|Charge|GetSpawnedChargeLaserSoundEvent) true))
  (if (Utilities|IsValid (Variables|Charge|GetSpawnedChargeLaserSystem))
    (Components|DestroyComponent (Variables|Charge|GetSpawnedChargeLaserSystem))))

(fn SpawnChargeLaserSystem
  (if (Utilities|IsValid (Variables|Charge|GetChargeLaserSystem))
    (if (not (Utilities|IsValid (Variables|Charge|GetSpawnedChargeLaserSystem)))
      (bind _returnvalue (Effects|SpawnEmitterAttached (Variables|Charge|GetChargeLaserSystem) (Variables|Default|GetLaserSocketComponent) (Variables|Default|GetSocketName) "0, 0, 0" "0, 0, 0" "1.000000,1.000000,1.000000" "SnapToTargetIncludingScale"))
      (Variables|Charge|SetSpawnedChargeLaserSystem _returnvalue))))

(fn UpdateFireLaserDecals
  (params (Laser%20Hit :type Hit%20Result%20Structure))
  (bind (_bblockinghit _binitialoverlap _time _distance _location _impactpoint _normal) (Collision|BreakHitResult Laser%20Hit))
  (if (.bBlockingHit (Collision|BreakHitResult Laser%20Hit))
    (Rendering|Decal|SpawnDecalatLocation (Utilities|Select :Index (Math|Random|RandomIntegerinRange 0 2) :Option%200 "/Game/NeoKaiju/Ability/StandardAbilities/LaserAbility/Decals/M_TempDamage1.M_TempDamage1" :Option%201 "/Game/NeoKaiju/Ability/StandardAbilities/LaserAbility/Decals/M_TempDamage2.M_TempDamage2" :Option%202 "/Game/NeoKaiju/Ability/StandardAbilities/LaserAbility/Decals/M_TempDamage3.M_TempDamage3") (Math|Conversions|ToVector(Float) (Math|Random|RandomFloatinRange 3e+01 65.0)) _impactpoint (Math|Rotator|MakeRotfromX _normal) 4.0)))

(fn PlayFireForceFeedback
  (Game|Feedback|ClientPlayForceFeedback (Game|GetPlayerController 0) (Variables|Fire|GetFireLaserForceFeedback) "None" true false false))

(fn StopFireForceFeedback
  (Utilities|IsValid (Game|GetPlayerController 0)
    (:Is%20Valid
      (Game|Feedback|ClientStopForceFeedback (Game|GetPlayerController 0) (Variables|Fire|GetFireLaserForceFeedback) "None"))))

(fn SpawnFireLaserBeam
  (params (OffsetFromStart :type Vector))
  (bind _returnvalue (Ability|GetOwningActorfromActorInfo))
  (bind _returnvalue_2 (Ability|GetAbilitySystemComponent _returnvalue))
  (bind _returnvalue_3 (Ability|Attribute|GetFloatAttributefromAbilitySystemComponent _returnvalue_2 "(AttributeName=\"KaijuLevel\",Attribute=StructProperty'\"/Script/Neokaiju.KaijuAttributeSet:KaijuLevel\"',AttributeOwner=Class'\"/Script/Neokaiju.KaijuAttributeSet\"')"))
  (bind _returnvalue_4 (Math|Float|Truncate _returnvalue_3))
  (bind _returnvalue_5 (- _returnvalue_4 1))
  (Variables|Fire|SetFireLaserBeam (Utilities|Array|Get(acopy) (Variables|Fire|GetFireLaserBeam_Array) _returnvalue_5))
  (if (== _returnvalue_5 3)
    (bind _returnvalue_6 (Niagara|SpawnSystemAttached "/Game/NeoKaiju/Ability/StandardAbilities/LaserAbility/LaserParticles.LaserParticles" (Variables|Default|GetLaserSocketComponent) (Variables|Default|GetSocketName) "0, 0, 0" "0, 0, 0" "SnapToTarget" false))
    (Variables|Default|SetExtra%20Particles%20Large%20Laser _returnvalue_6))
  (bind _returnvalue_7 (Effects|SpawnEmitterAttached (Variables|Fire|GetFireLaserBeam) (Variables|Default|GetLaserSocketComponent) (Variables|Default|GetSocketName) OffsetFromStart "0, 0, 0" (Math|Conversions|ToVector(Float) (.z (Transformation|GetWorldScale (Variables|Default|GetLaserSocketComponent)))) "SnapToTarget"))
  (Variables|Fire|SetSpawnedFireLaserBeam _returnvalue_7)
  (bind _returnvalue_8 (Niagara|SpawnSystemAttached (Variables|Charge|GetLaserNEwStart) (Variables|Default|GetLaserSocketComponent) (Variables|Default|GetSocketName) OffsetFromStart "0, 0, 0" "SnapToTarget" true))
  (Variables|Fire|SetLaserStartSpawned _returnvalue_8)
  (Fire|UpdateFireLaserBeam "0, 0, 0" (Collision|MakeHitResult false false 0.0 0.0 "0, 0, 0" (Transformation|GetSocketLocation (Variables|Default|GetLaserSocketComponent) (Variables|Default|GetSocketName)) "0,0,1" "0,0,1" 0 0)))

(fn CleanUpFireLaser
  (CallFunction|DestroyifValid (Variables|Default|GetExtra%20Particles%20Large%20Laser))
  (CallFunction|DestroyifValid (Variables|Fire|GetSpawnedFireLaserBeam))
  (CallFunction|DestroyifValid (Variables|Fire|GetLaserStartSpawned))
  (Utilities|IsValid (Variables|Fire|GetSpawned%20Niagara%20Fire%20Laser%20Impact)
    (:Is%20Valid
      (CallFunction|SetNiagaraSystemValues (Variables|Fire|GetSpawned%20Niagara%20Fire%20Laser%20Impact) (Utilities|Map|MakeMap "DustSprayRate" 0.0 "FireSprayRate" 0.0 "TrialSphere" 0.0 "LineRate" 0.0 "SphereEdge" 0.0 "CenterRate" 0.0)))
    (:Is%20Not%20Valid
      _))
  (Utilities|Time|SetTimerbyEvent (EventDispatchers|CreateEvent :!event CleanUpImpact) 0.3)
  (bind _returnvalue (Class|FMODBlueprintStatics|EventInstanceIsValid (Variables|Fire|GetSpawnedFireLaserSoundEvent)))
  (if _returnvalue
    (Class|FMODBlueprintStatics|EventInstanceStop (Variables|Fire|GetSpawnedFireLaserSoundEvent) true)))

(fn StopAnimMontage
  (bind _askaiju_character (Utilities|Casting|CastToKaijuCharacter (Ability|GetOwningActorfromActorInfo)))
  (Animation|StopAnimMontage _askaiju_character "/Game/NeoKaiju/Ability/StandardAbilities/LaserAbility/KaijuCharacter_Laser_Montage_v3.KaijuCharacter_Laser_Montage_v3"))

(fn CleanUpImpact
  (CallFunction|DestroyifValid (Variables|Fire|GetSpawned%20Niagara%20Fire%20Laser%20Impact)))

(fn SaveSocketInfo
  (params (SocketName :type Name) (SocketComponent :type Scene%20Component%20Object%20Reference))
  (Variables|Default|SetLaserSocketComponent SocketComponent)
  (Variables|Default|SetSocketName SocketName))

(fn PlayLaserMontage
  (params (NewParam :type Anim%20Montage%20Object%20Reference))
  (bind _askaiju_character (Utilities|Casting|CastToKaijuCharacter (Ability|GetAvatarActorfromActorInfo)))
  (Animation|PlayAnimMontage _askaiju_character NewParam 1.0 "charge"))

(fn SetAimDirectioninKaijuBP
  (params (Laser%20Aim%20Direction :type Vector))
  (bind _asbp_kaiju_character (Utilities|Casting|CastToBP_KaijuCharacter (Ability|GetOwningActorfromActorInfo)))
  (Variables|/Game/NeoKaiju/KaijuCharacter/BP_KaijuCharacter.BP_KaijuCharacter_C|SetLaser%20Aim%20Angle _asbp_kaiju_character (Class|SafeDirectionUtility|GetAngleOfVectorAwayfromDirection Laser%20Aim%20Direction (Variables|/Script/Neokaiju.KaijuMovementComponent|GetFacingDirection (Variables|/Script/Neokaiju.KaijuCharacter|GetKaijuMovement (Variables|Default|GetCharacter))))))

(fn LevelKaijutoGround
  (Class|KaijuMovementComponent|SetCharacterForward (Variables|/Script/Neokaiju.KaijuCharacter|GetKaijuMovement (Variables|Default|GetCharacter)) (Class|SafeDirectionUtility|GetSafeForwardDirectionfromFacing (Variables|/Script/Neokaiju.KaijuMovementComponent|GetFacingDirection (Variables|/Script/Neokaiju.KaijuCharacter|GetKaijuMovement (Variables|Default|GetCharacter)))) "0, 0, 0" "0, 0, 0" 0.0 0.0 true))