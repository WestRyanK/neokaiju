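; Gameplay ability that performs the kaiju's swipe attack, covering its sound, controller rumble and animation.
; On activation it plays the swipe sound event at the avatar's location and sends force feedback to player controller 0.
; It then casts the avatar to KaijuCharacter and plays the dash spin attack montage from its start section.
; The graph itself contains no hit detection, ability commit or EndAbility call.
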(event Ability|EventActivateAbility
  (CallFunction|PlayEvent (Variables|Default|GetSwipeSoundEvent) (Transformation|GetActorLocation (Ability|GetAvatarActorfromActorInfo)))
  (Game|Feedback|ClientPlayForceFeedback (Game|GetPlayerController 0) (Variables|Default|GetSwipeForceFeedback) "None" false false false)
  (CallFunction|PlaySwipeMontage))

(fn PlaySwipeMontage
  (bind _askaiju_character (Utilities|Casting|CastToKaijuCharacter (Ability|GetAvatarActorfromActorInfo)))
  (Animation|PlayAnimMontage _askaiju_character "/Game/NeoKaiju/Ability/StandardAbilities/SwipeAbility/AM_KaijuCharacter_dash_spin_attack.AM_KaijuCharacter_dash_spin_attack" 1.0 "start"))