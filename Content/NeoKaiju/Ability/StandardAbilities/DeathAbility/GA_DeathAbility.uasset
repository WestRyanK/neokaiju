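; Gameplay ability that handles a Kaiju character's death.
; OnDeath caches the avatar, starts a half-second timer, shuts off back and tail fire effects, and plays controller rumble for player 0.
; PlayDeathAnimation fakes a shatter: it plays the death sound, hides the mesh and spawns destructible jiblets in Kaiju armor material with sparks.
; Montage and launch nodes are left unused.
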(event Ability|EventActivateAbility)

(event Ability|EventOnEndAbility
  (params (bWasCancelled :type Boolean)))

(event EventOnDeath
  (bind _asbp_kaiju_character (Utilities|Casting|CastToBP_KaijuCharacter (Ability|GetAvatarActorfromActorInfo)))
  (Variables|Default|SetCharacter _asbp_kaiju_character)
  (Utilities|Time|SetTimerbyEvent (EventDispatchers|CreateEvent :!event PlayDeathAnimation) 0.5)
  (CallFunction|DeactivateFire)
  (Game|Feedback|ClientPlayForceFeedback (Game|GetPlayerController 0) (Variables|Default|GetDeathForceFeedback) "None" false false false))

(fn DeactivateFire
  (Components|Activation|Deactivate (Variables|/Game/NeoKaiju/KaijuCharacter/BP_KaijuCharacter.BP_KaijuCharacter_C|GetBV_BackFire (Variables|Default|GetCharacter)))
  (Components|Activation|Deactivate (Variables|/Game/NeoKaiju/KaijuCharacter/BP_KaijuCharacter.BP_KaijuCharacter_C|GetBV_TailFire (Variables|Default|GetCharacter)))
  (Components|Activation|Deactivate (Variables|/Game/NeoKaiju/KaijuCharacter/BP_KaijuCharacter.BP_KaijuCharacter_C|GetFV_BackFire (Variables|Default|GetCharacter)))
  (Components|Activation|Deactivate (Variables|/Game/NeoKaiju/KaijuCharacter/BP_KaijuCharacter.BP_KaijuCharacter_C|GetFV_TailFire (Variables|Default|GetCharacter))))

(fn PlayDeathAnimation
  (bind _character (Variables|Default|GetCharacter))
  (bind _mesh (Variables|/Script/Engine.Character|GetMesh _character))
  (bind _returnvalue (Transformation|GetWorldTransform _mesh))
  (bind (_location _rotation _scale) (Math|Transform|BreakTransform _returnvalue))
  (CallFunction|PlayEvent "/Game/Neokaiju/Audio/Events/Character/Death.Death" (Transformation|GetActorLocation (Ability|GetAvatarActorfromActorInfo)))
  (Rendering|SetVisibility _mesh false true)
  (bind _returnvalue_2 (Game|SpawnActorfromClass "/Game/NeoKaiju/Structures/Blocks/BP_BuildingJiblets.BP_BuildingJiblets_C" _returnvalue "Undefined" 0 "/Game/NeoKaiju/KaijuCharacter/SkeletalMeshes/static/DeathDM.DeathDM" 5e+02 0))
  (Rendering|Material|SetMaterial (Variables|/Script/ApexDestruction.DestructibleActor|GetDestructibleComponent _returnvalue_2) 0 "/Game/NeoKaiju/KaijuCharacter/Lvl1Materials/MI_KaijuArmor_Lvl1.MI_KaijuArmor_Lvl1")
  (Effects|SpawnEmitteratLocation "/Game/NeoKaiju/Cinematic/Sparks_impact.Sparks_impact" _location _rotation (/ _scale 2.0)))