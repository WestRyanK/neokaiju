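; Gameplay ability that presents a kaiju's level change with slow motion, camera focus, particles, a montage and growth.
; The pre-change event levels the kaiju's orientation, centers the camera focus point on it, then starts these effects.
; A timed lerp, adjusted for time dilation, eases actor scale toward an attribute value along a power curve.
; The post-change event restores camera and time, then swaps in that level's skeletal mesh.
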(event EventOnPreLevelChange
  (params (OldLevel :type Float%20%28single-precision%29) (NewLevel :type Float%20%28single-precision%29))
  (bind _askaiju_character (Utilities|Casting|CastToKaijuCharacter (Ability|GetAvatarActorfromActorInfo)))
  (Variables|Default|SetCharacter _askaiju_character)
  (CallFunction|LevelKaijutoGround)
  (CallFunction|FocusCameraonKaiju)
  (Utilities|Time|SetGlobalTimeDilation (Variables|Default|GetSlowdownMagnitude))
  (CallFunction|SpawnLevelChangeParticles OldLevel)
  (CallFunction|StartKaijuLerpScale)
  (CallFunction|PlayAnimationMontage))

(event EventOnPostLevelChange
  (params (OldLevel :type Float%20%28single-precision%29) (NewLevel :type Float%20%28single-precision%29))
  (CallFunction|PostLevelChange (Math|Float|Truncate NewLevel)))

(fn PlayAnimationMontage
  (bind _askaiju_character (Utilities|Casting|CastToKaijuCharacter (Ability|GetOwningActorfromActorInfo)))
  (Animation|PlayAnimMontage _askaiju_character "/Game/NeoKaiju/Ability/StandardAbilities/LevelChangeAbility/AM_KaijuCharacter_levelup.AM_KaijuCharacter_levelup" 1.0 "Default"))

(fn PostLevelChange
  (params (NewLevel :type Integer))
  (CallFunction|ReturnCameraOriginalPosition)
  (Utilities|Time|SetGlobalTimeDilation 1.0)
  (CallFunction|SetSkeletalMesh NewLevel))

(fn FocusCameraonKaiju
  (bind _character (Variables|Default|GetCharacter))
  (bind _rootcomponent (Variables|/Script/Engine.Actor|GetRootComponent _character))
  (bind _returnvalue (Transformation|GetWorldLocation _rootcomponent))
  (Transformation|SetWorldLocation (CallFunction|GetFocusPoint) (Math|Vector|MakeVector (.x _returnvalue) (.y (Transformation|GetWorldLocation (CallFunction|GetFocusPoint))) (.z _returnvalue)) false false))

(fn ReturnCameraOriginalPosition
  (Transformation|SetWorldLocation (CallFunction|GetFocusPoint) (Transformation|GetWorldLocation (Utilities|Array|Get(acopy) (Class|SceneComponent|GetParentComponents (CallFunction|GetFocusPoint)))) false false))

(fn GetFocusPoint
  (return (Variables|/Script/Neokaiju.KaijuCharacter|GetCameraFocusPoint (Variables|Default|GetCharacter))))

(fn SpawnLevelChangeParticles
  (params (OldLevel :type Float%20%28single-precision%29))
  (Niagara|SpawnSystemAttached (Utilities|Array|Get(acopy) (Variables|Default|GetLevelUps) (Math|Float|Truncate (- OldLevel 1.0))) (Variables|/Script/Engine.Actor|GetRootComponent (Ability|GetAvatarActorfromActorInfo)) "None" "0, 0, 0" "0, 0, 0" "SnapToTarget" true))

(fn SetSkeletalMesh
  (params (NewLevel :type Integer))
  (if (Utilities|Array|IsValidIndex (Variables|Default|GetKaijuLevelMeshes) NewLevel)
    (Class|SkinnedMeshComponent|SetSkeletalMesh (Variables|/Script/Engine.Character|GetMesh (Variables|Default|GetCharacter)) (Utilities|Array|Get(acopy) (Variables|Default|GetKaijuLevelMeshes) NewLevel) false)))

(fn StartKaijuLerpScale
  (bind _self self)
  (Variables|Default|SetStartScale (.y (Transformation|GetActorScale3D (Variables|Default|GetCharacter))))
  (Variables|Default|SetEndScale (.ReturnValue (Ability|Attribute|GetFloatAttribute (Variables|Default|GetCharacter) "(AttributeName=\"KaijuSizeScale\",Attribute=StructProperty'\"/Script/Neokaiju.KaijuAttributeSet:KaijuSizeScale\"',AttributeOwner=Class'\"/Script/Neokaiju.KaijuAttributeSet\"')")))
  (Variables|Default|SetScaleDistance (- (Variables|Default|GetEndScale) (Variables|Default|GetStartScale)))
  (bind _returnvalue (Class|LerpUtility|LerpFloatOverTime _self _self 0.0 1.0 (- (* (Variables|Default|GetSlomoDuration) (Variables|Default|GetSlowdownMagnitude)) 0.25) 0.01 0.0))
  (LocalVariables|SetScaleLerper _returnvalue)
  (EventDispatchers|BindEventtoFloatUpdated (LocalVariables|GetScaleLerper) (EventDispatchers|CreateEvent :!event ScaleKaijuTick))
  (Class|LerpUtility|Begin (LocalVariables|GetScaleLerper)))

(fn ScaleKaijuTick
  (params (ScaleValue :type Float%20%28single-precision%29))
  (Transformation|SetActorScale3D (Variables|Default|GetCharacter) (Math|Conversions|ToVector(Float) (+ (Variables|Default|GetStartScale) (* (Variables|Default|GetScaleDistance) (Math|Float|Power ScaleValue (Variables|Default|GetGrowthPower)))))))

(fn LevelKaijutoGround
  (Class|KaijuMovementComponent|SetCharacterForward (Variables|/Script/Neokaiju.KaijuCharacter|GetKaijuMovement (Variables|Default|GetCharacter)) (Class|SafeDirectionUtility|GetSafeForwardDirectionfromFacing (Variables|/Script/Neokaiju.KaijuMovementComponent|GetFacingDirection (Variables|/Script/Neokaiju.KaijuCharacter|GetKaijuMovement (Variables|Default|GetCharacter)))) "0, 0, 0" "0, 0, 0" 0.0 0.0 true))