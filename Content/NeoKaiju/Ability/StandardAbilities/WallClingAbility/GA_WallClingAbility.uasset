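; Gameplay ability for wall clinging that supplies the visual and controller rumble feedback.
; On cling start it plays a one-shot wall-hit rumble and a looping slide rumble on player 0.
; After a short delay it spawns a particle burst facing opposite the owning component's yaw and attaches a constant slide effect to that component.
; Ending the ability destroys the attached effect and stops the looping rumble.
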(event Ability|EventActivateAbility)

(event Ability|EventOnEndAbility
  (params (bWasCancelled :type Boolean))
  (CallFunction|DestroyifValid (Variables|Default|GetWallSlide))
  (CallFunction|StopForceFeedback))

(event EventOnBeginWallCling
  (bind _returnvalue (Class|GameplayAbility|GetOwningComponentfromActorInfo))
  (bind _returnvalue_2 (Transformation|GetWorldRotation _returnvalue))
  (bind (_roll _pitch _yaw) (Math|Rotator|BreakRotator _returnvalue_2))
  (CallFunction|PlayForceFeedback)
  (Ability|Tasks|WaitDelay 0.07
    (:then
      (Niagara|SpawnSystematLocation "/Game/NeoKaiju/Particles/John_Particles/PS_JParticleBurst.PS_JParticleBurst" (Transformation|GetWorldLocation _returnvalue) (Math|Rotator|MakeRotator _roll _pitch (+ _yaw 1.8e+02)))
      (bind _returnvalue_3 (Niagara|SpawnSystemAttached "/Game/NeoKaiju/Particles/John_Particles/PS_JParticleConst.PS_JParticleConst" _returnvalue "None" "0, 0, 0" "-90.000000, 0,0.000000" "KeepRelativeOffset" false))
      (Variables|Default|SetWallSlide _returnvalue_3))))

(fn PlayForceFeedback
  (Game|Feedback|ClientPlayForceFeedback (Game|GetPlayerController 0) (Variables|Default|GetWallHitForceFeedback) "None" false false false)
  (Game|Feedback|ClientPlayForceFeedback (Game|GetPlayerController 0) (Variables|Default|GetWallSlideForceFeedback) "None" true false false))

(fn StopForceFeedback
  (Utilities|IsValid (Game|GetPlayerController 0)
    (:Is%20Valid
      (Game|Feedback|ClientStopForceFeedback (Game|GetPlayerController 0) (Variables|Default|GetWallSlideForceFeedback) "None"))))