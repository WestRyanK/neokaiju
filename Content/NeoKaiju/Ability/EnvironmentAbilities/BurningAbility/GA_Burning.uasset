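; GA_Burning is an environment gameplay ability that shows a burning particle effect on its owning actor while active.
; On activation it runs the parent logic, then attaches the burn emitter at reduced scale to the owner's root component and stores the spawned component.
; When the ability ends, it destroys that component if still valid before handing off to the parent.
; The graph itself handles only the visual effect.
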(event Ability|EventActivateAbility
  (|CallParentFunction)
  (CallFunction|SpawnBurning))

(event Ability|EventOnEndAbility
  (params (bWasCancelled :type Boolean))
  (CallFunction|DestroySpawnedBurning)
  (|CallParentFunction false))

(fn SpawnBurning
  (bind _returnvalue (Effects|SpawnEmitterAttached (Variables|Default|GetBurnParticleEffect) (Variables|/Script/Engine.Actor|GetRootComponent (Ability|GetOwningActorfromActorInfo)) "None" "0, 0, 0" "0, 0, 0" (Math|Conversions|ToVector(Float) 0.5)))
  (Variables|Default|SetSpawnedBurnParticleEffect _returnvalue))

(fn DestroySpawnedBurning
  (if (Utilities|IsValid (Variables|Default|GetSpawnedBurnParticleEffect))
    (Components|DestroyComponent (Variables|Default|GetSpawnedBurnParticleEffect))))