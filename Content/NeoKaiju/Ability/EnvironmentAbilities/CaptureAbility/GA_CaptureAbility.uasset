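; Environment gameplay ability that reports when the player kaiju is trapped by or released from a capturing claw.
; Its capture begin and end events check whether the captive is player character 0, then call the matching trapped or released function on the kaiju character event subsystem.
; The graph holds no capture logic of its own, only these notifications.
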(event EventCaptureBegin
  (params (CaptiveActor :type Actor%20Object%20Reference))
  (if (== CaptiveActor (Game|GetPlayerCharacter 0))
    (Class|KaijuCharacterEventSubsystem|KaijuTrappedbyClaw (Subsystems|GetKaijuCharacterEventSubsystem))))

(event Ability|EventOnEndAbility
  (params (bWasCancelled :type Boolean)))

(event EventCaptureEnd
  (params (CaptiveActor :type Actor%20Object%20Reference))
  (if (== CaptiveActor (Game|GetPlayerCharacter 0))
    (Class|KaijuCharacterEventSubsystem|KaijuReleasedfromClaw (Subsystems|GetKaijuCharacterEventSubsystem))))