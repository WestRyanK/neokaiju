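; BP_AchievementCountdownTimer adds audio feedback to a countdown timer, playing a ten-second countdown sound as time nears its end.
; The nearing-end event starts the 2D FMOD event, stores its instance and sets a validity flag.
; On each tick, if the timer is no longer near its end while that flag is set, it clears the flag and stops and releases the sound.
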(event EventOnNearingEnd
  (bind _returnvalue (Class|FMODBlueprintStatics|PlayEvent2D "/Game/Neokaiju/Audio/Events/UI/TenSecondCountdown.TenSecondCountdown"))
  (Variables|Default|SetCountdownTickerSound _returnvalue)
  (Variables|Default|SetTickerValid true))

(event EventOnCountdownTicked
  (if (and (not (Class|BaseCountdownTimer|GetIsNearEnd)) (Variables|Default|GetTickerValid))
    (Variables|Default|SetTickerValid false)
    (bind _returnvalue (Class|FMODBlueprintStatics|EventInstanceIsValid (Variables|Default|GetCountdownTickerSound)))
    (if _returnvalue
      (Class|FMODBlueprintStatics|EventInstanceStop (Variables|Default|GetCountdownTickerSound) true))))