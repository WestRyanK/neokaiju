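; BP_CoreLibrary is a shared helper function library for NeoKaiju.
; It wraps null-safe cleanup of components, actors and widgets, hardcoded level names, map-driven Niagara float setting, and FMOD event playback.
; ShouldPlayDamageFX detects health dropping to quarter steps of a float attribute, and SetSfxEnabled toggles the SFX VCA between saved volume and zero.
; DisplayLoading does nothing, as its loading-screen widget nodes are disconnected.
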(fn DestroyifValid
  (params (Component :type Actor%20Component%20Object%20Reference))
  (Utilities|IsValid Component
    (:Is%20Valid
      (Components|DestroyComponent Component))))

(fn GetMainLevelName
  (return "VerticalSlice_Final"))

(fn GetMenuLevelName
  (return "MainMenuMap"))

(fn SetNiagaraSystemValues
  (params (NiagaraSystem :type Niagara%20Component%20Object%20Reference) (NamesAndValues :type Map%20of%20Names%20to%20Float%20%28single-precision%29s))
  (Utilities|IsValid NiagaraSystem
    (:Is%20Valid
      (bind _keys (Utilities|Map|Keys NamesAndValues))
      (for _array_element _keys
        (Niagara|SetNiagaraVariable(Float) NiagaraSystem _array_element (.Value (Utilities|Map|Find NamesAndValues _array_element)))))))

(fn DestroyActorifValid
  (params (Actor :type Actor%20Object%20Reference))
  (Utilities|IsValid Actor
    (:Is%20Valid
      (Actor|DestroyActor Actor))))

(fn RemoveifValid
  (params (Widget :type User%20Widget%20Object%20Reference))
  (Utilities|IsValid Widget
    (:Is%20Valid
      (Widget|RemovefromParent Widget))))

(fn PlayEvent
  (params (Event :type FMOD%20Event%20Object%20Reference) (Location :type Vector%20%28by%20ref%29))
  (bind _returnvalue (Class|FMODBlueprintStatics|PlayEventatLocation Event (Math|Conversions|ToTransform(Vector) Location)))
  (return _returnvalue))

(fn PlayEventAttached
  (params (Event :type FMOD%20Event%20Object%20Reference) (Location :type Scene%20Component%20Object%20Reference%20%28by%20ref%29))
  (bind _returnvalue (Class|FMODBlueprintStatics|PlayEventAttached Event Location "None" "0, 0, 0" "SnapToTarget" true))
  (return _returnvalue))

(fn ShouldPlayDamageFX
  (params (OldHealth :type Float%20%28single-precision%29) (NewHealth :type Float%20%28single-precision%29) (Actor :type Actor%20Object%20Reference))
  (LocalVariables|SetPlayIncrements (/ (.ReturnValue (Ability|Attribute|GetFloatAttribute Actor "(AttributeName=\"MaxHealth\",Attribute=StructProperty'\"/Script/Neokaiju.DamageableAttributeSet:MaxHealth\"',AttributeOwner=Class'\"/Script/Neokaiju.DamageableAttributeSet\"')")) 4.0))
  (LocalVariables|SetThreshold (* (Math|Float|Truncate (/ OldHealth (LocalVariables|GetPlayIncrements))) (LocalVariables|GetPlayIncrements)))
  (return (<= NewHealth (LocalVariables|GetThreshold))))

(fn SetSfxEnabled
  (params (WorldContextObject :type Object%20Object%20Reference) (SfxEnabled :type Boolean))
  (bind _asneokaiju_game_instance (Utilities|Casting|CastToNeokaijuGameInstance (Game|GetGameInstance WorldContextObject)))
  (Class|FMODBlueprintStatics|VCASetVolume "/Game/Neokaiju/Audio/VCAs/SFX_VCA.SFX_VCA" (select SfxEnabled (Class|KaijuGameUserSettings|GetSoundVolume (Variables|/Script/Neokaiju.NeokaijuGameInstance|GetGameSettings _asneokaiju_game_instance)) 0.0)))

(fn DisplayLoading
  (params (World%20Context%20Object :type Object%20Object%20Reference)))