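; Game mode for NeoKaiju play levels, handling the intro cinematic, level music, countdown start and SFX enabling around play phases.
; PlayIntroSequence builds a tag-based seamless sequence player with camera ease-out and binds the controller's skip request, while SequenceFinished unbinds it and sets a short timer.
; PrePlayPhaseBegan is overridden empty, with TransitionToPlay calling the parent version instead.
; Music starts alongside the countdown, fades through a Timeline, and stops at post-play or EndPlay.
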(event Custom|MusicFadeIn
  (bind _volume (Timeline|Fade PlayFromStart)
    (:Update
      (Class|FMODBlueprintStatics|EventInstanceSetVolume (Variables|Default|GetMusic) _volume))))

(event Custom|MusicFadeOut
  (bind _volume (Timeline|Fade ReverseFromEnd)
    (:Update
      (Class|FMODBlueprintStatics|EventInstanceSetVolume (Variables|Default|GetMusic) _volume))))

(event EventEndPlay
  (params (EndPlayReason :type EEndPlayReason%20Enum :default "Destroyed"))
  (Class|FMODBlueprintStatics|EventInstanceStop (Variables|Default|GetMusic) true)
  (CallFunction|SetSfxEnabled self true)
  (|CallParentFunction EndPlayReason))

(event EventPrePlayPhaseBegan)

(event EventStartMusicandTimer
  (bind _returnvalue (Class|FMODBlueprintStatics|PlayEvent2D "/Game/Neokaiju/Audio/Events/Music/Main_Theme.Main_Theme"))
  (Variables|Default|SetMusic _returnvalue)
  (Class|BaseCountdownTimer|StartCountdown (Variables|Default|GetCountdownTimer) false))

(event EventPlayPhaseBegan
  (Utilities|FlowControl|Delay 0.3)
  (CallFunction|SetSfxEnabled self true))

(event EventPostPlayPhaseBegan
  (CallFunction|StopMusic))

(fn ConstructionScript)

(fn PlayIntroSequence
  (bind _askaiju_character_controller (Utilities|Casting|CastToKaijuCharacterController (Game|GetPlayerController 0)))
  (bind _output_get (Variables|Default|SetCharacterController _askaiju_character_controller))
  (EventDispatchers|BindEventtoOnSkipIntroRequested _output_get (EventDispatchers|CreateEvent :!event StopSequence))
  (Development|PrintString "PrePlay Phase")
  (bind _returnvalue (Class|SeamlessSequencePlayer|CreateSeamlessSequencePlayerfromTags "OpeningSequence" "OpeningSequenceCamera" 0.0 1.0 true "VTBlend_Linear" "VTBlend_EaseInOut" 0.0 1.0))
  (bind _output_get_2 (Variables|Default|SetIntroSequencePlayer _returnvalue))
  (EventDispatchers|BindEventtoOnSeamlessSequencePlayerFinished _output_get_2 (EventDispatchers|CreateEvent :!event SequenceFinished))
  (Class|SeamlessSequencePlayer|PlaySequence (Variables|Default|GetIntroSequencePlayer)))

(fn StopSequence
  (Class|SeamlessSequencePlayer|StopSequence (Variables|Default|GetIntroSequencePlayer)))

(fn SequenceFinished
  (EventDispatchers|UnbindEventfromOnSkipIntroRequested (Variables|Default|GetCharacterController) (EventDispatchers|CreateEvent :!event StopSequence))
  (Utilities|Time|SetTimerbyEvent (EventDispatchers|CreateEvent :!event TransitiontoPlay) 0.25))

(fn ChoosePlayerStart
  (params (Player :type Controller%20Object%20Reference))
  (return (Class|NeokaijuPlayerStart|GetCurrentPlayerStart)))

(fn TransitiontoPlay
  (|CallParentFunction))

(fn StopMusic
  (Class|FMODBlueprintStatics|EventInstanceStop (Variables|Default|GetMusic) true))